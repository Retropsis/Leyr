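; BP_Chest is a container actor for a lootable chest with a Paper2D flipbook lid, seeded with a Gladius.
; Shortly after BeginPlay, it calls ServerAddItem on its Container to add the starting item.
; ToggleContainerLid forwards to a multicast event that jumps the flipbook to an open or closed frame and plays the matching sound at the chest's location.
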(event `self.ReceiveBeginPlay`
  (`parent.ReceiveBeginPlay`)
  (`KismetSystemLibrary.Delay` 0.2)
  (`InventoryComponent.ServerAddItem` (`self.Container`) (make `InventoryItemData` 2 1 1 "/Game/Inventory/ItemData/Weapons/DA_Gladius.DA_Gladius" 0.0 0.0 "/Game/World/Item/BP_Gladius.BP_Gladius_C")))

(event `self.ToggleContainerLid`
  (params (bOpen :type Boolean))
  (`self.MulticastToggleContainerLid` bOpen))

(event `MulticastToggleContainerLid`
  (params (IsOpen :type Boolean))
  (bind _returnvalue (`self.K2_GetActorLocation`))
  (if IsOpen
    (`PaperFlipbookComponent.SetPlaybackPositionInFrames` (`self.PaperFlipbook`) 2 false)
    (`GameplayStatics.PlaySoundAtLocation` "/Engine/VREditor/Sounds/UI/Floating_UI_Open.Floating_UI_Open" _returnvalue (struct) 1.0 1.0 0.0 null null null null)
    (else
      (`PaperFlipbookComponent.SetPlaybackPositionInFrames` (`self.PaperFlipbook`) 1 false)
      (`GameplayStatics.PlaySoundAtLocation` "/Engine/VREditor/Sounds/UI/Floating_UI_Close.Floating_UI_Close" _returnvalue (struct) 1.0 1.0 0.0 null null null null))))

(fn `UserConstructionScript`)