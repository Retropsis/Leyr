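; BP_ContainerBase is a base loot container actor with a flipbook lid and an inventory Container.
; BuildContainerLoot applies the flipbook and lid sounds from ContainerData, then resolves its items in DT_Items and adds them with their quantities through ServerAddItem.
; ToggleContainerLid calls a multicast event that switches the flipbook frame and plays the open or close sound.
; Hardcoded test items remain in unconnected nodes.
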(event `self.ToggleContainerLid`
  (params (bOpen :type Boolean))
  (`self.MulticastToggleContainerLid` bOpen))

(event `MulticastToggleContainerLid`
  (params (IsOpen :type Boolean))
  (bind _returnvalue (`self.K2_GetActorLocation`))
  (if IsOpen
    (`PaperFlipbookComponent.SetPlaybackPositionInFrames` (`self.PaperFlipbook`) 2 false)
    (`GameplayStatics.PlaySoundAtLocation` (`self.OpenLidSound`) _returnvalue (struct) 1.0 1.0 0.0 null null null null)
    (else
      (`PaperFlipbookComponent.SetPlaybackPositionInFrames` (`self.PaperFlipbook`) 1 false)
      (`GameplayStatics.PlaySoundAtLocation` (`self.CloseLidSound`) _returnvalue (struct) 1.0 1.0 0.0 null null null null))))

(event `self.BuildContainerLoot`
  (bind _containerdata (`self.ContainerData`))
  (`PaperFlipbookComponent.SetFlipbook` (`self.PaperFlipbook`) (`ContainerData.ContainerFlipbook` _containerdata))
  (set `self.OpenLidSound` (`ContainerData.OpenLidSound` _containerdata))
  (set `self.CloseLidSound` (`ContainerData.CloseLidSound` _containerdata))
  (for _array_element (`ContainerData.Items` _containerdata)
    (bind (_item _quantity) (break `ContainerItem` _array_element))
    (bind _returnvalue (`|GetDataTableRow` "/Game/World/Data/DT_Items.DT_Items" (`.RowName` (break `DataTableRowHandle` _item)))
      (:`then`
        (bind _structout (setmembers `InventoryItemData` :`StructRef` (`.ItemData` (break `ItemDataRow` _returnvalue)) :`Quantity` _quantity))
        (`InventoryComponent.ServerAddItem` (`self.Container`) _structout)))))

(fn `UserConstructionScript`)