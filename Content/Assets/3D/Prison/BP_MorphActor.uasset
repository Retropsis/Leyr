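; Prison actor that fakes a perspective shift by driving skeletal mesh morph targets from the player's camera position.
; A box trigger tracks the overlapping PlayerCharacter, and BeginPlay caches its extents and fully applies the Perspective morph.
; Each Tick maps the camera's X offset from the box center, scaled by extent, to LeftPos or RightPos weights.
; Vertical UpwardPos and GroundPos logic is disconnected, though Z is still debug-printed.
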(event `self.ReceiveBeginPlay`
  (set `self.ExtentX` (.x (`BoxComponent.GetScaledBoxExtent` (`self.Box`))))
  (set `self.ExtentZ` (.z (`BoxComponent.GetScaledBoxExtent` (`self.Box`))))
  (`SkeletalMeshComponent.SetMorphTarget` (`self.SkeletalMesh`) "Perspective" 1.0 false))

(event `self.ReceiveTick`
  (params (DeltaSeconds :type "Float (single-precision)"))
  (`self.Morph`))

(event `self.Box.OnComponentBeginOverlap`
  (params (OverlappedComponent :type "PrimitiveComponent Object Reference") (OtherActor :type "Actor Object Reference") (OtherComp :type "PrimitiveComponent Object Reference") (OtherBodyIndex :type Integer) (bFromSweep :type Boolean) (SweepResult :type "HitResult Structure (by ref)"))
  (bind _asplayer_character (cast `PlayerCharacter` OtherActor))
  (set `self.PlayerCharacter` _asplayer_character))

(event `self.Box.OnComponentEndOverlap`
  (params (OverlappedComponent :type "PrimitiveComponent Object Reference") (OtherActor :type "Actor Object Reference") (OtherComp :type "PrimitiveComponent Object Reference") (OtherBodyIndex :type Integer))
  (cast `PlayerCharacter` OtherActor)
  (set `self.PlayerCharacter` null))

(fn `Morph`
  (locals (CameraX :type "Float (double-precision)" :default 0.0) (CameraZ :type "Float (double-precision)"))
  (bind _playercharacter (`self.PlayerCharacter`)
    (:`then`
      (set `local.CameraX` (- (.x (`PlayerCharacter.GetCameraOffsetLocation` _playercharacter)) (.x (`SceneComponent.K2_GetComponentLocation` (`self.Box`)))))
      (bind _output_get (set `local.CameraZ` (- (.z (`PlayerCharacter.GetCameraOffsetLocation` _playercharacter)) (.z (`SceneComponent.K2_GetComponentLocation` (`self.Box`))))))
      (`KismetSystemLibrary.PrintString` (`KismetStringLibrary.Conv_DoubleToString` _output_get))
      (`|ExecutionSequence`
        (:`then_0`
          (if (< (`local.CameraX`) 0.0)
            (`SkeletalMeshComponent.SetMorphTarget` (`self.SkeletalMesh`) "LeftPos" (`KismetMathLibrary.MapRangeClamped` (/ (`KismetMathLibrary.Abs` (`local.CameraX`)) (- (`self.ExtentX`) 128.0)) 0.0 0.6 0.0 1.0) false)))
        (:`then_1`
          (if (> (`local.CameraX`) 0.0)
            (`SkeletalMeshComponent.SetMorphTarget` (`self.SkeletalMesh`) "RightPos" (`KismetMathLibrary.MapRangeClamped` (/ (`local.CameraX`) (- (`self.ExtentX`) 128.0)) 0.0 0.6 0.0 1.0) false)))))
    (:`else`)))

(fn `UserConstructionScript`)