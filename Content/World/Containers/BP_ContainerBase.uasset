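; Base world container Blueprint with a flipbook lid and sounds, relayed through a multicast event.
; Opening plays the flipbook from the start with CloseLidSound; closing jumps to the last frame without a play call, with OpenLidSound.
; BuildContainerLoot is empty; unconnected nodes would load art and sounds from ContainerData and add its items to the container via DT_DefaultItem.
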(event `self.ToggleContainerLid`
  (params (bOpen :type Boolean))
  (`self.MulticastToggleContainerLid` bOpen))

(event `MulticastToggleContainerLid`
  (params (IsOpen :type Boolean))
  (bind _returnvalue (`self.K2_GetActorLocation`))
  (if IsOpen
    (`PaperFlipbookComponent.SetPlaybackPositionInFrames` (`self.RenderComponent`) 1 false)
    (`PaperFlipbookComponent.PlayFromStart` (`self.RenderComponent`))
    (`PaperFlipbookComponent.SetPlayRate` (`self.RenderComponent`) 1.0)
    (`PaperFlipbookComponent.SetLooping` (`self.RenderComponent`) false)
    (`GameplayStatics.PlaySoundAtLocation` (`self.CloseLidSound`) _returnvalue (struct) 1.0 1.0 0.0 null null null null)
    (else
      (`PaperFlipbookComponent.SetPlaybackPositionInFrames` (`self.RenderComponent`) (- (`PaperFlipbookComponent.GetFlipbookLengthInFrames` (`self.RenderComponent`)) 1) false)
      (`PaperFlipbookComponent.SetPlayRate` (`self.RenderComponent`) 1.0)
      (`PaperFlipbookComponent.SetLooping` (`self.RenderComponent`) false)
      (`GameplayStatics.PlaySoundAtLocation` (`self.OpenLidSound`) _returnvalue (struct) 1.0 1.0 0.0 null null null null))))

(event `self.BuildContainerLoot`)

(fn `UserConstructionScript`)