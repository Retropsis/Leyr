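; BP_Platform_Default is a moving level platform that travels toward a current target point.
; Each tick it offsets BoxCollision along the normalized direction from the actor's location to CurrentTarget, scaled by Speed, without sweeping.
; When HasReachedTarget reports arrival, it calls ChooseNextTarget; neither function is defined here.
; Movement is not scaled by delta time, so travel speed depends on frame rate.
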(event `self.ReceiveTick`
  (params (DeltaSeconds :type "Float (single-precision)"))
  (`SceneComponent.K2_AddWorldOffset` (`self.BoxCollision`) (* (`KismetMathLibrary.Normal` (- (`self.CurrentTarget`) (`self.K2_GetActorLocation`))) (`self.Speed`)) false false)
  (if (`self.HasReachedTarget`)
    (`self.ChooseNextTarget`)))

(fn `UserConstructionScript`)