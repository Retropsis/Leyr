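; BP_EffectSpawner is a level actor that spawns effects when the player enters one of its six effect colliders.
; On BeginPlay it binds all six colliders' begin-overlap events to one shared handler.
; The handler filters for actors implementing PlayerInterface, then passes the overlapped collider and sweep result to SpawnEffects, whose logic is not defined in these graphs.
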(event `self.ReceiveBeginPlay`
  (add `PrimitiveComponent.OnComponentBeginOverlap` (`self.EffectCollider_0`) (delegate `OnBeginOverlap`))
  (add `PrimitiveComponent.OnComponentBeginOverlap` (`self.EffectCollider_1`) (delegate `OnBeginOverlap`))
  (add `PrimitiveComponent.OnComponentBeginOverlap` (`self.EffectCollider_2`) (delegate `OnBeginOverlap`))
  (add `PrimitiveComponent.OnComponentBeginOverlap` (`self.EffectCollider_3`) (delegate `OnBeginOverlap`))
  (add `PrimitiveComponent.OnComponentBeginOverlap` (`self.EffectCollider_4`) (delegate `OnBeginOverlap`))
  (add `PrimitiveComponent.OnComponentBeginOverlap` (`self.EffectCollider_5`) (delegate `OnBeginOverlap`)))

(event `OnBeginOverlap`
  (params (OverlappedComponent :type "PrimitiveComponent Object Reference") (OtherActor :type "Actor Object Reference") (OtherComp :type "PrimitiveComponent Object Reference") (OtherBodyIndex :type Integer) (bFromSweep :type Boolean) (SweepResult :type "HitResult Structure (by ref)"))
  (if (`KismetSystemLibrary.DoesImplementInterface` OtherActor "/Script/Leyr.PlayerInterface")
    (`|ExecutionSequence`
      (:`then_0`
        (`self.SpawnEffects` OverlappedComponent SweepResult)))))

(fn `UserConstructionScript`)