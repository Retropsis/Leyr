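; Breakable brazier prop that falls when a bone of its constrained MultiPartFlipbook is hit, presumably its hanging support.
; InteractHit makes the first constraint whose parent body matches the hit bone linearly breakable at a low threshold, then enables physics and WorldStatic blocking on the brazier capsule.
; The capsule's first subsequent hit unbinds the hit event and spawns impact sound and effect, guarded to fire once.
; It also prints the bone name for debugging.
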(event `InteractionInterface.InteractHit`
  (params (InteractingActor :type "Actor Object Reference") (BoneName :type Name))
  (`KismetSystemLibrary.PrintString` (`KismetStringLibrary.Conv_NameToString` BoneName) true true (struct :`G` 1.0 :`B` 0.591451 :`A` 1.0) 3.0)
  (bind _outconstraints (`SkeletalMeshComponent.GetConstraints` (`self.MultiPartFlipbook`) false))
  (for _array_element _outconstraints
    (bind _parentbody (`ConstraintInstanceBlueprintLibrary.GetAttachedBodyNames` _array_element))
    (if (== _parentbody BoneName)
      (`ConstraintInstanceBlueprintLibrary.SetLinearBreakable` _array_element true 10.0)
      (break)))
  (`PrimitiveComponent.SetCollisionResponseToChannel` (`self.Capsule_Brazier`) "ECC_WorldStatic" "ECR_Block")
  (`PrimitiveComponent.SetCollisionEnabled` (`self.Capsule_Brazier`) "PhysicsOnly")
  (`PrimitiveComponent.SetSimulatePhysics` (`self.Capsule_Brazier`) true)
  (add `PrimitiveComponent.OnComponentHit` (`self.Capsule_Brazier`) (`|CreateDelegate` :!event `BrazierOnHit`)))

(event `BrazierOnHit`
  (params (HitComponent :type "PrimitiveComponent Object Reference") (OtherActor :type "Actor Object Reference") (OtherComp :type "PrimitiveComponent Object Reference") (NormalImpulse :type "Vector Structure") (Hit :type "HitResult Structure (by ref)"))
  (bind (_bblockinghit _binitialoverlap _time _distance _location) (`GameplayStatics.BreakHitResult` Hit))
  (if (not (`self.bHit`))
    (set `self.bHit` true)
    (clear `PrimitiveComponent.OnComponentHit` (`self.Capsule_Brazier`))
    (`GameplayStatics.PlaySoundAtLocation` (`self.ImpactSound`) _location (struct) 1.0 1.0 0.0 null null null null)
    (`NiagaraFunctionLibrary.SpawnSystemAtLocation` (`self.ImpactEffect`) (+ _location (0.0 0.0 20.0)) (struct) (0.5 0.5 0.5))))

(fn `UserConstructionScript`)