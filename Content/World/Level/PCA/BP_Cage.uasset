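; BP_Cage is a cage actor with a flipbook door that can flash, shake and be knocked off.
; PlayFlashEffect animates flash color and strength on a dynamic material instance created at BeginPlay.
; PlayShakeEffect offsets the flipbook from its cached location on X and Z, randomly picking one of three timeline curves per axis.
; DoorDestroyed detaches BoxDoor, launches it with physics and ignored collision responses, and spins it through a slowed timeline.
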(event `self.ReceiveBeginPlay`
  (bind _returnvalue (`PrimitiveComponent.CreateDynamicMaterialInstance` (`self.DoorFlipbook`) 0 null "None"))
  (set `self.DynamicSpriteInstance` _returnvalue)
  (set `self.SpriteLocation` (`SceneComponent.RelativeLocation` (`self.DoorFlipbook`))))

(event `self.DoorDestroyed`
  (bind _box_door (`self.Box_Door`))
  (`SceneComponent.K2_DetachFromComponent` _box_door "KeepWorld" "KeepWorld" "KeepWorld" true)
  (`PrimitiveComponent.SetSimulatePhysics` _box_door true)
  (`PrimitiveComponent.SetEnableGravity` _box_door true)
  (`PrimitiveComponent.SetCollisionEnabled` _box_door "PhysicsOnly")
  (`PrimitiveComponent.AddImpulse` _box_door (125.0 0.0 0.0) "None" true)
  (`PrimitiveComponent.SetCollisionResponseToAllChannels` (`self.Box_Door`) "ECR_Ignore")
  (`TimelineComponent.SetPlayRate` (`self.RoationTimeline`) 0.25)
  (bind (_direction _alpha) (`Timeline|RoationTimeline` :!via `PlayFromStart`)
    (:`Update`
      (`SceneComponent.K2_SetRelativeRotation` (`self.Box_Door`) (`KismetMathLibrary.RLerp` (struct) (struct :`Pitch` -360.0) _alpha) false false))))

(event `self.PlayFlashEffect`
  (params (Strength :type "Float (single-precision)") (PlayRate :type "Float (single-precision)") (Color :type "LinearColor Structure"))
  (`MaterialInstanceDynamic.SetScalarParameterValue` (`self.DynamicSpriteInstance`) "FlashStrength" 0.0)
  (`MaterialInstanceDynamic.SetVectorParameterValue` (`self.DynamicSpriteInstance`) "FlashColor" Color)
  (`TimelineComponent.SetPlayRate` (`self.FlashTimeline`) PlayRate)
  (bind (_direction _alpha) (`Timeline|FlashTimeline` :!via `PlayFromStart`)
    (:`Update`
      (`MaterialInstanceDynamic.SetScalarParameterValue` (`self.DynamicSpriteInstance`) "FlashStrength" (`KismetMathLibrary.Lerp` 0.0 Strength _alpha)))))

(event `self.PlayShakeEffect`
  (params (Strength :type "Float (single-precision)") (PlayRate :type "Float (single-precision)"))
  (set `self.RandomTrack_X` (`KismetMathLibrary.RandomIntegerInRange` 0 2))
  (set `self.RandomTrack_Z` (`KismetMathLibrary.RandomIntegerInRange` 0 2))
  (`TimelineComponent.SetPlayRate` (`self.ShakingTimeline`) PlayRate)
  (bind (_direction _1 _2 _3) (`Timeline|ShakingTimeline` :!via `PlayFromStart`)
    (:`Update`
      (`SceneComponent.K2_SetRelativeLocation` (`self.DoorFlipbook`) (+ (`KismetMathLibrary.MakeVector` (`KismetMathLibrary.Lerp` 0.0 Strength (select `int` (`self.RandomTrack_X`) :`0` _1 :`1` _2 :`2` _3 :!type "Float (double-precision)")) 0.0 (`KismetMathLibrary.Lerp` 0.0 Strength (select `int` (`self.RandomTrack_Z`) :`0` _1 :`1` _2 :`2` _3 :!type "Float (double-precision)"))) (`self.SpriteLocation`)) false false))))

(fn `UserConstructionScript`)