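; Medium torch variant B, a world prop that flickers and can be extinguished by an interact hit.
; A timeline feeds Alpha and Scale into UpdateFlicker, then calls SelectFlicker on finish to loop.
; SelectFlicker rolls a random branch, but both outcomes play the same flicker.
; Hit events pass to HandleOnHit, which, like UpdateFlicker and Extinguish, is defined outside this graph.
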(event `self.SelectFlicker`
  (switch `int` (`KismetMathLibrary.RandomIntegerInRange` 0 1)
    (:`0`
      _)
    (:`1`
      _))
  (`self.Flicker`))

(event `Flicker`
  (bind (_direction _alpha _scale) (`Timeline|Timeline` :!via `PlayFromStart`)
    (:`Update`
      (`self.UpdateFlicker` _alpha _scale))
    (:`Finished`
      (`self.SelectFlicker`))))

(event `InteractionInterface.InteractHit`
  (params (InteractingActor :type "Actor Object Reference") (BoneName :type Name))
  (`self.Extinguish`))

(event `self.OnHit`
  (params (HitComponent :type "PrimitiveComponent Object Reference") (OtherActor :type "Actor Object Reference") (OtherComp :type "PrimitiveComponent Object Reference") (NormalImpulse :type "Vector Structure") (Hit :type "HitResult Structure (by ref)"))
  (`self.HandleOnHit` Hit))

(fn `UserConstructionScript`)