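; BP_Door3D is a 3D door that animates between its closed and open states.
; HandleDoorMoving plays a double-speed timeline, choosing the opening or closing alpha track from the current door state.
; That alpha moves the collision between closed and open world locations while rotating the mesh through 90 degrees, both without sweeping.
; When the timeline finishes, it calls HandleOnFinishedPlaying to end the move.
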(event `self.HandleDoorMoving`
  (`TimelineComponent.SetPlayRate` (`self.DoorTimeline`) 2.0)
  (bind (_direction _opening_alpha _closing_alpha) (`Timeline|DoorTimeline` :!via `PlayFromStart`)
    (:`Update`
      (bind _returnvalue (select `EDoorState` (`self.GetDoorState`) :`Opening` _opening_alpha :`Closing` _closing_alpha))
      (`SceneComponent.K2_SetWorldLocation` (`self.DoorCollision`) (`KismetMathLibrary.VLerp` (`self.CloseLocation`) (`self.OpenLocation`) _returnvalue) false false)
      (`SceneComponent.K2_SetRelativeRotation` (`self.DoorMesh`) (`KismetMathLibrary.RLerp` (struct) (struct :`Yaw` 90.0) _returnvalue) false false))
    (:`Finished`
      (`self.HandleOnFinishedPlaying`))))

(fn `UserConstructionScript`)