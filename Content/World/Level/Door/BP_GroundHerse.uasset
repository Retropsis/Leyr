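; Ground herse (portcullis) door that plays open or close animations by door state and fakes perspective on its skeletal mesh with morph targets.
; Opening also starts a looping timer that spawns a capped series of rubble Niagara bursts.
; While the player is inside the overlap box, Tick drives left/right morphs from the camera's horizontal offset to the box center.
; Vertical morph logic exists but is disconnected.
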(event `self.HandleDoorMoving`
  (set `self.Count` 0)
  (`SkeletalMeshComponent.PlayAnimation` (`self.SKM_GroundHerse`) (select `EDoorState` (`self.GetDoorState`) :`Open` "/Game/Assets/3D/Prison/V2/Herse/SS_GroundHerse_Open.SS_GroundHerse_Open" :`Close` "/Game/Assets/3D/Prison/V2/Herse/SS_GroundHerse_Close.SS_GroundHerse_Close" :`Opening` "/Game/Assets/3D/Prison/V2/Herse/SS_GroundHerse_Open.SS_GroundHerse_Open" :`Closing` "/Game/Assets/3D/Prison/V2/Herse/SS_GroundHerse_Close.SS_GroundHerse_Close" :!type "AnimationAsset Object Reference") false)
  (if (`|EnumEquality` (`self.GetDoorState`) "Opening")
    (bind _returnvalue (`KismetSystemLibrary.K2_SetTimerDelegate` (delegate `SpawnVFX`) 0.5 true))
    (set `self.VFX_Timer` _returnvalue)
    (`self.SpawnVFX`)))

(event `SpawnVFX`
  (if (< (`self.Count`) 13)
    (`NiagaraFunctionLibrary.SpawnSystemAtLocation` "/Game/Effects/Dust/Rubbles/NS_Rubbles_Ledge.NS_Rubbles_Ledge" (`SceneComponent.K2_GetComponentLocation` (`self.VFX_SpawningPoint`)))
    (`/Engine/EditorBlueprintResources/StandardMacros.IncrementInt` (`self.Count`))
    (else
      (`KismetSystemLibrary.K2_ClearAndInvalidateTimerHandle` (`self.VFX_Timer`)))))

(event `self.ReceiveBeginPlay`
  (set `self.ExtentX` (.x (`BoxComponent.GetScaledBoxExtent` (`self.OverlapBox`))))
  (set `self.ExtentZ` (.z (`BoxComponent.GetScaledBoxExtent` (`self.OverlapBox`))))
  (`SkeletalMeshComponent.SetMorphTarget` (`self.SKM_GroundHerse`) "Perspective" 0.5 false))

(event `self.ReceiveTick`
  (params (DeltaSeconds :type "Float (single-precision)"))
  (`self.Morph`))

(event `self.OverlapBox.OnComponentBeginOverlap`
  (params (OverlappedComponent :type "PrimitiveComponent Object Reference") (OtherActor :type "Actor Object Reference") (OtherComp :type "PrimitiveComponent Object Reference") (OtherBodyIndex :type Integer) (bFromSweep :type Boolean) (SweepResult :type "HitResult Structure (by ref)"))
  (bind _asplayer_character (cast `PlayerCharacter` OtherActor))
  (set `self.PlayerCharacter` _asplayer_character))

(event `self.OverlapBox.OnComponentEndOverlap`
  (params (OverlappedComponent :type "PrimitiveComponent Object Reference") (OtherActor :type "Actor Object Reference") (OtherComp :type "PrimitiveComponent Object Reference") (OtherBodyIndex :type Integer))
  (cast `PlayerCharacter` OtherActor)
  (set `self.PlayerCharacter` null))

(fn `Morph`
  (locals (CameraX :type "Float (double-precision)") (CameraZ :type "Float (double-precision)"))
  (bind _playercharacter (`self.PlayerCharacter`)
    (:`then`
      (set `local.CameraX` (- (.x (`PlayerCharacter.GetCameraOffsetLocation` _playercharacter)) (.x (`SceneComponent.K2_GetComponentLocation` (`self.OverlapBox`)))))
      (set `local.CameraZ` (- (.z (`PlayerCharacter.GetCameraOffsetLocation` _playercharacter)) (.z (`SceneComponent.K2_GetComponentLocation` (`self.OverlapBox`)))))
      (`|ExecutionSequence`
        (:`then_0`
          (if (< (`local.CameraX`) 0.0)
            (`SkeletalMeshComponent.SetMorphTarget` (`self.SKM_GroundHerse`) "LeftPos" (`KismetMathLibrary.MapRangeClamped` (/ (`KismetMathLibrary.Abs` (`local.CameraX`)) (- (`self.ExtentX`) 128.0)) 0.0 0.6 0.0 1.0) false)))
        (:`then_1`
          (if (> (`local.CameraX`) 0.0)
            (`SkeletalMeshComponent.SetMorphTarget` (`self.SKM_GroundHerse`) "RightPos" (`KismetMathLibrary.MapRangeClamped` (/ (`local.CameraX`) (- (`self.ExtentX`) 128.0)) 0.0 0.6 0.0 1.0) false)))))
    (:`else`)))

(fn `UserConstructionScript`)