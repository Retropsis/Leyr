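; BP_MovingSands is a 2D level piece that draws a horizontal strip of sand tiles; this graph holds no movement or overlap logic.
; Its construction script rebuilds a Paper2D grouped sprite, adding one Tile instance per Width unit at a fixed tile spacing.
; Instances are placed in world space, centered on the actor's X by integer half-width, at its Z and pinned to the Y=0 plane.
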(fn `UserConstructionScript`
  (`PaperGroupedSpriteComponent.ClearInstances` (`self.PaperGroupedSprite`))
  (`/Engine/EditorBlueprintResources/StandardMacros.IsValid` (`self.Tile`)
    (:`Is Valid`
      (for _index (range (`self.Width`))
        (`PaperGroupedSpriteComponent.AddInstance` (`self.PaperGroupedSprite`) (`KismetMathLibrary.MakeTransform` (`KismetMathLibrary.MakeVector` (`KismetMathLibrary.Conv_IntToDouble` (+ (+ (- (.x (`self.K2_GetActorLocation`)) (* (/ (`self.Width`) 2) 64)) (* _index 64)) 32)) 0.0 (.z (`self.K2_GetActorLocation`)))) (`self.Tile`) true (struct :`R` 1.0 :`G` 1.0 :`B` 1.0 :`A` 1.0))))))