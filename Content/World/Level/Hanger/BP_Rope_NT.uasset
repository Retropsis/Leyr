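; BP_Rope_NT is a level rope assembled from Paper2D sprite tiles, with a box collision named for hanging.
; The construction script rebuilds a grouped-sprite row along X from Length, using fixed first and last tiles and random middle tiles.
; It sizes HangingCollision to the length and shifts the tile map left to center it.
; Tile spacing uses TileWidth, while collision and centering use a hardcoded 64-unit half-width.
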(fn `BuildTileMap`
  (locals (TileIndex :type Integer))
  (`PaperGroupedSpriteComponent.ClearInstances` (`self.TileMap`))
  (for _index (range (`self.Length`))
    (set `local.TileIndex` _index)
    (`PaperGroupedSpriteComponent.AddInstance` (`self.TileMap`) (`KismetMathLibrary.MakeTransform` (`KismetMathLibrary.MakeVector` (`KismetMathLibrary.Conv_IntToDouble` (* (`local.TileIndex`) (`self.TileWidth`))))) (select `bool` (== (`local.TileIndex`) 0) :`false` (select `bool` (== (`local.TileIndex`) (- (`self.Length`) 1)) :`false` (`KismetArrayLibrary.Array_Random` (`self.Tiles`)) :`true` (`self.LastTile`)) :`true` (`self.FirstTile`)) false (struct :`R` 1.0 :`G` 1.0 :`B` 1.0 :`A` 1.0)))
  (`BoxComponent.SetBoxExtent` (`self.HangingCollision`) (`KismetMathLibrary.MakeVector` (`KismetMathLibrary.Conv_IntToDouble` (* (`self.Length`) 64)) 100.0 16.0) true)
  (`SceneComponent.K2_SetRelativeLocation` (`self.TileMap`) (`KismetMathLibrary.MakeVector` (`KismetMathLibrary.Conv_IntToDouble` (* (* (- (`self.Length`) 1) 64) -1))) false false))

(fn `UserConstructionScript`
  (`self.BuildTileMap`))