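; BP_Ladder_32 is a hanger level piece that builds a vertical ladder of configurable length from 2D sprites.
; The construction script rebuilds the grouped sprite instances, stacking fixed first and last tiles around randomly picked middle tiles.
; It then sizes the HangingCollision box to the ladder length and shifts the sprite stack down to center it on that box.
; The event graph holds no active logic.
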(fn `BuildTileMap`
  (locals (TileIndex :type Integer))
  (`PaperGroupedSpriteComponent.ClearInstances` (`self.TileMap`))
  (for _index (range (`self.Length`))
    (set `local.TileIndex` _index)
    (`PaperGroupedSpriteComponent.AddInstance` (`self.TileMap`) (`KismetMathLibrary.MakeTransform` (`KismetMathLibrary.MakeVector` 0.0 0.0 (`KismetMathLibrary.Conv_IntToDouble` (* (`local.TileIndex`) (`self.TileWidth`))))) (select `bool` (== (`local.TileIndex`) 0) :`false` (select `bool` (== (`local.TileIndex`) (- (`self.Length`) 1)) :`false` (`KismetArrayLibrary.Array_Random` (`self.Tiles`)) :`true` (`self.LastTile`)) :`true` (`self.FirstTile`)) false (struct :`R` 1.0 :`G` 1.0 :`B` 1.0 :`A` 1.0)))
  (`BoxComponent.SetBoxExtent` (`self.HangingCollision`) (`KismetMathLibrary.MakeVector` 8.0 100.0 (`KismetMathLibrary.Conv_IntToDouble` (* (`self.Length`) 48))) true)
  (`SceneComponent.K2_SetRelativeLocation` (`self.TileMap`) (`KismetMathLibrary.MakeVector` 0.0 0.0 (`KismetMathLibrary.Conv_IntToDouble` (* (* (- (`self.Length`) 1) 48) -1))) false false))

(fn `UserConstructionScript`
  (`self.BuildTileMap`))