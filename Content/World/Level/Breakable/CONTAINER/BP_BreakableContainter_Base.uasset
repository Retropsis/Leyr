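; Base Blueprint for breakable containers that spawns loot items from its LootData asset when SpawnLoot is called.
; Evenly spaced rotators and a random distance range scatter drops along X only, at the container's height with world Y fixed at zero.
; SpawnLootItem spawns every entry in one loop, initializes each from its data table row and despawn flag, then clears the loot timer.
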(event `self.SpawnLoot`
  (bind _lootdata (`self.LootData`))
  (`/Engine/EditorBlueprintResources/StandardMacros.IsValid` _lootdata
    (:`Is Valid`
      (bind _returnvalue (`LootDataSet.GetLootItems` _lootdata))
      (bind _output_get (set `self.LootItems` _returnvalue))
      (set `self.LootRotations` (`self.GetLootRotations` _output_get))
      (set `self.LootCount` 0)
      (bind _returnvalue_2 (`KismetSystemLibrary.K2_SetTimerDelegate` :`Time` 0.1 :`bLooping` true))
      (set `self.LootTimer` _returnvalue_2)
      (`self.SpawnLootItem`))))

(event `SpawnLootItem`
  (for _index (range (`KismetArrayLibrary.Array_Length` (`self.LootItems`)))
    (bind ((`ItemClass` _itemclass) (`ItemRowHandle` _itemrowhandle) (`bShouldDespawn` _bshoulddespawn)) (break `LootData` (`|GetArrayItem` (`self.LootItems`) _index)))
    (bind _returnvalue (`|SpawnActorFromClass` _itemclass (`self.GetLootTransform` _index) "AlwaysSpawn" "MultiplyWithRoot" null null))
    (`Item.InitializeItemFromDataTable` (cast `Item` _returnvalue :!pure true) (`.RowName` (break `DataTableRowHandle` _itemrowhandle)) _bshoulddespawn))
  (`KismetSystemLibrary.K2_ClearAndInvalidateTimerHandle` (`self.LootTimer`)))

(fn `GetLootRotations`
  (params (TargetArray :type "Array of LootData Structure (by ref)"))
  (returns (ReturnValue :type "Array of Rotator Structure"))
  (return (`LeyrAbilitySystemLibrary.EvenlySpacedRotators` (`self.GetActorForwardVector`) (`KismetMathLibrary.Vector_Right`) 360.0 (`KismetArrayLibrary.Array_Length` TargetArray))))

(fn `GetLootTransform`
  (params (Count :type Integer))
  (returns (ReturnValue :type "Transform Structure"))
  (bind _returnvalue (`self.K2_GetActorLocation`))
  (return (`KismetMathLibrary.MakeTransform` (`KismetMathLibrary.MakeVector` (.x (+ (* (`KismetMathLibrary.GetForwardVector` (`|GetArrayItem` (`self.LootRotations`) Count)) (`KismetMathLibrary.RandomFloatInRange` (`self.MinSpawnDistance`) (`self.MaxSpawnDistance`))) _returnvalue)) 0.0 (.z _returnvalue)))))

(fn `UserConstructionScript`)