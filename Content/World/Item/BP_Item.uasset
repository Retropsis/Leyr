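; BP_Item is a world item actor that plays a spawn animation and then hands off to sinusoidal movement.
; On BeginPlay, the LocationZ timeline offsets height from the initial location by SpawnApex, pins Y to zero and animates Z scale, then calls StartSinusoidalMovement.
; Tick applies the calculated location and rotation unless physics is simulating.
; The StartRotation call is disconnected and never runs.
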(event `self.ReceiveBeginPlay`
  (bind (_direction _z _scale) (`Timeline|LocationZ` :!via `PlayFromStart`)
    (:`Update`
      (set `self.CalculatedLocation` (`self.CalculateZ` _z))
      (`self.SetActorScale3D` (`KismetMathLibrary.MakeVector` 1.0 1.0 _scale)))
    (:`Finished`
      (`self.StartSinusoidalMovement`))))

(event `self.ReceiveTick`
  (params (DeltaSeconds :type "Float (single-precision)"))
  (if (not (`self.IsSimulatingPhysics`))
    (`self.K2_SetActorLocation` (`self.CalculatedLocation`))
    (`self.K2_SetActorRotation` (`self.CalculatedRotation`))))

(fn `CalculateZ`
  (params (A :type "Float (double-precision)"))
  (returns (ReturnValue :type "Vector Structure"))
  (return (`KismetMathLibrary.MakeVector` (.x (`self.InitialLocation`)) 0.0 (+ (.z (`self.InitialLocation`)) (* A (`self.SpawnApex`))))))

(fn `UserConstructionScript`)