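; Deep Hopper AI creature Blueprint that animates a multi-part 2D body with four separately animated legs.
; On each state update, it checks whether the forward vector faces negative X and swaps each leg's left/right anim instance class to match, then passes the state to that instance.
; The construction script attaches the sprite to the body flipbook's Head socket.
; Older direct flipbook-switching chains remain but never run.
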(event `MultiPartAIInterface.UpdateMultiPartAnimInstances`
  (params (State :type "EMultiPartAnimationState Enum" :default "None"))
  (`self.MultiPart_ChangeDirections` (< (.x (`self.GetActorForwardVector`)) 0.0) State))

(event `self.MultiPart_ChangeDirections`
  (params (bIsFlipped :type Boolean) (State :type "EMultiPartAnimationState Enum" :default "None"))
  (`|ExecutionSequence`
    (:`then_0`
      (`PaperZDAnimationComponent.SetAnimInstanceClass` (`self.FrontLeg_L_Component`) (select `bool` bIsFlipped :`false` "/Game/AI/DeepHopper/ABP_FrontLeg_L.ABP_FrontLeg_L_C" :`true` "/Game/AI/DeepHopper/ABP_FrontLeg_R.ABP_FrontLeg_R_C" :!type "PaperZDAnimInstance Class Reference"))
      (`AICharacterAnimInstance.SetMultiPartAnimInstance` (cast `AICharacterAnimInstance` (`PaperZDAnimationComponent.AnimInstance` (`self.FrontLeg_L_Component`)) :!pure true) State))
    (:`then_1`
      (`PaperZDAnimationComponent.SetAnimInstanceClass` (`self.FrontLeg_R_Component`) (select `bool` bIsFlipped :`false` "/Game/AI/DeepHopper/ABP_FrontLeg_R.ABP_FrontLeg_R_C" :`true` "/Game/AI/DeepHopper/ABP_FrontLeg_L.ABP_FrontLeg_L_C" :!type "PaperZDAnimInstance Class Reference"))
      (`AICharacterAnimInstance.SetMultiPartAnimInstance` (cast `AICharacterAnimInstance` (`PaperZDAnimationComponent.AnimInstance` (`self.FrontLeg_R_Component`)) :!pure true) State))
    (:`then_2`
      (`PaperZDAnimationComponent.SetAnimInstanceClass` (`self.BackLeg_R_Component`) (select `bool` bIsFlipped :`false` "/Game/AI/DeepHopper/ABP_BackLeg_R.ABP_BackLeg_R_C" :`true` "/Game/AI/DeepHopper/ABP_BackLeg_L.ABP_BackLeg_L_C" :!type "PaperZDAnimInstance Class Reference"))
      (`AICharacterAnimInstance.SetMultiPartAnimInstance` (cast `AICharacterAnimInstance` (`PaperZDAnimationComponent.AnimInstance` (`self.BackLeg_R_Component`)) :!pure true) State))
    (:`then_3`
      (`PaperZDAnimationComponent.SetAnimInstanceClass` (`self.BackLeg_L_Component`) (select `bool` bIsFlipped :`false` "/Game/AI/DeepHopper/ABP_BackLeg_L.ABP_BackLeg_L_C" :`true` "/Game/AI/DeepHopper/ABP_BackLeg_R.ABP_BackLeg_R_C" :!type "PaperZDAnimInstance Class Reference"))
      (`AICharacterAnimInstance.SetMultiPartAnimInstance` (cast `AICharacterAnimInstance` (`PaperZDAnimationComponent.AnimInstance` (`self.BackLeg_L_Component`)) :!pure true) State))))

(fn `UserConstructionScript`
  (`parent.UserConstructionScript`)
  (`SceneComponent.K2_AttachToComponent` (`self.Sprite`) (`self.MultiPartFlipbook`) "Head" "KeepRelative" "KeepRelative" "KeepRelative" true))