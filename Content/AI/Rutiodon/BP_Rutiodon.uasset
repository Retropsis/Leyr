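; Rutiodon AI character built from multiple flipbook parts, with the head attached to a socket and body capsules feeding overlap damage.
; Hit flashes drive each part's dynamic material from its own timeline alpha track.
; Turning swaps leg flipbooks and translucent sort priority to fake depth.
; Timelines lerp the actor through out-and-back attacks that end the ability by gameplay event, a tag-selected splatter attack, and a death ending in Niagara particles.
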(event `self.HandleDeathMultiParts`
  (`PrimitiveComponent.SetCollisionEnabled` (`self.Body_Capsule_03`) "NoCollision")
  (`PrimitiveComponent.SetCollisionEnabled` (`self.Body_Capsule_04`) "NoCollision")
  (`PrimitiveComponent.SetCollisionEnabled` (`self.Body_Capsule_05`) "NoCollision")
  (`PrimitiveComponent.SetCollisionEnabled` (`self.Head_Capsule`) "NoCollision")
  (`PrimitiveComponent.SetCollisionEnabled` (`self.Body_Capsule_02`) "NoCollision"))

(event `self.ReceiveBeginPlay`
  (`parent.ReceiveBeginPlay`)
  (`KismetSystemLibrary.Delay` 0.2)
  (`self.Add Flipbooks`)
  (`KismetArrayLibrary.Array_Add` (`self.DMI_First`) (`self.DynamicSpriteInstance`))
  (for _array_element (`self.Flipbooks`)
    (bind _returnvalue (`PrimitiveComponent.CreateDynamicMaterialInstance` _array_element 0 null "None"))
    (`KismetArrayLibrary.Array_Add` (`self.DMI_First`) _returnvalue)))

(event `self.PlayFlashEffect`
  (params (Strength :type "Float (single-precision)") (PlayRate :type "Float (single-precision)") (Color :type "LinearColor Structure"))
  (`MaterialInstanceDynamic.SetScalarParameterValue` (`self.DynamicSpriteInstance`) "FlashStrength" Strength)
  (`MaterialInstanceDynamic.SetVectorParameterValue` (`self.DynamicSpriteInstance`) "FlashColor" Color)
  (`TimelineComponent.SetPlayRate` (`self.FirstTimeline`) PlayRate)
  (bind (_direction _alpha_head _alpha_7 _alpha_6 _alpha_5 _alpha_4 _alpha_3 _alpha_2 _alpha_1 _alpha_root) (`Timeline|FirstTimeline` :!via `PlayFromStart`)
    (:`Update`
      (for (_array_element _array_index) (`self.DMI_First`)
        (`MaterialInstanceDynamic.SetScalarParameterValue` _array_element "FlashStrength" (`KismetMathLibrary.Lerp` 0.0 Strength (select `int` _array_index :`0` _alpha_head :`1` _alpha_7 :`2` _alpha_6 :`3` _alpha_5 :`4` _alpha_4 :`5` _alpha_3 :`6` _alpha_2 :`7` _alpha_1 :`8` _alpha_root :`9` _alpha_root :`10` _alpha_root :`11` _alpha_root)))))))

(event `self.SetupCollisionDamage`
  (add `PrimitiveComponent.OnComponentBeginOverlap` (`self.Head_Capsule`) (delegate `OnComponentBeginOverlap_Event`))
  (add `PrimitiveComponent.OnComponentBeginOverlap` (`self.Body_Capsule_02`) (delegate `OnComponentBeginOverlap_Event`))
  (add `PrimitiveComponent.OnComponentBeginOverlap` (`self.Body_Capsule_03`) (delegate `OnComponentBeginOverlap_Event`))
  (add `PrimitiveComponent.OnComponentBeginOverlap` (`self.Body_Capsule_04`) (delegate `OnComponentBeginOverlap_Event`))
  (add `PrimitiveComponent.OnComponentBeginOverlap` (`self.Body_Capsule_05`) (delegate `OnComponentBeginOverlap_Event`)))

(event `OnComponentBeginOverlap_Event`
  (params (OverlappedComponent :type "PrimitiveComponent Object Reference") (OtherActor :type "Actor Object Reference") (OtherComp :type "PrimitiveComponent Object Reference") (OtherBodyIndex :type Integer) (bFromSweep :type Boolean) (SweepResult :type "HitResult Structure (by ref)"))
  (`self.HandleBeginOverlap` OtherActor))

(event `MultiPartAIInterface.UpdateMultiPartAnimInstances`
  (params (State :type "EMultiPartAnimationState Enum" :default "None"))
  (`self.MultiPart_ChangeDirections` (< (.x (`self.GetActorForwardVector`)) 0.0) State))

(event `self.MultiPart_ChangeDirections`
  (params (bIsFlipped :type Boolean) (State :type "EMultiPartAnimationState Enum" :default "None"))
  (`self.FlipMultiPartDirection` bIsFlipped))

(event `AIInterface.TimelineMovement`
  (params (TargetDestination :type "Vector Structure"))
  (bind _forward (`self.Forward`))
  (set `self.EndTimelineLocation` TargetDestination)
  (`TimelineComponent.SetPlayRate` (`self.Forward`) 1.0)
  (bind (_direction _jumpingupz) (`Timeline|Forward` :!via `PlayFromStart`)
    (:`Update`
      (`self.K2_SetActorLocation` (`KismetMathLibrary.VLerp` (`self.InitialTimelineLocation`) (`self.EndTimelineLocation`) _jumpingupz))
      (if (>= (/ (`TimelineComponent.GetPlaybackPosition` _forward) (`TimelineComponent.GetTimelineLength` _forward)) 0.25)
        (`/Engine/EditorBlueprintResources/StandardMacros.DoOnce` false :!label _label
          (:`Completed`
            (`self.EndTimelineMovement`)))))
    (:`Finished`
      (`KismetSystemLibrary.Delay` 0.5)
      (set `self.EndTimelineLocation` (`self.K2_GetActorLocation`))
      (bind (_direction_2 _z) (`Timeline|Return` :!via `PlayFromStart`)
        (:`Update`
          (`self.K2_SetActorLocation` (`KismetMathLibrary.VLerp` (`self.EndTimelineLocation`) (`self.InitialTimelineLocation`) _z))
          (goto _label :!via `Reset`))
        (:`Finished`
          (`AbilitySystemBlueprintLibrary.SendGameplayEventToActor` self (struct :`TagName` "Montage.EndAbility")))))))

(event `MultiPartAIInterface.PlayMultiPartMontages`
  (params (MontageTag :type "GameplayTag Structure (by ref)") (TargetLocation :type "Vector Structure (by ref)"))
  (bind _destroyedtimeline (`self.DestroyedTimeline`))
  (bind _x (.x (`self.InitialDestroyedLocation`)))
  (bind _z (.z (`self.InitialDestroyedLocation`)))
  (`|SwitchGameplayTag` MontageTag
    (:`Defeated`
      (set `self.InitialDestroyedLocation` (`self.K2_GetActorLocation`))
      (`|ExecutionSequence`
        (:`then_0`
          (`PaperFlipbookComponent.SetFlipbook` (`self.FrontLeg_L`) "/Game/Assets/Monster/Rutiodon/Destroyed/FB_Rutiodon_Destroyed_FrontLeg_L.FB_Rutiodon_Destroyed_FrontLeg_L")
          (`PaperFlipbookComponent.SetFlipbook` (`self.Body_02`) "/Game/Assets/Monster/Rutiodon/Destroyed/FB_Rutiodon_Destroyed_Body_2.FB_Rutiodon_Destroyed_Body_2"))
        (:`then_1`
          (`PaperFlipbookComponent.SetFlipbook` (`self.FrontLeg_R`) "/Game/Assets/Monster/Rutiodon/Destroyed/FB_Rutiodon_Destroyed_FrontLeg_R.FB_Rutiodon_Destroyed_FrontLeg_R")
          (`PaperFlipbookComponent.SetFlipbook` (`self.Body_03`) "/Game/Assets/Monster/Rutiodon/Destroyed/FB_Rutiodon_Destroyed_Body_03.FB_Rutiodon_Destroyed_Body_03"))
        (:`then_2`
          (`PaperFlipbookComponent.SetFlipbook` (`self.BackLeg_L`) "/Game/Assets/Monster/Rutiodon/Destroyed/FB_Rutiodon_Destroyed_BackLeg_L.FB_Rutiodon_Destroyed_BackLeg_L")
          (`PaperFlipbookComponent.SetFlipbook` (`self.Body_04`) "/Game/Assets/Monster/Rutiodon/Destroyed/FB_Rutiodon_Destroyed_Body_04.FB_Rutiodon_Destroyed_Body_04"))
        (:`then_3`
          (`PaperFlipbookComponent.SetFlipbook` (`self.Sprite`) "/Game/Assets/Monster/Rutiodon/Destroyed/FB_Rutiodon_Destroyed_Head.FB_Rutiodon_Destroyed_Head")
          (`PaperFlipbookComponent.SetFlipbook` (`self.Body_05`) "/Game/Assets/Monster/Rutiodon/Destroyed/FB_Rutiodon_Destroyed_Body_05.FB_Rutiodon_Destroyed_Body_05"))
        (:`then_4`
          (`PaperFlipbookComponent.SetFlipbook` (`self.BackLeg_R`) "/Game/Assets/Monster/Rutiodon/Destroyed/FB_Rutiodon_Destroyed_BackLeg_R.FB_Rutiodon_Destroyed_BackLeg_R")
          (`PaperFlipbookComponent.SetFlipbook` (`self.Body_01`) "/Game/Assets/Monster/Rutiodon/Destroyed/FB_Rutiodon_Destroyed_Body_01.FB_Rutiodon_Destroyed_Body_01")
          (`TimelineComponent.SetPlayRate` (`self.DestroyedTimeline`) 1.0)
          (bind (_direction _x_2 _z_2) (`Timeline|DestroyedTimeline` :!via `PlayFromStart`)
            (:`Update`
              (`self.K2_SetActorLocation` (`KismetMathLibrary.MakeVector` (`KismetMathLibrary.Lerp` _x (+ _x (* (.x (`self.GetActorForwardVector`)) -75.0)) _x_2) 0.0 (`KismetMathLibrary.Lerp` _z (+ _z 125.0) _z_2)))
              (if (> (/ (`TimelineComponent.GetPlaybackPosition` _destroyedtimeline) (`TimelineComponent.GetTimelineLength` _destroyedtimeline)) 0.98)
                (`|DoOnceMultiInput`
                  (:`A Out`
                    (`NiagaraFunctionLibrary.SpawnSystemAtLocation` "/Game/Effects/BloodSplat/Rutiodon/NS_Rutiodon_Particles.NS_Rutiodon_Particles" (`KismetMathLibrary.MakeVector` (+ (.x (`self.InitialDestroyedLocation`)) (* (.x (`self.GetActorForwardVector`)) -110.0)) 0.0 (+ (.z (`self.InitialDestroyedLocation`)) 25.0)))
                    (`PaperZDAnimationComponent.SetAnimInstanceClass` (`self.AnimationComponent`) null)
                    (`|ExecutionSequence`
                      (:`then_0`
                        (`PaperFlipbookComponent.SetFlipbook` (`self.FrontLeg_L`) null)
                        (`PaperFlipbookComponent.SetFlipbook` (`self.Body_02`) null))
                      (:`then_1`
                        (`PaperFlipbookComponent.SetFlipbook` (`self.FrontLeg_R`) null)
                        (`PaperFlipbookComponent.SetFlipbook` (`self.Body_03`) null))
                      (:`then_2`
                        (`PaperFlipbookComponent.SetFlipbook` (`self.BackLeg_L`) null)
                        (`PaperFlipbookComponent.SetFlipbook` (`self.Body_04`) null))
                      (:`then_3`
                        (`PaperFlipbookComponent.SetFlipbook` (`self.Sprite`) null)
                        (`PaperFlipbookComponent.SetFlipbook` (`self.Body_05`) null))
                      (:`then_4`
                        (`PaperFlipbookComponent.SetFlipbook` (`self.BackLeg_R`) null)
                        (`PaperFlipbookComponent.SetFlipbook` (`self.Body_01`) null)))))))))))
    (:`Montage.Attack.2`
      (set `self.InitialSplatterLocation` (`self.K2_GetActorLocation`))
      (set `self.SplatterTargetLocation` TargetLocation)
      (`|ExecutionSequence`
        (:`then_0`
          (`PaperFlipbookComponent.SetFlipbook` (`self.FrontLeg_L`) "/Game/Assets/Monster/Rutiodon/Splatter/FB_Rutiodon_Splatter_FrontLeg_L.FB_Rutiodon_Splatter_FrontLeg_L"))
        (:`then_1`
          (`PaperFlipbookComponent.SetFlipbook` (`self.FrontLeg_R`) "/Game/Assets/Monster/Rutiodon/Splatter/FB_Rutiodon_Splatter_FrontLeg_R.FB_Rutiodon_Splatter_FrontLeg_R")
          (`TimelineComponent.SetPlayRate` (`self.SplatterTimeline`) 1.0)
          (bind (_direction_2 _x_3) (`Timeline|SplatterTimeline` :!via `PlayFromStart`)
            (:`Update`
              (`self.K2_SetActorLocation` (`KismetMathLibrary.VLerp` (`self.InitialSplatterLocation`) (`self.SplatterTargetLocation`) _x_3)))
            (:`Finished`
              (`KismetSystemLibrary.Delay` 1.5)
              (`PaperFlipbookComponent.SetFlipbook` (`self.FrontLeg_L`) "/Game/Assets/Monster/Rutiodon/FB_Rutiodon_FrontLeg_L_Swim.FB_Rutiodon_FrontLeg_L_Swim")
              (`PaperFlipbookComponent.SetFlipbook` (`self.FrontLeg_R`) "/Game/Assets/Monster/Rutiodon/FB_Rutiodon_FrontLeg_R_Swim.FB_Rutiodon_FrontLeg_R_Swim"))))))))

(fn `Add Flipbooks`
  (`|ExecutionSequence`
    (:`then_0`
      (`KismetArrayLibrary.Array_Add` (`self.Flipbooks`) (`self.FrontLeg_L`))
      (`KismetArrayLibrary.Array_Add` (`self.Flipbooks`) (`self.FrontLeg_R`)))
    (:`then_1`
      (`KismetArrayLibrary.Array_Add` (`self.Flipbooks`) (`self.Body_01`))
      (`KismetArrayLibrary.Array_Add` (`self.Flipbooks`) (`self.Body_02`))
      (`KismetArrayLibrary.Array_Add` (`self.Flipbooks`) (`self.Body_03`))
      (`KismetArrayLibrary.Array_Add` (`self.Flipbooks`) (`self.Body_04`))
      (`KismetArrayLibrary.Array_Add` (`self.Flipbooks`) (`self.Body_05`)))
    (:`then_2`
      (`KismetArrayLibrary.Array_Add` (`self.Flipbooks`) (`self.BackLeg_L`))
      (`KismetArrayLibrary.Array_Add` (`self.Flipbooks`) (`self.BackLeg_R`)))))

(fn `FlipMultiPartDirection`
  (params (IsFlipped :type Boolean))
  (if IsFlipped
    (`PaperFlipbookComponent.SetFlipbook` (`self.BackLeg_R`) null)
    (`PaperFlipbookComponent.SetFlipbook` (`self.BackLeg_L`) "/Game/Assets/Monster/Rutiodon/FB_Rutiodon_BackLeg_R_Swim.FB_Rutiodon_BackLeg_R_Swim")
    (`PaperFlipbookComponent.SetFlipbook` (`self.FrontLeg_L`) "/Game/Assets/Monster/Rutiodon/FB_Rutiodon_FrontLeg_R_Swim.FB_Rutiodon_FrontLeg_R_Swim")
    (`PaperFlipbookComponent.SetFlipbook` (`self.FrontLeg_R`) null)
    (`PrimitiveComponent.SetTranslucentSortPriority` (`self.FrontLeg_L`) (`self.HighestSortPriority`))
    (`PrimitiveComponent.SetTranslucentSortPriority` (`self.BackLeg_L`) (`self.HighestSortPriority`))
    (`PrimitiveComponent.SetTranslucentSortPriority` (`self.FrontLeg_R`) (`self.LowestSortPriority`))
    (`PrimitiveComponent.SetTranslucentSortPriority` (`self.BackLeg_R`) (`self.LowestSortPriority`))
    (else
      (`PaperFlipbookComponent.SetFlipbook` (`self.BackLeg_R`) "/Game/Assets/Monster/Rutiodon/FB_Rutiodon_BackLeg_R_Swim.FB_Rutiodon_BackLeg_R_Swim")
      (`PaperFlipbookComponent.SetFlipbook` (`self.BackLeg_L`) null)
      (`PaperFlipbookComponent.SetFlipbook` (`self.FrontLeg_L`) null)
      (`PaperFlipbookComponent.SetFlipbook` (`self.FrontLeg_R`) "/Game/Assets/Monster/Rutiodon/FB_Rutiodon_FrontLeg_R_Swim.FB_Rutiodon_FrontLeg_R_Swim")
      (`PrimitiveComponent.SetTranslucentSortPriority` (`self.FrontLeg_R`) (`self.HighestSortPriority`))
      (`PrimitiveComponent.SetTranslucentSortPriority` (`self.BackLeg_R`) (`self.HighestSortPriority`))
      (`PrimitiveComponent.SetTranslucentSortPriority` (`self.FrontLeg_L`) (`self.LowestSortPriority`))
      (`PrimitiveComponent.SetTranslucentSortPriority` (`self.BackLeg_L`) (`self.LowestSortPriority`)))))

(fn `UserConstructionScript`
  (`parent.UserConstructionScript`)
  (`SceneComponent.K2_AttachToComponent` (`self.Sprite`) (`self.MultiPartFlipbook`) "Head" "KeepRelative" "KeepRelative" "KeepRelative" true))