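; Pterygota larva AI actor that plays a parasite spawning animation and hops forward when it begins play.
; BeginPlay starts the PaperZD animation override, then computes a raised apex and a forward landing point from the spawn transform.
; Two chained timelines lerp the location up to the apex, then down to the target, without sweeping for collision.
; A disconnected flipbook play-rate adjustment never runs.
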(event `self.ReceiveBeginPlay`
  (bind _returnvalue (`self.K2_GetActorLocation`))
  (`PaperZDPlaySlotOverrideAction.PlayAnimationOverrideWithCallbacks` (`PaperZDAnimationComponent.AnimInstance` (`self.AnimationComponent`)) "/Game/Assets/Monster/Dorn_Parasite/AnimSequences/Dorn_Parasite_Spawning.Dorn_Parasite_Spawning"
    (:`then`
      (bind _output_get (set `self.imitialLocation` _returnvalue))
      (set `self.ApexLocation` (`KismetMathLibrary.MakeVector` (.x (+ _returnvalue (* (`self.GetActorForwardVector`) 80.0))) (.y _output_get) (+ (.z _output_get) 100.0)))
      (set `self.TargetLocation` (+ (`self.K2_GetActorLocation`) (* (`self.GetActorForwardVector`) 120.0)))
      (bind (_direction _alpha) (`Timeline|SpawnTimeline` :!via `PlayFromStart`)
        (:`Update`
          (`self.K2_SetActorLocation` (`KismetMathLibrary.VLerp` (`self.imitialLocation`) (`self.ApexLocation`) _alpha)))
        (:`Finished`
          (bind (_direction_2 _alpha_2) (`Timeline|Timeline_0` :!via `PlayFromStart`)
            (:`Update`
              (`self.K2_SetActorLocation` (`KismetMathLibrary.VLerp` (`self.ApexLocation`) (`self.TargetLocation`) _alpha_2)))))))))

(fn `UserConstructionScript`)