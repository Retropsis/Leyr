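; Pterygota egg pawn that plays its hatching sprite animation and then spawns a Pterygota larva.
; On BeginPlay it stops its AI controller's brain logic so the egg stays inert during playback.
; When playback finishes, it spawns the larva at its X/Z with a fixed Y depth, passes on its spline actor reference and spawns the larva's controller.
; The egg then disables its capsule collision rather than being destroyed.
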(event `self.ReceiveBeginPlay`
  (`PaperFlipbookComponent.SetPlayRate` (`self.Sprite`) 1.0)
  (`PaperFlipbookComponent.PlayFromStart` (`self.Sprite`))
  (add `PaperFlipbookComponent.OnFinishedPlaying` (`self.Sprite`) (delegate `OnFinishedPlaying_Event`))
  (bind _asbp_base_aicontroller (cast `/Game/AI/Behaviour/BP_BaseAIController` (`self.GetController`)))
  (`BrainComponent.StopLogic` (`AIController.BrainComponent` _asbp_base_aicontroller) "I'm just an egg"))

(event `OnFinishedPlaying_Event`
  (bind _returnvalue (`|SpawnActorFromClass` "/Game/AI/PterygotaLarva/BP_PterygotaLarva.BP_PterygotaLarva_C" (`KismetMathLibrary.MakeTransform` (`KismetMathLibrary.MakeVector` (.x (.location (`self.GetTransform`))) 10.0 (.z (.location (`self.GetTransform`))))) "AlwaysSpawn" "MultiplyWithRoot" null null))
  (set `AICharacter.SplineComponentActor` (`self.SplineComponentActor`) _returnvalue)
  (`self.SpawnDefaultController` _returnvalue)
  (`PrimitiveComponent.SetCollisionEnabled` (`self.CapsuleComponent`) "NoCollision"))

(fn `UserConstructionScript`)