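; Giant crocodile enemy that leaps vertically from a starting point and returns to it, with overlap handling on its body, head and tail.
; One timeline drives the jump height, then a second lerps it back, both using teleporting moves.
; The tail runs partially blended physics on the MultiPartFlipbook, with a sprite snapped to its Head socket.
; Bubbles attach while the capsule overlaps a crocodile effect boundary and deactivate on exit.
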(event `AIInterface.TimelineMovement`
  (bind (_direction _jumpingupz) (`Timeline|Timeline` :!via `PlayFromStart`)
    (:`Update`
      (`self.K2_SetActorLocation` (`KismetMathLibrary.MakeVector` (.x (`self.InitialTimelineLocation`)) (.y (`self.InitialTimelineLocation`)) (+ (.z (`self.InitialTimelineLocation`)) (* _jumpingupz (`self.JumpApex`)))) false true))
    (:`Finished`
      (`self.EndTimelineMovement`)
      (set `self.EndTimelineLocation` (`self.K2_GetActorLocation`))
      (bind (_direction_2 _z) (`Timeline|Timeline_0` :!via `PlayFromStart`)
        (:`Update`
          (`self.K2_SetActorLocation` (`KismetMathLibrary.VLerp` (`self.EndTimelineLocation`) (`self.InitialTimelineLocation`) _z) false true))))))

(event `self.ReceiveBeginPlay`
  (`self.ToggleTailPhysics` true))

(event `self.SetupCollisionDamage`
  (add `PrimitiveComponent.OnComponentBeginOverlap` (`self.Root_Box`) (delegate `OnComponentBeginOverlap_Event`))
  (add `PrimitiveComponent.OnComponentBeginOverlap` (`self.Head_Capsule`) (delegate `OnComponentBeginOverlap_Event`))
  (add `PrimitiveComponent.OnComponentBeginOverlap` (`self.Tail_Capsule_1`) (delegate `OnComponentBeginOverlap_Event`))
  (add `PrimitiveComponent.OnComponentBeginOverlap` (`self.Tail_Capsule_2`) (delegate `OnComponentBeginOverlap_Event`))
  (add `PrimitiveComponent.OnComponentBeginOverlap` (`self.Tail_Capsule_3`) (delegate `OnComponentBeginOverlap_Event`))
  (add `PrimitiveComponent.OnComponentBeginOverlap` (`self.Tail_Capsule_4`) (delegate `OnComponentBeginOverlap_Event`))
  (add `PrimitiveComponent.OnComponentBeginOverlap` (`self.Tail_Capsule_5`) (delegate `OnComponentBeginOverlap_Event`)))

(event `OnComponentBeginOverlap_Event`
  (params (OverlappedComponent :type "PrimitiveComponent Object Reference") (OtherActor :type "Actor Object Reference") (OtherComp :type "PrimitiveComponent Object Reference") (OtherBodyIndex :type Integer) (bFromSweep :type Boolean) (SweepResult :type "HitResult Structure (by ref)"))
  (`self.HandleBeginOverlap` OtherActor))

(event `self.CapsuleComponent.OnComponentBeginOverlap`
  (params (OverlappedComponent :type "PrimitiveComponent Object Reference") (OtherActor :type "Actor Object Reference") (OtherComp :type "PrimitiveComponent Object Reference") (OtherBodyIndex :type Integer) (bFromSweep :type Boolean) (SweepResult :type "HitResult Structure (by ref)"))
  (if (`GameplayStatics.ObjectIsA` OtherActor "/Game/World/Map/EffectBoundary_GiantCrocodile.EffectBoundary_GiantCrocodile_C")
    (bind _returnvalue (`NiagaraFunctionLibrary.SpawnSystemAttached` "/Game/Effects/Bubbles/NS_Bubbles.NS_Bubbles" (`self.CapsuleComponent`) "None" (0.0 0.0 0.0) (struct) "KeepRelativeOffset" true))
    (set `self.Bubbles` _returnvalue)))

(event `self.CapsuleComponent.OnComponentEndOverlap`
  (params (OverlappedComponent :type "PrimitiveComponent Object Reference") (OtherActor :type "Actor Object Reference") (OtherComp :type "PrimitiveComponent Object Reference") (OtherBodyIndex :type Integer))
  (if (`GameplayStatics.ObjectIsA` OtherActor "/Game/World/Map/EffectBoundary_GiantCrocodile.EffectBoundary_GiantCrocodile_C")
    (bind _bubbles (`self.Bubbles`)
      (:`then`
        (`ActorComponent.Deactivate` _bubbles))
      (:`else`))))

(fn `ToggleTailPhysics`
  (params (Enable :type Boolean))
  (`PrimitiveComponent.SetCollisionEnabled` (`self.MultiPartFlipbook`) (select `bool` Enable :`false` "NoCollision" :`true` "PhysicsOnly" :!type "ECollisionEnabled Enum"))
  (`SkeletalMeshComponent.SetAllBodiesBelowSimulatePhysics` (`self.MultiPartFlipbook`) (`self.TailRoot`) (`local.Enable`) false)
  (`SkeletalMeshComponent.SetAllBodiesBelowPhysicsBlendWeight` (`self.MultiPartFlipbook`) (`self.TailRoot`) (select `bool` (`local.Enable`) :`true` 0.5 :!type "Float (single-precision)") false false))

(fn `UserConstructionScript`
  (`parent.UserConstructionScript`)
  (`SceneComponent.K2_AttachToComponent` (`self.Sprite`) (`self.MultiPartFlipbook`) "Head" "SnapToTarget" "SnapToTarget" "SnapToTarget" true))