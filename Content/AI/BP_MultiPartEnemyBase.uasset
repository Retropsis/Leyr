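; Base Blueprint for multi-part enemies, providing loot drops and sprite hit-style effects in a 2D plane.
; SpawnLoot spawns all LootData items at once, initialized from data table rows; its looping timer is cleared immediately.
; Evenly spaced rotators and random distances scatter drops along X, at Y zero and the enemy's height.
; Timelines drive a material flash and a sprite shake using randomly chosen tracks per axis.
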(event `self.SpawnLoot`
  (bind _lootdata (`self.LootData`))
  (`/Engine/EditorBlueprintResources/StandardMacros.IsValid` _lootdata
    (:`Is Valid`
      (bind _returnvalue (`LootDataSet.GetLootItems` _lootdata))
      (bind _output_get (set `self.LootItems` _returnvalue))
      (set `self.LootRotations` (`self.GetLootRotations` _output_get))
      (set `self.LootCount` 0)
      (bind _returnvalue_2 (`KismetSystemLibrary.K2_SetTimerDelegate` (delegate `SpawnLootItem`) 0.1 true))
      (set `self.LootTimer` _returnvalue_2)
      (`self.SpawnLootItem`))))

(event `SpawnLootItem`
  (for _index (range (`KismetArrayLibrary.Array_Length` (`self.LootItems`)))
    (bind ((`ItemClass` _itemclass) (`ItemRowHandle` _itemrowhandle)) (break `LootData` (`|GetArrayItem` (`self.LootItems`) _index)))
    (bind _returnvalue (`|SpawnActorFromClass` _itemclass (`self.GetLootTransform` _index) "AlwaysSpawn" "MultiplyWithRoot" null null))
    (`Item.InitializeItemFromDataTable` (cast `Item` _returnvalue :!pure true) (`.RowName` (break `DataTableRowHandle` _itemrowhandle)) false))
  (`KismetSystemLibrary.K2_ClearAndInvalidateTimerHandle` (`self.LootTimer`)))

(event `self.PlayFlashEffect`
  (params (Strength :type "Float (single-precision)") (PlayRate :type "Float (single-precision)") (Color :type "LinearColor Structure"))
  (`MaterialInstanceDynamic.SetScalarParameterValue` (`self.DynamicSpriteInstance`) "FlashStrength" Strength)
  (`MaterialInstanceDynamic.SetVectorParameterValue` (`self.DynamicSpriteInstance`) "FlashColor" Color)
  (`TimelineComponent.SetPlayRate` (`self.FlashTimeline`) PlayRate)
  (bind (_direction _alpha) (`Timeline|FlashTimeline` :!via `PlayFromStart`)
    (:`Update`
      (`MaterialInstanceDynamic.SetScalarParameterValue` (`self.DynamicSpriteInstance`) "FlashStrength" (`KismetMathLibrary.Lerp` 0.0 Strength _alpha)))))

(event `self.PlayShakeEffect`
  (params (Strength :type "Float (single-precision)") (PlayRate :type "Float (single-precision)"))
  (set `self.RandomTrack_X` (`KismetMathLibrary.RandomIntegerInRange` 0 2))
  (set `self.RandomTrack_Z` (`KismetMathLibrary.RandomIntegerInRange` 0 2))
  (`TimelineComponent.SetPlayRate` (`self.ShakingTimeline`) PlayRate)
  (bind (_direction _1 _2 _3) (`Timeline|ShakingTimeline` :!via `PlayFromStart`)
    (:`Update`
      (`SceneComponent.K2_SetRelativeLocation` (`self.Sprite`) (+ (`KismetMathLibrary.MakeVector` (`KismetMathLibrary.Lerp` 0.0 Strength (select `int` (`self.RandomTrack_X`) :`0` _1 :`1` _2 :`2` _3 :!type "Float (double-precision)")) 0.0 (`KismetMathLibrary.Lerp` 0.0 Strength (select `int` (`self.RandomTrack_Z`) :`0` _1 :`1` _2 :`2` _3 :!type "Float (double-precision)"))) (`self.SpriteLocation`)) false false))))

(fn `GetLootRotations`
  (params (TargetArray :type "Array of LootData Structure (by ref)"))
  (returns (ReturnValue :type "Array of Rotator Structure"))
  (return (`LeyrAbilitySystemLibrary.EvenlySpacedRotators` (`self.GetActorForwardVector`) (`KismetMathLibrary.Vector_Right`) 360.0 (`KismetArrayLibrary.Array_Length` TargetArray))))

(fn `GetLootTransform`
  (params (Count :type Integer))
  (returns (ReturnValue :type "Transform Structure"))
  (bind _returnvalue (`self.K2_GetActorLocation`))
  (return (`KismetMathLibrary.MakeTransform` (`KismetMathLibrary.MakeVector` (.x (+ (* (`KismetMathLibrary.GetForwardVector` (`|GetArrayItem` (`self.LootRotations`) Count)) (`KismetMathLibrary.RandomFloatInRange` (`self.MinSpawnDistance`) (`self.MaxSpawnDistance`))) _returnvalue)) 0.0 (.z _returnvalue)))))

(fn `UserConstructionScript`)