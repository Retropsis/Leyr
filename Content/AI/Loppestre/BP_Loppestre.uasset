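; Loppestre AI creature Blueprint built on a multi-part flipbook, with its sprite snapped to the Head socket at construction.
; A ToggleTailPhysics function blends partial physics simulation into bones below TailRoot, but its only call here is disconnected.
; The timeline jump-and-return, multi-part collision binding to HandleBeginOverlap, and bubble effects in crocodile boundaries are also disconnected, leaving their entry events empty.
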(event `AIInterface.TimelineMovement`)

(event `self.ReceiveBeginPlay`)

(event `self.SetupCollisionDamage`)

(event `OnComponentBeginOverlap_Event`
  (params (OverlappedComponent :type "PrimitiveComponent Object Reference") (OtherActor :type "Actor Object Reference") (OtherComp :type "PrimitiveComponent Object Reference") (OtherBodyIndex :type Integer) (bFromSweep :type Boolean) (SweepResult :type "HitResult Structure (by ref)"))
  (`self.HandleBeginOverlap` OtherActor))

(event `self.CapsuleComponent.OnComponentBeginOverlap`
  (params (OverlappedComponent :type "PrimitiveComponent Object Reference") (OtherActor :type "Actor Object Reference") (OtherComp :type "PrimitiveComponent Object Reference") (OtherBodyIndex :type Integer) (bFromSweep :type Boolean) (SweepResult :type "HitResult Structure (by ref)")))

(event `self.CapsuleComponent.OnComponentEndOverlap`
  (params (OverlappedComponent :type "PrimitiveComponent Object Reference") (OtherActor :type "Actor Object Reference") (OtherComp :type "PrimitiveComponent Object Reference") (OtherBodyIndex :type Integer)))

(fn `ToggleTailPhysics`
  (params (Enable :type Boolean))
  (`PrimitiveComponent.SetCollisionEnabled` (`self.MultiPartFlipbook`) (select `bool` Enable :`false` "NoCollision" :`true` "PhysicsOnly" :!type "ECollisionEnabled Enum"))
  (`SkeletalMeshComponent.SetAllBodiesBelowSimulatePhysics` (`self.MultiPartFlipbook`) (`self.TailRoot`) (`local.Enable`) false)
  (`SkeletalMeshComponent.SetAllBodiesBelowPhysicsBlendWeight` (`self.MultiPartFlipbook`) (`self.TailRoot`) (select `bool` (`local.Enable`) :`true` 0.5 :!type "Float (single-precision)") false false))

(fn `UserConstructionScript`
  (`parent.UserConstructionScript`)
  (`SceneComponent.K2_AttachToComponent` (`self.Sprite`) (`self.MultiPartFlipbook`) "Head" "SnapToTarget" "SnapToTarget" "SnapToTarget" true))