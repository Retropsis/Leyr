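; BP_BoneSnake is a multi-part Paper2D bone snake AI character that scales in on spawn.
; Hit reacts swap four body flipbooks to the hit animation, restoring them when the first one's finish event fires.
; Death handling disables five collision boxes, and separate timeline events drive material dissolves.
; It also turns by yaw toward targets and spawns LootData items at random distances along X, with Y fixed at zero.
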(event `self.HandleOnAnimationFinished`
  (`self.HandleHitReactFinished`))

(event `self.PlayHitReactMontage`
  (`self.PlayHitReact`))

(event `self.HandleDeathMultiParts`
  (`PrimitiveComponent.SetCollisionEnabled` (`self.Box1`) "NoCollision")
  (`PrimitiveComponent.SetCollisionEnabled` (`self.Box`) "NoCollision")
  (`PrimitiveComponent.SetCollisionEnabled` (`self.Box3`) "NoCollision")
  (`PrimitiveComponent.SetCollisionEnabled` (`self.Box2`) "NoCollision")
  (`PrimitiveComponent.SetCollisionEnabled` (`self.Box4`) "NoCollision"))

(event `self.ReceiveBeginPlay`
  (bind (_direction _scale) (`Timeline|Timeline_1` :!via `PlayFromStart`)
    (:`Update`
      (`self.SetActorScale3D` (`KismetMathLibrary.VLerp` (0.0 0.0 0.0) (1.0 1.0 1.0) _scale))
      (add `PaperFlipbookComponent.OnFinishedPlaying` (`self.PaperFlipbook_1`) (`|CreateDelegate` :!event `HandleHitReactFinished`)))))

(event `CombatInterface.UpdateFacingTarget`
  (params (Target :type "Vector Structure (by ref)"))
  ;[1 1 1] Add Or Update MotionWarping Facing Location
  (`self.K2_SetActorRotation` (`KismetMathLibrary.MakeRotator` 0.0 0.0 (.yaw (`KismetMathLibrary.FindLookAtRotation` (`self.K2_GetActorLocation`) Target)))))

(event `CustomEvent`
  (params (DynamicMaterialInstance :type "MaterialInstanceDynamic Object Reference"))
  (bind (_direction _dissolveamount) (`Timeline|Timeline`)
    (:`Update`
      (`MaterialInstanceDynamic.SetScalarParameterValue` DynamicMaterialInstance "Dissolve" _dissolveamount))))

(event `CustomEvent_1`
  (params (DynamicMaterialInstance :type "MaterialInstanceDynamic Object Reference"))
  (bind (_direction _dissolveamount) (`Timeline|Timeline_0`)
    (:`Update`
      (`MaterialInstanceDynamic.SetScalarParameterValue` DynamicMaterialInstance "Dissolve" _dissolveamount))))

(event `self.SpawnLoot`
  (bind _lootdata (`self.LootData`))
  (`/Engine/EditorBlueprintResources/StandardMacros.IsValid` _lootdata
    (:`Is Valid`
      (bind _returnvalue (`LootDataSet.GetLootItems` _lootdata))
      (bind _output_get (set `self.LootItems` _returnvalue))
      (set `self.LootRotations` (`self.GetLootRotations` _output_get))
      (set `self.LootCount` 0)
      (bind _returnvalue_2 (`KismetSystemLibrary.K2_SetTimerDelegate` (delegate `SpawnLootItem`) 0.1 true))
      (set `self.LootTimer` _returnvalue_2)
      (`self.SpawnLootItem`))))

(event `SpawnLootItem`
  (for _index (range (`KismetArrayLibrary.Array_Length` (`self.LootItems`)))
    (bind (_itemclass _itemrowhandle) (break `LootData` (`|GetArrayItem` (`self.LootItems`) _index)))
    (bind _returnvalue (`|SpawnActorFromClass` _itemclass (`self.GetLootTransform` _index) "AlwaysSpawn" "MultiplyWithRoot" null null))
    (`Item.InitializeItemFromDataTable` (cast `Item` _returnvalue :!pure true) (`.RowName` (break `DataTableRowHandle` _itemrowhandle))))
  (`KismetSystemLibrary.K2_ClearAndInvalidateTimerHandle` (`self.LootTimer`)))

(fn `GetLootRotations`
  (params (TargetArray :type "Array of LootData Structure (by ref)"))
  (returns (ReturnValue :type "Array of Rotator Structure"))
  (return (`LeyrAbilitySystemLibrary.EvenlySpacedRotators` (`self.GetActorForwardVector`) (`KismetMathLibrary.Vector_Right`) 360.0 (`KismetArrayLibrary.Array_Length` TargetArray))))

(fn `GetLootTransform`
  (params (Count :type Integer))
  (returns (ReturnValue :type "Transform Structure"))
  (bind _returnvalue (`self.K2_GetActorLocation`))
  (return (`KismetMathLibrary.MakeTransform` (`KismetMathLibrary.MakeVector` (.x (+ (* (`KismetMathLibrary.GetForwardVector` (`|GetArrayItem` (`self.LootRotations`))) (`KismetMathLibrary.RandomFloatInRange` (`self.MinSpawnDistance`) (`self.MaxSpawnDistance`))) _returnvalue)) 0.0 (.z _returnvalue)))))

(fn `HandleHitReactFinished`
  (`|ExecutionSequence`
    (:`then_0`
      (`PaperFlipbookComponent.SetFlipbook` (`self.PaperFlipbook_1`) "/Game/Assets/Monster/BoneSnake/FB_BoneSnake_Body.FB_BoneSnake_Body"))
    (:`then_1`
      (`PaperFlipbookComponent.SetFlipbook` (`self.PaperFlipbook_2`) "/Game/Assets/Monster/BoneSnake/FB_BoneSnake_Body.FB_BoneSnake_Body"))
    (:`then_2`
      (`PaperFlipbookComponent.SetFlipbook` (`self.PaperFlipbook_3`) "/Game/Assets/Monster/BoneSnake/FB_BoneSnake_Body.FB_BoneSnake_Body"))
    (:`then_3`
      (`PaperFlipbookComponent.SetFlipbook` (`self.PaperFlipbook_4`) "/Game/Assets/Monster/BoneSnake/FB_BoneSnake_Body.FB_BoneSnake_Body"))
    (:`then_4`
      (clear `PaperFlipbookComponent.OnFinishedPlaying` (`self.PaperFlipbook_1`)))))

(fn `PlayHitReact`
  (`|ExecutionSequence`
    (:`then_0`
      (`PaperFlipbookComponent.SetFlipbook` (`self.PaperFlipbook_1`) "/Game/Assets/Monster/BoneSnake/FB_BoneSnakeBody_Hit.FB_BoneSnakeBody_Hit")
      (`PaperFlipbookComponent.SetFlipbook` (`self.PaperFlipbook_2`) "/Game/Assets/Monster/BoneSnake/FB_BoneSnakeBody_Hit.FB_BoneSnakeBody_Hit")
      (`PaperFlipbookComponent.SetFlipbook` (`self.PaperFlipbook_3`) "/Game/Assets/Monster/BoneSnake/FB_BoneSnakeBody_Hit.FB_BoneSnakeBody_Hit")
      (`PaperFlipbookComponent.SetFlipbook` (`self.PaperFlipbook_4`) "/Game/Assets/Monster/BoneSnake/FB_BoneSnakeBody_Hit.FB_BoneSnakeBody_Hit"))
    (:`then_1`
      (`PaperFlipbookComponent.SetLooping` (`self.PaperFlipbook_1`) false)
      (`PaperFlipbookComponent.SetPlayRate` (`self.PaperFlipbook_2`) 1.0)
      (`PaperFlipbookComponent.SetPlayRate` (`self.PaperFlipbook_3`) 1.0)
      (`PaperFlipbookComponent.SetPlayRate` (`self.PaperFlipbook_4`) 1.0)
      (`PaperFlipbookComponent.SetPlayRate` (`self.PaperFlipbook_1`) 1.0)
      (`PaperFlipbookComponent.Play` (`self.PaperFlipbook_1`))
      (add `PaperFlipbookComponent.OnFinishedPlaying` (`self.PaperFlipbook_1`) (`|CreateDelegate` :!event `HandleHitReactFinished`)))))

(fn `UserConstructionScript`
  (`parent.UserConstructionScript`))