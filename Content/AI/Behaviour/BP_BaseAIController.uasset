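; Base AI controller that uses AI Perception to spot the player and switch its controlled AICharacter into chasing.
; Perception updates filter for Player-tagged actors and store each last sensed stimulus, calling SightSense when the updated actor's array index is zero.
; On successful sensing, SightSense moves Patrol or Search states to Chase and sets max fly speed.
; Debug prints report whether the player is in sight.
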(event `self.AIPerception.OnPerceptionUpdated`
  (params (UpdatedActors :type "Array of Actor Object Reference (by ref)"))
  (for (_array_element _array_index) UpdatedActors
    (if (`self.ActorHasTag` _array_element "Player")
      (bind _info (`AIPerceptionComponent.GetActorsPerception` (`self.AIPerception`) _array_element))
      (for _array_element_2 (`.LastSensedStimuli` (break `ActorPerceptionBlueprintInfo` _info))
        (set `self.ActiveSense` _array_element_2)
        (switch `int` _array_index
          (:`0`
            (`self.SightSense`)))))))

(event `SightSense`
  (bind ((`StimulusLocation` _stimuluslocation) (`ReceiverLocation` _receiverlocation) (`bSuccessfullySensed` _bsuccessfullysensed)) (break `AIStimulus` (`self.ActiveSense`)))
  (bind _asaicharacter (cast `AICharacter` (`self.K2_GetPawn`) :!pure true))
  (if _bsuccessfullysensed
    (set `self.Stimulus Location` _stimuluslocation)
    (set `self.Receiver Location` _receiverlocation)
    (`KismetSystemLibrary.PrintString` "Player On Sight" true true (struct :`G` 1.0 :`B` 0.421747 :`A` 1.0) 4.0)
    (bind _returnvalue (`AICharacter.GetBehaviourState` (cast `AICharacter` (`self.K2_GetPawn`) :!pure true)))
    (switch `EBehaviourState` _returnvalue
      (:`Patrol`
        _)
      (:`Search`
        _))
    (`AICharacter.SetBehaviourState` _asaicharacter "Chase")
    (set `CharacterMovementComponent.MaxFlySpeed` 250.0 (`Character.CharacterMovement` _asaicharacter))
    (else
      (`KismetSystemLibrary.PrintString` "Player NOT On Sight" true true (struct :`R` 1.0 :`B` 0.086574 :`A` 1.0) 4.0))))

(fn `UserConstructionScript`)