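; Murdoch AI character Blueprint that supplies timeline-driven movement for a scripted jump and a defeat knockback.
; TimelineMovement disables gravity, plays a jump animation override and raises the actor to JumpApex.
; A sped-up fall timeline then lerps it to the target, restores gravity and calls CallEndTimelineMovement.
; On the Defeated tag, TimelineMovementforTag moves it backward along X with a timeline-driven Z offset, pinning Y to zero.
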(event `AIInterface.TimelineMovement`
  (params (TargetDestination :type "Vector Structure"))
  (set `self.TargetDestination` TargetDestination)
  (`|ExecutionSequence`
    (:`then_0`
      (set `CharacterMovementComponent.GravityScale` 0.0 (`self.CharacterMovement`))
      (`PaperZDAnimInstance.K2_PlayAnimationOverride` (`PaperZDAnimationComponent.AnimInstance` (`self.AnimationComponent`)) "/Game/Assets/Monster/Murdoch/AnimSequences/Murdoch_Jump.Murdoch_Jump" "DefaultSlot" 1.0 0.0))
    (:`then_1`
      (bind (_direction _jumpingupz) (`Timeline|JumpTimeline` :!via `PlayFromStart`)
        (:`Update`
          (`self.K2_SetActorLocation` (`KismetMathLibrary.MakeVector` (.x (`self.InitialTimelineLocation`)) (.y (`self.InitialTimelineLocation`)) (+ (.z (`self.InitialTimelineLocation`)) (* _jumpingupz (`self.JumpApex`))))))
        (:`Finished`
          (set `self.EndTimelineLocation` (`self.K2_GetActorLocation`))
          (`TimelineComponent.SetPlayRate` (`self.FallTimeline`) 5.0)
          (bind (_direction_2 _z) (`Timeline|FallTimeline` :!via `PlayFromStart`)
            (:`Update`
              (`self.K2_SetActorLocation` (`KismetMathLibrary.VLerp` (`self.EndTimelineLocation`) (`self.TargetDestination`) _z)))
            (:`Finished`
              (set `CharacterMovementComponent.GravityScale` (`self.BaseGravityScale`) (`self.CharacterMovement`))
              (`self.EndTimelineMovement`))))))))

(event `AIInterface.TimelineMovementForTag`
  (params (Tag :type "GameplayTag Structure (by ref)") (TargetDestination :type "Vector Structure (by ref)"))
  (bind _x (.x (`self.InitialDestroyedLocation`)))
  (bind _z (.z (`self.InitialDestroyedLocation`)))
  (`|SwitchGameplayTag` Tag
    (:`Defeated`
      (set `self.InitialDestroyedLocation` (`self.K2_GetActorLocation`))
      (`TimelineComponent.SetPlayRate` (`self.DestroyedTimeline`) 1.0)
      (bind (_direction _x_2 _z_2) (`Timeline|DestroyedTimeline` :!via `PlayFromStart`)
        (:`Update`
          (`self.K2_SetActorLocation` (`KismetMathLibrary.MakeVector` (`KismetMathLibrary.Lerp` _x (+ _x (* (.x (`self.GetActorForwardVector`)) -75.0)) _x_2) 0.0 (`KismetMathLibrary.Lerp` _z (+ _z 125.0) _z_2))))))))

(fn `UserConstructionScript`
  (`parent.UserConstructionScript`))