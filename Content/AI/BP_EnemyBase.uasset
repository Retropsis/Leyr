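; BP_EnemyBase is a base enemy Blueprint that handles spawn, facing and dissolve behavior for AI enemies.
; On BeginPlay, a timeline uniformly scales the Sprite component.
; UpdateFacingTarget, commented as a motion-warping facing update, instantly sets the actor's rotation to a yaw-only look-at toward the target.
; Separate body and weapon dissolve events each run a timeline that drives the Dissolve scalar on the supplied dynamic material instance.
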(event `self.ReceiveBeginPlay`
  (bind (_direction _scale) (`Timeline|Spawn`)
    (:`Update`
      (`SceneComponent.SetRelativeScale3D` (`self.Sprite`) (`KismetMathLibrary.MakeVector` _scale _scale _scale)))))

(event `CombatInterface.UpdateFacingTarget`
  (params (Target :type "Vector Structure (by ref)"))
  ;[1 1 1] Add Or Update MotionWarping Facing Location
  (`self.K2_SetActorRotation` (`KismetMathLibrary.MakeRotator` 0.0 0.0 (.yaw (`KismetMathLibrary.FindLookAtRotation` (`self.K2_GetActorLocation`) Target)))))

(event `self.StartDissolveTimeline`
  (params (DynamicMaterialInstance :type "MaterialInstanceDynamic Object Reference"))
  (bind (_direction _dissolveamount) (`Timeline|Dissolve`)
    (:`Update`
      (`MaterialInstanceDynamic.SetScalarParameterValue` DynamicMaterialInstance "Dissolve" _dissolveamount))))

(event `self.StartWeaponDissolveTimeline`
  (params (DynamicMaterialInstance :type "MaterialInstanceDynamic Object Reference"))
  (bind (_direction _dissolveamount) (`Timeline|Timeline`)
    (:`Update`
      (`MaterialInstanceDynamic.SetScalarParameterValue` DynamicMaterialInstance "Dissolve" _dissolveamount))))

(fn `UserConstructionScript`)