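; BP_Man-eater is a multi-part Paper2D AI enemy built from a head sprite on a socket and a chain of trunk flipbooks down to the root.
; Capsule overlaps along the body feed the overlap handler for collision damage.
; Dynamic materials ordered head to root let one timeline drive hit flashes with a separate alpha track per segment.
; Death switches trunk flipbooks to a non-looping dither, spawns combustion Niagara effects at each and disables capsule collision.
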(event `self.ReceiveBeginPlay`
  (`parent.ReceiveBeginPlay`)
  (`KismetSystemLibrary.Delay` 0.2)
  (`self.Add Flipbooks`)
  (`KismetArrayLibrary.Array_Add` (`self.DMI_First`) (`self.DynamicSpriteInstance`))
  (for _array_element (`self.Flipbooks`)
    (bind _returnvalue (`PrimitiveComponent.CreateDynamicMaterialInstance` _array_element 0 null "None"))
    (`KismetArrayLibrary.Array_Add` (`self.DMI_First`) _returnvalue)))

(event `self.SetupCollisionDamage`
  (add `PrimitiveComponent.OnComponentBeginOverlap` (`self.Capsule_Root`) (delegate `OnComponentBeginOverlap_Event`))
  (add `PrimitiveComponent.OnComponentBeginOverlap` (`self.Capsule_1`) (delegate `OnComponentBeginOverlap_Event`))
  (add `PrimitiveComponent.OnComponentBeginOverlap` (`self.Capsule_2`) (delegate `OnComponentBeginOverlap_Event`))
  (add `PrimitiveComponent.OnComponentBeginOverlap` (`self.Capsule_3`) (delegate `OnComponentBeginOverlap_Event`))
  (add `PrimitiveComponent.OnComponentBeginOverlap` (`self.Capsule_4`) (delegate `OnComponentBeginOverlap_Event`))
  (add `PrimitiveComponent.OnComponentBeginOverlap` (`self.Capsule_5`) (delegate `OnComponentBeginOverlap_Event`))
  (add `PrimitiveComponent.OnComponentBeginOverlap` (`self.Capsule_6`) (delegate `OnComponentBeginOverlap_Event`))
  (add `PrimitiveComponent.OnComponentBeginOverlap` (`self.Capsule_7`) (delegate `OnComponentBeginOverlap_Event`)))

(event `OnComponentBeginOverlap_Event`
  (params (OverlappedComponent :type "PrimitiveComponent Object Reference") (OtherActor :type "Actor Object Reference") (OtherComp :type "PrimitiveComponent Object Reference") (OtherBodyIndex :type Integer) (bFromSweep :type Boolean) (SweepResult :type "HitResult Structure (by ref)"))
  (`self.HandleBeginOverlap` OtherActor))

(event `self.PlayFlashEffect`
  (params (Strength :type "Float (single-precision)") (PlayRate :type "Float (single-precision)") (Color :type "LinearColor Structure"))
  (`MaterialInstanceDynamic.SetScalarParameterValue` (`self.DynamicSpriteInstance`) "FlashStrength" Strength)
  (`MaterialInstanceDynamic.SetVectorParameterValue` (`self.DynamicSpriteInstance`) "FlashColor" Color)
  (`TimelineComponent.SetPlayRate` (`self.FirstTimeline`) PlayRate)
  (bind (_direction _alpha_head _alpha_7 _alpha_6 _alpha_5 _alpha_4 _alpha_3 _alpha_2 _alpha_1 _alpha_root) (`Timeline|FirstTimeline` :!via `PlayFromStart`)
    (:`Update`
      (for (_array_element _array_index) (`self.DMI_First`)
        (`MaterialInstanceDynamic.SetScalarParameterValue` _array_element "FlashStrength" (`KismetMathLibrary.Lerp` 0.0 Strength (select `int` _array_index :`0` _alpha_head :`1` _alpha_7 :`2` _alpha_6 :`3` _alpha_5 :`4` _alpha_4 :`5` _alpha_3 :`6` _alpha_2 :`7` _alpha_1 :`8` _alpha_root)))))))

(event `self.HandleDeathMultiParts`
  (for _array_element (`self.Flipbooks`)
    (`PaperFlipbookComponent.SetFlipbook` _array_element "/Game/Assets/Monster/Dorn_Maneater/Dorn_Man-eater_Trunk_Dither.Dorn_Man-eater_Trunk_Dither")
    (`PaperFlipbookComponent.SetLooping` _array_element false)
    (`NiagaraFunctionLibrary.SpawnSystemAtLocation` "/Game/Effects/Combustion/NS_Combustion_01.NS_Combustion_01" (`KismetMathLibrary.MakeVector` (.x (`SceneComponent.K2_GetComponentLocation` _array_element)) 10.0 (.z (`SceneComponent.K2_GetComponentLocation` _array_element)))))
  (`PrimitiveComponent.SetCollisionEnabled` (`self.Capsule_Root`) "NoCollision")
  (`PrimitiveComponent.SetCollisionEnabled` (`self.Capsule_1`) "NoCollision")
  (`PrimitiveComponent.SetCollisionEnabled` (`self.Capsule_2`) "NoCollision")
  (`PrimitiveComponent.SetCollisionEnabled` (`self.Capsule_3`) "NoCollision")
  (`PrimitiveComponent.SetCollisionEnabled` (`self.Capsule_4`) "NoCollision")
  (`PrimitiveComponent.SetCollisionEnabled` (`self.Capsule_5`) "NoCollision")
  (`PrimitiveComponent.SetCollisionEnabled` (`self.Capsule_6`) "NoCollision")
  (`PrimitiveComponent.SetCollisionEnabled` (`self.Capsule_7`) "NoCollision")
  (`PrimitiveComponent.SetCollisionEnabled` (`self.Capsule_Head`) "NoCollision"))

(fn `Add Flipbooks`
  (`KismetArrayLibrary.Array_Add` (`self.Flipbooks`) (`self.PaperFlipbook_7`))
  (`KismetArrayLibrary.Array_Add` (`self.Flipbooks`) (`self.PaperFlipbook_6`))
  (`KismetArrayLibrary.Array_Add` (`self.Flipbooks`) (`self.PaperFlipbook_5`))
  (`KismetArrayLibrary.Array_Add` (`self.Flipbooks`) (`self.PaperFlipbook_4`))
  (`KismetArrayLibrary.Array_Add` (`self.Flipbooks`) (`self.PaperFlipbook_3`))
  (`KismetArrayLibrary.Array_Add` (`self.Flipbooks`) (`self.PaperFlipbook_2`))
  (`KismetArrayLibrary.Array_Add` (`self.Flipbooks`) (`self.PaperFlipbook_1`))
  (`KismetArrayLibrary.Array_Add` (`self.Flipbooks`) (`self.PaperFlipbook_Root`)))

(fn `UserConstructionScript`
  (`SceneComponent.K2_AttachToComponent` (`self.Sprite`) (`self.MultiPartFlipbook`) "Head" "KeepRelative" "KeepRelative" "KeepRelative" true))