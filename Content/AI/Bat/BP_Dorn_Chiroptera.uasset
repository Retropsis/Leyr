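; Bat enemy Blueprint that moves by timelines in the X-Z plane, adding sine flight and dive movement to its parent class.
; SineMove lerps between start and end points with a scaled sine offset on Z, checks for an end condition each update, and restarts when finished.
; TimelineMovement targets a point JumpApex below the bat, lerps its location there via the BatDive curve, then calls CallEndTimelineMovement.
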(event `AIInterface.SineMove`
  (`self.InitializeSineMove`)
  (bind (_direction _x _sinez) (`Timeline|SineTimeline` :!via `PlayFromStart`)
    (:`Update`
      (`self.K2_SetActorLocation` (`KismetMathLibrary.MakeVector` (.x (`KismetMathLibrary.VLerp` (`self.InitialTimelineLocation`) (`self.EndTimelineLocation`) _x)) 0.0 (+ (.z (`KismetMathLibrary.VLerp` (`self.InitialTimelineLocation`) (`self.EndTimelineLocation`) _x)) (* _sinez (`self.SineAmplitude`)))))
      (`self.ShouldEndSineMove` (`self.SineTimeline`)))
    (:`Finished`
      (`AIInterface.SineMove`))))

(event `AIInterface.TimelineMovement`
  (set `self.EndTimelineLocation` (`KismetMathLibrary.MakeVector` (.x (`self.K2_GetActorLocation`)) 0.0 (- (.z (`self.K2_GetActorLocation`)) (`self.JumpApex`))))
  (bind (_direction _flyz) (`Timeline|BatDive` :!via `PlayFromStart`)
    (:`Update`
      (`self.K2_SetActorLocation` (`KismetMathLibrary.VLerp` (`self.InitialTimelineLocation`) (`self.EndTimelineLocation`) _flyz)))
    (:`Finished`
      (`self.EndTimelineMovement`))))

(fn `UserConstructionScript`
  (`parent.UserConstructionScript`))