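; Player character Blueprint that handles attack-agnostic facing updates and a colored sprite flash effect.
; UpdateFacingTarget feeds a location into the Motion Warping component as the FacingTarget warp target.
; PlayFlashEffect sets flash color and strength on the dynamic sprite material, then replays a timeline at the given rate to interpolate strength between zero and the requested value.
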(event `CombatInterface.UpdateFacingTarget`
  (params (Target :type "Vector Structure (by ref)"))
  (`MotionWarpingComponent.AddOrUpdateWarpTargetFromLocation` (`self.MotionWarping`) "FacingTarget" Target))

(event `self.PlayFlashEffect`
  (params (Strength :type "Float (single-precision)") (PlayRate :type "Float (single-precision)") (Color :type "LinearColor Structure"))
  (`MaterialInstanceDynamic.SetScalarParameterValue` (`self.DynamicSpriteInstance`) "FlashStrength" Strength)
  (`MaterialInstanceDynamic.SetVectorParameterValue` (`self.DynamicSpriteInstance`) "FlashColor" Color)
  (`TimelineComponent.SetPlayRate` (`self.FlashTimeline`) PlayRate)
  (bind (_direction _alpha) (`Timeline|FlashTimeline` :!via `PlayFromStart`)
    (:`Update`
      (`MaterialInstanceDynamic.SetScalarParameterValue` (`self.DynamicSpriteInstance`) "FlashStrength" (`KismetMathLibrary.Lerp` 0.0 Strength _alpha)))))

(fn `UserConstructionScript`)