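; Player controller that owns the local player's main UI layout and bridges inventory changes to its widgets.
; BeginPlay creates the root layout, pushes the HUD, then pushes and deactivates the inventory layout to initialise it.
; Toggle events open the inventory, optionally with a container window sized by slot count; container-closing logic is unconnected.
; Slot update and reset events relay through Client events to grid widgets, resolved only for the Inventory container type.
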(event `self.ReceiveBeginPlay`
  (`/Engine/EditorBlueprintResources/ActorMacros.Switch Has Authority`
    (:`Authority`
      (if (`self.IsLocalPlayerController`)
        (bind _returnvalue (`|CreateWidget` "/Game/UI/Inventory/CU_MainUILayout.CU_MainUILayout_C" self :!label _label))
        (bind _output_get (set `self.RootLayout` _returnvalue))
        (`UserWidget.AddToViewport` _output_get 0)
        (`/Game/UI/Inventory/CU_MainUILayout.PushDefaultHUDLayout` (`self.RootLayout`))
        (`self.InitializeInventoryWidget`)))
    (:`Remote`
      (goto _label))))

(event `self.ToggleInventory`
  (if (not (`self.bIsInventoryOpen`)) :!label _label_2
    (`/Game/UI/Inventory/CU_MainUILayout.PushInventoryLayout` (`self.RootLayout`)))
  (`self.ToggleInputMode`))

(event `ControllerInterface.CloseInventory`
  (goto _label_2))

(event `ToggleMainInventory`)

(event `ControllerInterface.ToggleContainer`
  (params (SlotCount :type Integer))
  (if (not (`self.bIsContainerOpen`))
    (`/Game/UI/Inventory/WBP_Inventory.SetContainerWindow` (`/Game/UI/Inventory/CU_InventoryLayout.WBP_Inventory` (`/Game/UI/Inventory/CU_MainUILayout.InventoryLayout` (`self.RootLayout`))) SlotCount "Visible")
    (set `self.bIsContainerOpen` true)
    (`self.ToggleInventory`)))

(event `ControllerInterface.UpdateInventorySlot`
  (params (ContainerType :type "EContainerType Enum" :default "Inventory") (SlotIndex :type Integer) (ItemData :type "InventoryItemData Structure"))
  (`self.ClientUpdateInventorySlot` ContainerType SlotIndex ItemData))

(event `ClientUpdateInventorySlot`
  (params (ContainerType :type "EContainerType Enum" :default "Inventory") (SlotIndex :type Integer) (ItemData :type "InventoryItemData Structure"))
  (bind _inventoryslot (`self.GetInventoryWidget` ContainerType SlotIndex))
  (`/Engine/EditorBlueprintResources/StandardMacros.IsValid` _inventoryslot
    (:`Is Valid`
      (`/Game/UI/Inventory/WBP_InventorySlot.UpdateInventorySlot` _inventoryslot ItemData))))

(event `ControllerInterface.ResetInventorySlot`
  (params (ContainerType :type "EContainerType Enum" :default "Inventory") (SlotIndex :type Integer))
  (`self.ClientResetInventorySlot` ContainerType SlotIndex))

(event `ClientResetInventorySlot`
  (params (ContainerType :type "EContainerType Enum" :default "Inventory") (SlotIndex :type Integer))
  (bind _inventoryslot (`self.GetInventoryWidget` ContainerType SlotIndex))
  (`/Engine/EditorBlueprintResources/StandardMacros.IsValid` _inventoryslot
    (:`Is Valid`
      (`/Game/UI/Inventory/WBP_InventorySlot.ResetInventorySlot` _inventoryslot))))

(fn `GetInventoryWidget`
  (params (ContainerType :type "EContainerType Enum" :default "Inventory") (SlotIndex :type Integer))
  (returns (InventorySlot :type "/Game/UI/Inventory/WBP_InventorySlot Object Reference"))
  (switch `EContainerType` ContainerType
    (:`Inventory`
      (return (`|GetArrayItem` (`/Game/UI/Inventory/WBP_InventoryGrid.Slots` (`/Game/UI/Inventory/WBP_Inventory.WBP_InventoryGrid` (`/Game/UI/Inventory/CU_InventoryLayout.WBP_Inventory` (`/Game/UI/Inventory/CU_MainUILayout.InventoryLayout` (`self.RootLayout`))))) (`local.SlotIndex`))))))

(fn `InitializeInventoryWidget`
  (`/Game/UI/Inventory/CU_MainUILayout.PushInventoryLayout` (`self.RootLayout`))
  (set `self.bIsInventoryOpen` true)
  (bind _inventorylayout (`/Game/UI/Inventory/CU_MainUILayout.InventoryLayout` (`self.RootLayout`))
    (:`then`
      (`CommonActivatableWidget.DeactivateWidget` _inventorylayout))
    (:`else`)))

(fn `UserConstructionScript`)