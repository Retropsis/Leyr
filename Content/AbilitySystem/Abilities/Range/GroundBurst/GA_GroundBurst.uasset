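; Ranged gameplay ability for a 2D Paper character that fires a GroundBurst projectile attack.
; On activation it initializes, plays the GroundBurst animation override and waits once for the Montage.Attack.1 gameplay event.
; That event spawns a projectile at the weapon socket, aimed horizontally along the avatar's forward X with target Y flattened to zero.
; Animation completion or cancellation ends the ability, and OnEndAbility runs PrepareToEndAbility.
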(event `self.K2_OnEndAbility`
  (params (bWasCancelled :type Boolean))
  (`self.PrepareToEndAbility`))

(event `self.K2_ActivateAbility`
  (`self.InitAbility`)
  (`PaperZDPlaySlotOverrideAction.PlayAnimationOverrideWithCallbacks` (`self.PaperAnimInstance`) "/Game/AI/TheScourge/AnimSequences/GroundBurst.GroundBurst"
    (:`then`
      (`AbilityTask_WaitGameplayEvent.WaitGameplayEvent` (struct :`TagName` "Montage.Attack.1") null true
        (:`EventReceived`
          (bind _returnvalue (message `CombatInterface.GetCombatSocketLocation` (`self.GetAvatarActorFromActorInfo`) (`BlueprintGameplayTagLibrary.MakeLiteralGameplayTag` (struct :`TagName` "CombatSocket.Weapon"))))
          (`self.SpawnProjectile` (`BlueprintGameplayTagLibrary.MakeLiteralGameplayTag` (struct :`TagName` "CombatSocket.Weapon")) (`KismetMathLibrary.MakeVector` (+ (.x _returnvalue) (* (.x (`Actor.GetActorForwardVector` (`self.GetAvatarActorFromActorInfo`))) 100.0)) 0.0 (.z _returnvalue))))))
    (:`OnCompleted`
      (`self.K2_EndAbility` :!label _label))
    (:`OnCancelled`
      (goto _label))))