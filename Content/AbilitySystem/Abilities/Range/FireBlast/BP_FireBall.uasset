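; Boomerang-style fireball actor for the FireBlast ability that flies out, returns to its instigator and explodes on arrival.
; On the server, an outgoing timeline lerps it forward to an apex, then a returning timeline homes it on the instigator's current location.
; Within explode distance it calls OnHit, applies radial damage effects with outward airborne knockback to nearby live players except the instigator, and destroys itself.
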(event `self.StartOutgoingTimeline`
  (`/Engine/EditorBlueprintResources/ActorMacros.Switch Has Authority`
    (:`Authority`
      (set `self.InitialLocation` (`self.K2_GetActorLocation`))
      (set `self.ApexLocation` (+ (`self.InitialLocation`) (* (`self.GetActorForwardVector`) (`self.TravelDistance`))))
      (bind (_direction _outgoingtrack) (`Timeline|OutgoingTimeline`)
        (:`Update`
          (`self.K2_SetActorLocation` (`KismetMathLibrary.VLerp` (`self.InitialLocation`) (`self.ApexLocation`) _outgoingtrack)))
        (:`Finished`
          (`self.K2_SetActorRotation` (`KismetMathLibrary.Conv_VectorToRotator` (* (`self.GetActorForwardVector`) -1.0)))
          (bind (_direction_2 _outgoingtrack_2) (`Timeline|ReturningTimeline` :!via `PlayFromStart`)
            (:`Update`
              (`self.K2_SetActorLocation` (`KismetMathLibrary.VLerp` (`self.ApexLocation`) (`self.K2_GetActorLocation` (`self.Instigator`)) _outgoingtrack_2))
              (if (`self.IsWithinExplodeDistance`)
                (`self.OnHit`)
                (`LeyrAbilitySystemLibrary.SetIsRadialDamageEffectParam` (`self.ExplosionDamageParams`) true 30.0 125.0 (`self.K2_GetActorLocation`))
                (bind _outoverlappingactors (`LeyrAbilitySystemLibrary.GetLivePlayersWithinRadius` (`|MakeArray` (`self.Instigator`) self :!type "Actor Object Reference") 125.0 (`self.K2_GetActorLocation`)))
                (for _array_element _outoverlappingactors
                  (setmembers `AdditionalEffectParams` :`StructRef` (`self.ExplosionDamageParams`) :`TargetAbilitySystemComponent` (`AbilitySystemBlueprintLibrary.GetAbilitySystemComponent` _array_element))
                  (`LeyrAbilitySystemLibrary.SetAirborneDirection` (`self.ExplosionDamageParams`) (- (`self.K2_GetActorLocation` _array_element) (`self.K2_GetActorLocation`)) 150.0)
                  (`LeyrAbilitySystemLibrary.ApplyAdditionalEffect` (`self.ExplosionDamageParams`)))
                (`self.K2_DestroyActor`)))))))))

(fn `IsWithinExplodeDistance`
  (returns (ReturnValue :type Boolean))
  (return (<= (`KismetMathLibrary.VSize` (- (`self.K2_GetActorLocation`) (`self.K2_GetActorLocation` (`self.Instigator`)))) (`self.ExplodeDistance`))))

(fn `UserConstructionScript`)