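; BP_Boomerang is a ranged ability boomerang actor that flies from its initial location to an apex and back.
; StartOutgoingTimeline runs on authority only, chaining outgoing and return timelines that lerp the actor's location without sweeping.
; When the return finishes, it calls OutgoingTimelineEnd, then starts a self-restarting timeline that spins the Boomerang component in pitch.
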(event `self.StartOutgoingTimeline`
  (`/Engine/EditorBlueprintResources/ActorMacros.Switch Has Authority`
    (:`Authority`
      (bind (_direction _outgoingtrack) (`Timeline|BoomerangTimeline`)
        (:`Update`
          (`self.K2_SetActorLocation` (`KismetMathLibrary.VLerp` (`self.InitialLocation`) (`self.ApexLocation`) _outgoingtrack)))
        (:`Finished`
          (bind (_direction_2 _outgoingtrack_2) (`Timeline|BoomerangTimelineReturn` :!via `PlayFromStart`)
            (:`Update`
              (`self.K2_SetActorLocation` (`KismetMathLibrary.VLerp` (`self.ApexLocation`) (`self.InitialLocation`) _outgoingtrack_2)))
            (:`Finished`
              (`self.OutgoingTimelineEnd`)
              (bind (_direction_3 _outgoingtrack_3) (`Timeline|Timeline` :!via `PlayFromStart` :!label _label)
                (:`Update`
                  (`SceneComponent.K2_SetRelativeRotation` (`self.Boomerang`) (`KismetMathLibrary.MakeRotator` 0.0 (* _outgoingtrack_3 -1800.0)) false false))
                (:`Finished`
                  (goto _label :!via `PlayFromStart`))))))))))

(fn `UserConstructionScript`)