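; Kunai projectile Blueprint for a ranged ability that animates the kunai after a hit.
; OnHitTimeline starts two timelines: one spins the actor in pitch, the other lerps it from its stored hit-animation start location to a target location, named as a backward move.
; When the movement timeline finishes, it calls PrepareToDestroyProjectile.
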(event `self.OnHitTimeline`
  (`|ExecutionSequence`
    (:`then_0`
      (bind (_direction _yaw) (`Timeline|Rotate` :!via `PlayFromStart`)
        (:`Update`
          (`self.K2_SetActorRotation` (`KismetMathLibrary.MakeRotator` 0.0 (* _yaw 1080.0))))))
    (:`then_1`
      (bind (_direction_2 _alpha) (`Timeline|MovingBackward` :!via `PlayFromStart`)
        (:`Update`
          (`self.K2_SetActorLocation` (`KismetMathLibrary.VLerp` (`self.InitialOnHitTimeline`) (`self.TargetLocation`) _alpha)))
        (:`Finished`
          (`self.PrepareToDestroyProjectile`))))))

(fn `UserConstructionScript`)