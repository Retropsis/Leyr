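; Ranged attack gameplay ability for AI characters that picks its 2D animation from the avatar's behaviour state and fires a projectile.
; It faces the combat target, or a point just ahead when none exists, and uses that location as the aim.
; Only Patrol and Duck map to attack montages.
; The montage's gameplay event tag triggers the projectile spawn at its socket, and animation completion or cancellation ends the ability.
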(event `self.K2_ActivateAbility`
  (bind _returnvalue (`self.GetAvatarActorFromActorInfo`))
  (`self.InitAbility`)
  (bind _returnvalue_2 (message `EnemyInterface.GetCombatTarget` (`self.GetAvatarActorFromActorInfo`)))
  (`/Engine/EditorBlueprintResources/StandardMacros.IsValid` _returnvalue_2
    (:`Is Valid`
      (set `self.bHasTarget` true)
      (bind _output_get (set `self.TargetLocation` (`Actor.K2_GetActorLocation` _returnvalue_2)))
      (message `CombatInterface.UpdateFacingTarget` (`self.GetAvatarActorFromActorInfo`) _output_get))
    (:`Is Not Valid`
      (bind _output_get_2 (set `self.TargetLocation` (+ (`Actor.K2_GetActorLocation` _returnvalue) (* (`Actor.GetActorForwardVector` _returnvalue) 50.0))))
      (message `CombatInterface.UpdateFacingTarget` _returnvalue _output_get_2)))
  (bind _returnvalue_3 (message `CombatInterface.GetPaperAnimInstance` (`self.GetAvatarActorFromActorInfo`)))
  (bind _returnvalue_4 (message `CombatInterface.GetAttackMontages` (`self.GetAvatarActorFromActorInfo`) "Default"))
  (bind _asaicharacter (cast `AICharacter` (`self.GetAvatarActorFromActorInfo`)))
  (bind _returnvalue_5 (`AICharacter.GetBehaviourState` _asaicharacter))
  (bind _output_get_3 (set `self.TaggedMontage` (select `EBehaviourState` _returnvalue_5 :`Patrol` (`|GetArrayItem` _returnvalue_4) :`Duck` (`|GetArrayItem` _returnvalue_4 1))))
  (bind ((`MontageTag` _montagetag) (`SocketTag` _sockettag) (`Montage` _montage)) (break `TaggedMontage` _output_get_3))
  (`PaperZDPlaySlotOverrideAction.PlayAnimationOverrideWithCallbacks` _returnvalue_3 _montage
    (:`then`
      (`AbilityTask_WaitGameplayEvent.WaitGameplayEvent` _montagetag null true
        (:`EventReceived`
          (`self.SpawnProjectile` _sockettag (`self.TargetLocation`)))))
    (:`OnCompleted`
      (`self.K2_EndAbility` :!label _label))
    (:`OnCancelled`
      (goto _label))))