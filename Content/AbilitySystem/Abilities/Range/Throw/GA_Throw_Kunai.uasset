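; Gameplay ability that throws a kunai as a projectile.
; On activation it picks a Paper animation from the combat state and plays it as an override, ending at once if none is valid.
; A one-shot Montage.Throwing gameplay event spawns the projectile from the weapon socket toward the target location, and animation completion or cancellation ends the ability.
; The inventory cost commit is left unconnected and never runs.
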(event `self.K2_OnEndAbility`
  (params (bWasCancelled :type Boolean))
  (`self.PrepareToEndAbility`))

(event `self.K2_ActivateAbility`
  (`self.InitAbility`)
  (`self.SelectMontageTagFromCombatState`)
  (`self.SetCurrentSequence`)
  (`/Engine/EditorBlueprintResources/StandardMacros.IsValid` (`self.SelectedMontage`)
    (:`Is Valid`
      (`PaperZDPlaySlotOverrideAction.PlayAnimationOverrideWithCallbacks` (`self.PaperAnimInstance`) (`self.SelectedMontage`)
        (:`then`
          (`AbilityTask_WaitGameplayEvent.WaitGameplayEvent` (struct :`TagName` "Montage.Throwing") null true
            (:`EventReceived`
              (`self.SpawnProjectile` (`BlueprintGameplayTagLibrary.MakeLiteralGameplayTag` (struct :`TagName` "CombatSocket.Weapon")) (`self.TargetLocation`)))))
        (:`OnCompleted`
          (`self.K2_EndAbility` :!label _label))
        (:`OnCancelled`
          (goto _label))))
    (:`Is Not Valid`
      (`self.K2_EndAbility`))))