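; GA_Throw is a ranged gameplay ability that plays a character throw animation and spawns a projectile toward a target location.
; While the Paper2D animation override plays, it waits once for the Montage.Throwing gameplay event, then spawns the projectile from the weapon combat socket.
; The ability ends when the animation completes or is cancelled, and an inventory cost commit node is left unconnected.
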(event `self.K2_OnEndAbility`
  (params (bWasCancelled :type Boolean))
  (`self.PrepareToEndAbility`))

(event `self.K2_ActivateAbility`
  (`self.InitAbility`)
  (`PaperZDPlaySlotOverrideAction.PlayAnimationOverrideWithCallbacks` (`self.PaperAnimInstance`) "/Game/Assets/Character/AnimSequences/Character_Throw.Character_Throw"
    (:`then`
      (`AbilityTask_WaitGameplayEvent.WaitGameplayEvent` (struct :`TagName` "Montage.Throwing") null true
        (:`EventReceived`
          (`self.SpawnProjectile` (`BlueprintGameplayTagLibrary.MakeLiteralGameplayTag` (struct :`TagName` "CombatSocket.Weapon")) (`self.TargetLocation`)))))
    (:`OnCompleted`
      (`self.K2_EndAbility` :!label _label))
    (:`OnCancelled`
      (goto _label))))