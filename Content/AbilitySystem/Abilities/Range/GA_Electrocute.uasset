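; Electrocute ranged Gameplay Ability: a channeled beam with chained targets that lasts until input release.
; It plays a Paper animation override and, as the event wait starts, fires a burst cue and adds looping cues and debug spheres to additional targets.
; The Electrocute event sets Casting state and traces the main beam's target.
; Ending removes the cues; cursor targeting is unconnected and no damage is applied here.
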(event `self.K2_OnEndAbility`
  (params (bWasCancelled :type Boolean))
  (`self.PrepareToEndAbility`)
  (message `CombatInterface.SetCombatStateToHandle` (`self.GetAvatarActorFromActorInfo`) "Unoccupied")
  (`GameplayCueFunctionLibrary.RemoveGameplayCueOnActor` (select `bool` (`self.FirstTargetImplementsInterface`) :`false` (`self.GetAvatarActorFromActorInfo`) :`true` (`self.MouseHitActor`)) (struct :`TagName` "GameplayCue.Electrocute.Loop") (`self.FirstTargetCueParams`))
  (if (`self.FirstTargetImplementsInterface`)
    (bind _keys (`BlueprintMapLibrary.Map_Keys` (`self.AdditionalTargetsToCueParams`)))
    (for _array_element _keys
      (`GameplayCueFunctionLibrary.RemoveGameplayCueOnActor` _array_element (struct :`TagName` "GameplayCue.Electrocute.Loop") (`BlueprintMapLibrary.Map_Find` (`self.AdditionalTargetsToCueParams`) _array_element)))))

(event `self.K2_ActivateAbility`
  (`self.InitAbility`)
  (bind _output_get (set `self.FirstTargetImplementsInterface` (`KismetSystemLibrary.DoesImplementInterface` (`self.GetAvatarActorFromActorInfo`) "/Script/Leyr.CombatInterface")))
  (if _output_get
    (`self.StoreOwnerVariables`)
    (`|ExecutionSequence`
      (:`then_0`
        (message `CombatInterface.UpdateFacingTarget` (`self.GetAvatarActorFromActorInfo`) (`Actor.GetActorForwardVector` (`self.GetAvatarActorFromActorInfo`)))
        (bind _returnvalue (message `CombatInterface.GetPaperAnimInstance` (`self.GetAvatarActorFromActorInfo`)))
        (`PaperZDPlaySlotOverrideAction.PlayAnimationOverrideWithCallbacks` _returnvalue "/Game/Assets/Character/AnimSequences/Casting.Casting"
          (:`then`
            (`AbilityTask_WaitGameplayEvent.WaitGameplayEvent` (struct :`TagName` "Event.Montage.Electrocute") null true
              (:`then`
                (`self.K2_ExecuteGameplayCue` (struct :`TagName` "GameplayCue.Electrocute"))
                (if (`self.FirstTargetImplementsInterface`)
                  (bind _outadditionaltargets (`self.StoreAdditionalTargets`))
                  (for _array_element _outadditionaltargets
                    (`KismetSystemLibrary.DrawDebugSphere` (`Actor.K2_GetActorLocation` _array_element) 15.0 12 (struct :`R` 1.0 :`G` 1.0 :`B` 1.0 :`A` 1.0) 8.0)
                    (`self.AddCuesToAdditionalTargets` _array_element))))
              (:`EventReceived`
                (message `CombatInterface.SetCombatStateToHandle` (`self.GetAvatarActorFromActorInfo`) "Casting")
                (`self.SpawnBeam`))))))
      (:`then_1`
        (`AbilityTask_WaitInputRelease.WaitInputRelease` false
          (:`OnRelease`
            (`CharacterMovementComponent.SetMovementMode` (`Character.CharacterMovement` (`self.OwnerCharacter`)) "MOVE_Walking" 0)
            (`self.K2_EndAbility`)))))
    (else
      (`self.K2_EndAbility`))))

(fn `AddCuesToAdditionalTargets`
  (params (AdditionalTarget :type "Actor Object Reference"))
  (bind _additionaltarget (`local.AdditionalTarget`))
  (bind _returnvalue (`AbilitySystemBlueprintLibrary.MakeGameplayCueParameters` 0.0 0.0 (struct) (struct) (struct) (struct) (struct) (`Actor.K2_GetActorLocation` _additionaltarget) (0.0 0.0 0.0) null null _additionaltarget null 1 1 (`Actor.RootComponent` (`self.MouseHitActor`))))
  (`BlueprintMapLibrary.Map_Add` (`self.AdditionalTargetsToCueParams`) AdditionalTarget _returnvalue)
  (`GameplayCueFunctionLibrary.AddGameplayCueOnActor` (`local.AdditionalTarget`) (struct :`TagName` "GameplayCue.Electrocute.Loop") _returnvalue))

(fn `SpawnBeam`
  (locals (CueTarget :type "Actor Object Reference"))
  (`self.TraceFirstTarget` (`Actor.K2_GetActorLocation` (`self.GetAvatarActorFromActorInfo`)))
  (set `self.FirstTargetCueParams` (`AbilitySystemBlueprintLibrary.MakeGameplayCueParameters` 0.0 0.0 (struct) (struct) (struct) (struct) (struct) (`Actor.K2_GetActorLocation` (`self.GetAvatarActorFromActorInfo`)) (0.0 0.0 0.0) null null (`self.MouseHitActor`) null 1 1 (`Actor.RootComponent` (`self.GetAvatarActorFromActorInfo`))))
  (if (`KismetSystemLibrary.DoesImplementInterface` (`self.MouseHitActor`) "/Script/Leyr.CombatInterface")
    (set `local.CueTarget` (`self.MouseHitActor`))
    (else
      (set `local.CueTarget` (`self.GetAvatarActorFromActorInfo`))))
  (`GameplayCueFunctionLibrary.AddGameplayCueOnActor` (`local.CueTarget`) (struct :`TagName` "GameplayCue.Electrocute.Loop") (`self.FirstTargetCueParams`)))