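; GA_RangeAttack is a gameplay ability that performs a ranged attack for its avatar using Paper animation.
; On activation it turns the avatar toward its combat target and plays a random attack montage of the configured sequence type as an animation override.
; The montage's gameplay event tag triggers SpawnProjectile from the montage's socket toward the target's current location, with optional pitch override.
; The ability ends when the animation completes or is cancelled.
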(event `self.K2_ActivateAbility`
  (bind _returnvalue (`self.GetAvatarActorFromActorInfo`))
  (bind _returnvalue_2 (message `EnemyInterface.GetCombatTarget` _returnvalue))
  (message `CombatInterface.UpdateFacingTarget` _returnvalue (`Actor.K2_GetActorLocation` _returnvalue_2))
  (bind _returnvalue_3 (message `CombatInterface.GetPaperAnimInstance` _returnvalue))
  (bind _returnvalue_4 (message `CombatInterface.GetAttackMontages` _returnvalue (`self.SequenceType`)))
  (bind _output_get (set `self.TaggedMontage` (`KismetArrayLibrary.Array_Random` _returnvalue_4)))
  (bind (_abilitypower _damagetype _montagetag _sockettag _montage) (break `TaggedMontage` _output_get))
  (`PaperZDPlaySlotOverrideAction.PlayAnimationOverrideWithCallbacks` _returnvalue_3 _montage
    (:`then`
      (`AbilityTask_WaitGameplayEvent.WaitGameplayEvent` _montagetag null true
        (:`then`
          (message `CombatInterface.GetCombatSocketLocation` (`self.GetAvatarActorFromActorInfo`) _sockettag)
          (bind _returnvalue_5 (message `EnemyInterface.GetCombatTarget` (`self.GetAvatarActorFromActorInfo`)))
          (`self.SpawnProjectile` (`Actor.K2_GetActorLocation` _returnvalue_5) _sockettag (`self.OverridePitch`) (`self.PitchOverride`)))))
    (:`OnCompleted`
      (`self.K2_EndAbility` :!label _label))
    (:`OnCancelled`
      (goto _label))))