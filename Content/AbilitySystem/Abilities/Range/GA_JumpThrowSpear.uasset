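; Gameplay ability for a ranged spear throw, named for a jump attack, that fires a projectile in the avatar's facing direction.
; It gets the anim instance and a random tagged attack montage through avatar message calls, then plays it as a Paper animation override.
; The montage's gameplay event triggers SpawnProjectile once, using its socket tag, a point ahead of the avatar and optional pitch override.
; The ability ends when the animation completes or is cancelled.
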(event `self.K2_ActivateAbility`
  (bind _returnvalue (`self.GetAvatarActorFromActorInfo`))
  (bind _returnvalue_2 (`self.GetAvatarActorFromActorInfo`))
  (bind _returnvalue_3 (message `CombatInterface.GetPaperAnimInstance` _returnvalue_2))
  (bind _returnvalue_4 (message `CombatInterface.GetAttackMontages` _returnvalue_2))
  (bind _output_get (set `self.TaggedMontage` (`KismetArrayLibrary.Array_Random` _returnvalue_4)))
  (bind (_abilitypower _damagetype _montagetag _sockettag _montage) (break `TaggedMontage` _output_get))
  (`PaperZDPlaySlotOverrideAction.PlayAnimationOverrideWithCallbacks` _returnvalue_3 _montage
    (:`then`
      (`AbilityTask_WaitGameplayEvent.WaitGameplayEvent` _montagetag null true
        (:`EventReceived`
          (message `CombatInterface.GetCombatSocketLocation` (`self.GetAvatarActorFromActorInfo`) _sockettag)
          (`self.SpawnProjectile` (+ (`Actor.K2_GetActorLocation` _returnvalue) (* (`Actor.GetActorForwardVector` _returnvalue) 500.0)) _sockettag (`self.OverridePitch`) (`self.PitchOverride`)))))
    (:`OnCompleted`
      (`self.K2_EndAbility` :!label _label))
    (:`OnCancelled`
      (goto _label))))