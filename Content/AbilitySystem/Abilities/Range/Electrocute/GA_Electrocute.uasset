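; Channeled lightning ability that locks a beam onto a primary target and branches it to additional targets while input is held.
; A casting animation event triggers targeting and looping beam cues, then a timer commits cost and applies lightning damage to each target.
; Release (with a minimum hold time), primary death or failed cost ends it.
; Ending clears cues, applies additional effects to remaining targets on authority and commits cooldown.
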(event `self.K2_OnEndAbility`
  (params (bWasCancelled :type Boolean))
  (`|ExecutionSequence`
    (:`then_0`
      (`GameplayCueFunctionLibrary.RemoveGameplayCueOnActor` (select `bool` (`self.SuccessfulHit`) :`false` (`self.GetAvatarActorFromActorInfo`) :`true` (`self.HitActor`)) (struct :`TagName` "GameplayCue.Electrocute.Loop") (`self.FirstTargetCueParams`)))
    (:`then_1`
      (if (`self.SuccessfulHit`)
        (`self.ClearPrimaryTarget`)
        (`self.ClearAdditionalTargets`)))
    (:`then_2`
      (`BlueprintMapLibrary.Map_Clear` (`self.AdditionalTargetsToCueParams`))
      (set `self.SuccessfulHit` false)
      (set `self.TimeHeld` 0.0)
      (message `CombatInterface.SetCombatStateToHandle` (`self.GetAvatarActorFromActorInfo`) "Unoccupied" (make `CombatStateParams`))
      (`self.K2_CommitAbilityCooldown` false)
      (`self.PrepareToEndAbility`))))

(event `self.K2_ActivateAbility`
  (`self.InitAbility`)
  (`self.StoreOwnerVariables`)
  (message `CombatInterface.SetCombatStateToHandle` (`self.GetAvatarActorFromActorInfo`) "Casting" (make `CombatStateParams`))
  (`|ExecutionSequence`
    (:`then_0`
      (message `CombatInterface.UpdateFacingTarget` (`self.GetAvatarActorFromActorInfo`) (`Actor.GetActorForwardVector` (`self.GetAvatarActorFromActorInfo`)))
      (bind _returnvalue (message `CombatInterface.GetPaperAnimInstance` (`self.GetAvatarActorFromActorInfo`)))
      (`PaperZDPlaySlotOverrideAction.PlayAnimationOverrideWithCallbacks` _returnvalue "/Game/Assets/Character/AnimSequences/Casting.Casting"
        (:`then`
          (`AbilityTask_WaitGameplayEvent.WaitGameplayEvent` (struct :`TagName` "Montage.Casting") null true
            (:`EventReceived`
              ;[0 0 0] Sound Only
              (`self.K2_ExecuteGameplayCue` (struct :`TagName` "GameplayCue.Electrocute"))
              (bind _returnvalue_2 (`self.StoreFirstTarget`))
              (set `self.SuccessfulHit` _returnvalue_2)
              (`self.AddBeamCueToPrimary`)
              (if (`self.SuccessfulHit`)
                (`|ExecutionSequence`
                  (:`then_0`
                    (bind _outadditionaltargets (`self.StoreAdditionalTargets`))
                    (for _array_element _outadditionaltargets
                      (message `CombatInterface.SetIsElectrocuted` _array_element true)
                      (`self.AddBeamCueToAdditionals` _array_element)))
                  (:`then_1`
                    ;[0 0 0] Damage Tick
                    (bind _returnvalue_3 (`KismetSystemLibrary.K2_SetTimerDelegate` (delegate `DamageTick`) (`self.Frequency`) true))
                    (set `self.DamageTickTimer` _returnvalue_3)))))))
        (:`OnCancelled`
          (`self.K2_EndAbility`))))
    (:`then_1`
      ;[0 0 0] Release
      (bind (_asynctaskproxy _timeheld) (`AbilityTask_WaitInputRelease.WaitInputRelease` false)
        (:`OnRelease`
          (bind _output_get (set `self.TimeHeld` _timeheld))
          (if (< _output_get (`self.MinAbilityTime`))
            (`self.K2_HasAuthority`
              (:`True`
                (`KismetSystemLibrary.Delay` (- (`self.MinAbilityTime`) (`self.TimeHeld`))))
              (:`False`
                _)))
          (`self.K2_EndAbility`))))))

(event `DamageTick`
  ;[0 0 0] Damage Tick
  (bind _returnvalue (`self.K2_CommitAbilityCost` false))
  (if _returnvalue
    (`self.ApplyDamage` (`self.HitActor`))
    (bind _keys (`BlueprintMapLibrary.Map_Keys` (`self.AdditionalTargetsToCueParams`)))
    (for _array_element _keys
      (`self.ApplyDamage` _array_element))
    (else
      (`KismetSystemLibrary.K2_ClearAndInvalidateTimerHandle` (`self.DamageTickTimer`))
      (`self.K2_EndAbility`))))

(event `self.PrimaryTargetDied`
  (params (DeadActor :type "Actor Object Reference"))
  (`GameplayCueFunctionLibrary.RemoveGameplayCueOnActor` DeadActor (struct :`TagName` "GameplayCue.Electrocute.Loop") (`self.FirstTargetCueParams`))
  (`KismetSystemLibrary.K2_ClearAndInvalidateTimerHandle` (`self.DamageTickTimer`))
  (`self.K2_EndAbility`))

(event `self.AdditionalTargetDied`
  (params (DeadActor :type "Actor Object Reference"))
  (`GameplayCueFunctionLibrary.RemoveGameplayCueOnActor` DeadActor (struct :`TagName` "GameplayCue.Electrocute.Loop") (`BlueprintMapLibrary.Map_Find` (`self.AdditionalTargetsToCueParams`) DeadActor))
  (`BlueprintMapLibrary.Map_Remove` (`self.AdditionalTargetsToCueParams`) DeadActor))

(fn `AddBeamCueToAdditionals`
  (params (AdditionalTarget :type "Actor Object Reference"))
  (bind _additionaltarget (`local.AdditionalTarget`))
  (bind _returnvalue (`AbilitySystemBlueprintLibrary.MakeGameplayCueParameters` 0.0 0.0 (struct) (struct) (struct) (struct) (struct) (`Actor.K2_GetActorLocation` _additionaltarget) (0.0 0.0 0.0) null null _additionaltarget null 1 1 (`Actor.RootComponent` (`self.HitActor`))))
  (`BlueprintMapLibrary.Map_Add` (`self.AdditionalTargetsToCueParams`) AdditionalTarget _returnvalue)
  (`GameplayCueFunctionLibrary.AddGameplayCueOnActor` (`local.AdditionalTarget`) (struct :`TagName` "GameplayCue.Electrocute.Loop") _returnvalue))

(fn `AddBeamCueToPrimary`
  (locals (CueTarget :type "Actor Object Reference"))
  (set `self.FirstTargetCueParams` (`AbilitySystemBlueprintLibrary.MakeGameplayCueParameters` 0.0 0.0 (struct) (struct) (struct) (struct) (struct) (`self.HitLocation`) (0.0 0.0 0.0) null null (`self.HitActor`) null 1 1 (`Actor.RootComponent` (`self.GetAvatarActorFromActorInfo`))))
  (if (`self.SuccessfulHit`)
    (set `local.CueTarget` (`self.HitActor`))
    (message `CombatInterface.SetIsElectrocuted` (`local.CueTarget`) true)
    (else
      (set `local.CueTarget` (`self.GetAvatarActorFromActorInfo`))))
  (`GameplayCueFunctionLibrary.AddGameplayCueOnActor` (`local.CueTarget`) (struct :`TagName` "GameplayCue.Electrocute.Loop") (`self.FirstTargetCueParams`)))

(fn `ApplyDamage`
  (params (TargetActor :type "Actor Object Reference"))
  (locals (ASC :type "AbilitySystemComponent Object Reference"))
  (bind _returnvalue (`AbilitySystemBlueprintLibrary.GetAbilitySystemComponent` (`local.TargetActor`)))
  (`/Engine/EditorBlueprintResources/StandardMacros.IsValid` TargetActor
    (:`Is Valid`
      (bind _output_get (set `local.ASC` (`self.GetAbilitySystemComponentFromActorInfo`)))
      (`/Engine/EditorBlueprintResources/StandardMacros.IsValid` _output_get
        (:`Is Valid`
          (bind _returnvalue_2 (`AbilitySystemBlueprintLibrary.AssignTagSetByCallerMagnitude` (`AbilitySystemComponent.MakeOutgoingSpec` (`local.ASC`) "/Game/AbilitySystem/Effects/GE_Damage.GE_Damage_C" (`KismetMathLibrary.Conv_IntToDouble` (`self.GetAbilityLevel`)) (`AbilitySystemComponent.MakeEffectContext` (`local.ASC`))) (struct :`TagName` "Damage.Lightning") (`self.GetAbilityPowerAtLevel`)))
          (`/Engine/EditorBlueprintResources/StandardMacros.IsValid` _returnvalue
            (:`Is Valid`
              (`AbilitySystemComponent.BP_ApplyGameplayEffectSpecToSelf` _returnvalue _returnvalue_2))))))))

(fn `ClearAdditionalTargets`
  (locals (AdditionalTarget :type "Actor Object Reference"))
  (bind _keys (`BlueprintMapLibrary.Map_Keys` (`self.AdditionalTargetsToCueParams`)))
  (for _array_element _keys
    (bind _output_get (set `local.AdditionalTarget` _array_element))
    (message `CombatInterface.SetIsElectrocuted` _output_get false)
    (`GameplayCueFunctionLibrary.RemoveGameplayCueOnActor` (`local.AdditionalTarget`) (struct :`TagName` "GameplayCue.Electrocute.Loop") (`BlueprintMapLibrary.Map_Find` (`self.AdditionalTargetsToCueParams`) (`local.AdditionalTarget`)))
    (`self.ClearAdditionalOnDeathDelegate` (`local.AdditionalTarget`))
    (`self.K2_HasAuthority`
      (:`True`
        (`LeyrAbilitySystemLibrary.ApplyAdditionalEffect` (`self.MakeAdditionalEffectParamsFromClassDefaults` (`local.AdditionalTarget`)))))))

(fn `ClearPrimaryTarget`
  (`self.ClearPrimaryOnDeathDelegate`)
  (message `CombatInterface.SetIsElectrocuted` (`self.HitActor`) false)
  (`self.K2_HasAuthority`
    (:`True`
      (`LeyrAbilitySystemLibrary.ApplyAdditionalEffect` (`self.MakeAdditionalEffectParamsFromClassDefaults` (`self.HitActor`))))))