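; Gameplay ability that casts an earthquake as a timed series of ground impacts.
; On the casting animation's gameplay event, it spawns a BP_PointCollection at the avatar and gets ground points, their count scaling with ability level up to a cap.
; A looping timer visits each point, firing a gameplay cue, drawing debug spheres and applying radial effects to nearby live players except the caster.
; When points run out, the ability ends, destroying the collection and clearing the timer.
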(event `self.K2_OnEndAbility`
  (params (bWasCancelled :type Boolean))
  (`self.PrepareToEndAbility`)
  (`Actor.K2_DestroyActor` (`self.PointCollection`))
  (`KismetSystemLibrary.K2_ClearAndInvalidateTimerHandle` (`self.SpawnTimer`)))

(event `self.K2_ActivateAbility`
  (`self.InitAbility`)
  (bind _returnvalue (message `CombatInterface.GetPaperAnimInstance` (`self.GetAvatarActorFromActorInfo`)))
  (`PaperZDPlaySlotOverrideAction.PlayAnimationOverrideWithCallbacks` _returnvalue "/Game/Assets/Character/AnimSequences/Casting.Casting"
    (:`then`
      (`AbilityTask_WaitGameplayEvent.WaitGameplayEvent` (struct :`TagName` "Montage.Casting") null true
        (:`EventReceived`
          (bind _returnvalue_2 (`|SpawnActorFromClass` "/Game/AbilitySystem/Actor/Collection/BP_PointCollection.BP_PointCollection_C" (`Actor.GetTransform` (`self.GetAvatarActorFromActorInfo`)) "AlwaysSpawn" "MultiplyWithRoot" null null))
          (bind _output_get (set `self.PointCollection` _returnvalue_2))
          (bind _output_get_2 (set `self.Points` (`PointCollection.GetGroundPoints` _output_get (`KismetMathLibrary.Min` (`self.GetAbilityLevel`) (`self.NumPoints`)) 0.0)))
          (set `self.ValidPointCount` (`KismetArrayLibrary.Array_Length` _output_get_2))
          (bind _returnvalue_3 (`KismetSystemLibrary.K2_SetTimerDelegate` (delegate `SpawnShard`) (`self.SpawnFrequency`) true))
          (set `self.SpawnTimer` _returnvalue_3)
          (`self.SpawnShard`))))))

(event `SpawnShard`
  (if (< (`self.PointCount`) (`self.ValidPointCount`))
    (bind _output_get (set `self.SpawnLoaction` (`SceneComponent.K2_GetComponentLocation` (`|GetArrayItem` (`self.Points`) (`self.PointCount`)))))
    (`KismetSystemLibrary.DrawDebugSphere` _output_get (`self.GetRadialDamageInnerRadius`) 12 (struct :`R` 1.0 :`G` 0.14218 :`A` 1.0) 20.0)
    (`KismetSystemLibrary.DrawDebugSphere` _output_get (`self.GetRadialDamageOuterRadius`) 12 (struct :`R` 1.0 :`G` 0.731228 :`B` 0.121967 :`A` 1.0) 20.0)
    (`/Engine/EditorBlueprintResources/StandardMacros.IncrementInt` (`self.PointCount`)
      (:`  `
        (`self.K2_ExecuteGameplayCueWithParams` (struct :`TagName` "GameplayCue.Earth.Earthquake") (`AbilitySystemBlueprintLibrary.MakeGameplayCueParameters` 0.0 0.0 (struct) (struct) (struct) (struct) (struct) (`self.SpawnLoaction`)))
        (bind _outoverlappingactors (`LeyrAbilitySystemLibrary.GetLivePlayersWithinRadius` (`|MakeArray` (`self.GetAvatarActorFromActorInfo`)) (`self.GetRadialDamageOuterRadius`) (`self.SpawnLoaction`)))
        (bind _output_get_2 (set `self.OverlappingActors` _outoverlappingactors))
        (for _array_element _output_get_2
          (bind _structout (setmembers `AdditionalEffectParams` :`StructRef` (`self.MakeAdditionalEffectParamsFromClassDefaults` _array_element) :`RadialDamageOrigin` (`self.SpawnLoaction`)))
          (`LeyrAbilitySystemLibrary.ApplyAdditionalEffect` _structout))))
    (else
      (`self.K2_EndAbility`))))