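; Earthquake gameplay ability that erupts a series of timed shards at ground points around the caster, affecting nearby live players except the caster.
; A Paper animation's casting event triggers the cost check, then a spawned point collection supplies ground points, capped by ability level.
; A looping timer fires a gameplay cue and applies radial effects at each point, committing cooldown after the last.
; Ending the ability clears the timer and point collection.
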(event `self.K2_OnEndAbility`
  (params (bWasCancelled :type Boolean))
  (`self.PrepareToEndAbility`)
  (`KismetSystemLibrary.K2_ClearAndInvalidateTimerHandle` (`self.SpawnTimer`))
  (bind _pointcollection (`self.PointCollection`)
    (:`then`
      (`Actor.K2_DestroyActor` _pointcollection))
    (:`else`)))

(event `self.K2_ActivateAbility`
  (`self.InitAbility`)
  (bind _returnvalue (message `CombatInterface.GetPaperAnimInstance` (`self.GetAvatarActorFromActorInfo`)))
  (`PaperZDPlaySlotOverrideAction.PlayAnimationOverrideWithCallbacks` _returnvalue "/Game/Assets/Character/AnimSequences/Casting.Casting"
    (:`then`
      (`AbilityTask_WaitGameplayEvent.WaitGameplayEvent` (struct :`TagName` "Montage.Casting") null true
        (:`EventReceived`
          (bind _returnvalue_2 (`self.K2_CheckAbilityCost`))
          (if _returnvalue_2
            (bind _returnvalue_3 (`|SpawnActorFromClass` "/Game/AbilitySystem/Actor/Collection/BP_PointCollection.BP_PointCollection_C" (`KismetMathLibrary.MakeTransform` (`KismetMathLibrary.MakeVector` (.x (`Actor.K2_GetActorLocation` (`self.GetAvatarActorFromActorInfo`))) (.y (`Actor.K2_GetActorLocation` (`self.GetAvatarActorFromActorInfo`))) (- (.z (`Actor.K2_GetActorLocation` (`self.GetAvatarActorFromActorInfo`))) 25.0))) "AlwaysSpawn" "MultiplyWithRoot" null null))
            (bind _output_get (set `self.PointCollection` _returnvalue_3))
            (bind _output_get_2 (set `self.Points` (`PointCollection.GetGroundPoints` _output_get (`KismetMathLibrary.Min` (`self.GetAbilityLevel`) (`self.NumPoints`)) 0.0)))
            (set `self.ValidPointCount` (`KismetArrayLibrary.Array_Length` _output_get_2))
            (bind _returnvalue_4 (`KismetSystemLibrary.K2_SetTimerDelegate` (delegate `SpawnShard`) (`self.SpawnFrequency`) true))
            (set `self.SpawnTimer` _returnvalue_4)
            (`self.SpawnShard`)
            (`self.K2_CommitAbilityCost` false)
            (else
              (`self.K2_EndAbility`))))))))

(event `SpawnShard`
  (if (< (`self.PointCount`) (`self.ValidPointCount`))
    (bind _output_get (set `self.SpawnLoaction` (`SceneComponent.K2_GetComponentLocation` (`|GetArrayItem` (`self.Points`) (`self.PointCount`)))))
    (`/Engine/EditorBlueprintResources/StandardMacros.IncrementInt` (`self.PointCount`)
      (:`  `
        (`self.K2_ExecuteGameplayCueWithParams` (struct :`TagName` "GameplayCue.Earth.Earthquake") (`AbilitySystemBlueprintLibrary.MakeGameplayCueParameters` 0.0 0.0 (struct) (struct) (struct) (struct) (struct) (`self.SpawnLoaction`)))
        (bind _outoverlappingactors (`LeyrAbilitySystemLibrary.GetLivePlayersWithinRadius` (`|MakeArray` (`self.GetAvatarActorFromActorInfo`)) (`self.GetRadialDamageOuterRadius`) (`self.SpawnLoaction`)))
        (bind _output_get_2 (set `self.OverlappingActors` _outoverlappingactors))
        (for _array_element _output_get_2
          (bind _structout (setmembers `AdditionalEffectParams` :`StructRef` (`self.MakeAdditionalEffectParamsFromClassDefaults` _array_element) :`RadialDamageOrigin` (`self.SpawnLoaction`)))
          (`LeyrAbilitySystemLibrary.ApplyAdditionalEffect` _structout))))
    (else
      (`self.K2_CommitAbilityCooldown` false)
      (`self.K2_EndAbility`))))