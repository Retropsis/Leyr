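; GA_VenomBall is a gameplay ability that plays a Paper2D attack animation and spawns projectiles.
; On activation it aims at the avatar's combat target, or at a point just ahead when there is none.
; It plays a random default attack animation, waits for that animation's gameplay event, then faces the aim point and spawns projectiles from the tagged socket.
; The ability ends when the animation completes or is cancelled.
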(event `self.K2_ActivateAbility`
  (bind _returnvalue (`self.GetAvatarActorFromActorInfo`))
  (`self.InitAbility`)
  (bind _returnvalue_2 (message `EnemyInterface.GetCombatTarget` (`self.GetAvatarActorFromActorInfo`)))
  (`/Engine/EditorBlueprintResources/StandardMacros.IsValid` _returnvalue_2
    (:`Is Valid`
      (set `self.bHasTarget` true)
      (set `self.TargetLocation` (`Actor.K2_GetActorLocation` _returnvalue_2)))
    (:`Is Not Valid`
      (bind _output_get (set `self.TargetLocation` (+ (`Actor.K2_GetActorLocation` _returnvalue) (* (`Actor.GetActorForwardVector` _returnvalue) 50.0))))
      (message `CombatInterface.UpdateFacingTarget` _returnvalue _output_get)))
  (bind _returnvalue_3 (message `CombatInterface.GetPaperAnimInstance` (`self.GetAvatarActorFromActorInfo`)))
  (bind _returnvalue_4 (message `CombatInterface.GetAttackMontages` (`self.GetAvatarActorFromActorInfo`) "Default"))
  (bind _output_get_2 (set `self.TaggedMontage` (`KismetArrayLibrary.Array_Random` _returnvalue_4)))
  (bind ((`MontageTag` _montagetag) (`SocketTag` _sockettag) (`Montage` _montage)) (break `TaggedMontage` _output_get_2))
  (`PaperZDPlaySlotOverrideAction.PlayAnimationOverrideWithCallbacks` _returnvalue_3 _montage
    (:`then`
      (`AbilityTask_WaitGameplayEvent.WaitGameplayEvent` _montagetag null true
        (:`EventReceived`
          (message `CombatInterface.UpdateFacingTarget` (`self.GetAvatarActorFromActorInfo`) (`self.TargetLocation`))
          (`self.SpawnProjectiles` (`self.TargetLocation`) _sockettag))))
    (:`OnCompleted`
      (`self.K2_EndAbility` :!label _label))
    (:`OnCancelled`
      (goto _label))))