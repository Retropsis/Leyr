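; Gameplay ability that moves the avatar up and off a rope, playing the Rope_ClimbUp Paper animation override.
; As the animation starts, a timed root motion MoveTo force lifts the character just over one capsule height straight up in Walking mode.
; The ability ends when the move times out at its destination or the animation is cancelled, and resets combat state to Unoccupied.
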(event `self.K2_OnEndAbility`
  (params (bWasCancelled :type Boolean))
  (message `CombatInterface.SetCombatStateToHandle` (`self.GetAvatarActorFromActorInfo`) "Unoccupied"))

(event `self.K2_ActivateAbility`
  (`self.InitAbility`)
  (bind _returnvalue (message `CombatInterface.GetPaperAnimInstance` (`self.GetAvatarActorFromActorInfo`)))
  (`PaperZDPlaySlotOverrideAction.PlayAnimationOverrideWithCallbacks` _returnvalue "/Game/Assets/Character/AnimSequences/Rope_ClimbUp.Rope_ClimbUp"
    (:`then`
      (`AbilityTask_ApplyRootMotionMoveToForce.ApplyRootMotionMoveToForce` "None" (`self.GetTargetLocation`) 0.35 false "MOVE_Walking" false null "ClampVelocity"
        (:`OnTimedOutAndDestinationReached`
          (`self.K2_EndAbility`))))
    (:`OnCancelled`
      (`self.K2_EndAbility`))))

(fn `GetTargetLocation`
  (returns (ReturnValue :type "Vector Structure"))
  (bind _returnvalue (`self.GetAvatarActorFromActorInfo`))
  (return (+ (`Actor.K2_GetActorLocation` _returnvalue) (`KismetMathLibrary.MakeVector` 0.0 0.0 (+ (* (`CapsuleComponent.GetScaledCapsuleHalfHeight` (`Character.CapsuleComponent` (cast `Character` _returnvalue :!pure true))) 2.0) 10.0)))))