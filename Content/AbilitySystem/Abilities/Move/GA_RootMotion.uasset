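; Gameplay ability that moves a Paper2D-animated character through ledge hops and rope climbs, chosen by the avatar's current combat state.
; Each state selects an animation override, duration and target offset from capsule height, plus forward X for ledges.
; Playback starts a root motion MoveToForce toward that target.
; Arrival or animation cancellation ends the ability, resetting combat state to Unoccupied; animation completion only prints a debug string.
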(event `self.K2_OnEndAbility`
  (params (bWasCancelled :type Boolean))
  (message `CombatInterface.SetCombatStateToHandle` (`self.GetAvatarActorFromActorInfo`) "Unoccupied"))

(event `self.K2_ActivateAbility`
  (bind _returnvalue (`self.GetAvatarActorFromActorInfo`))
  (`self.InitAbility`)
  (bind _returnvalue_2 (message `CombatInterface.GetPaperAnimInstance` _returnvalue))
  (bind _returnvalue_3 (message `CombatInterface.GetCombatState` _returnvalue))
  (switch `ECombatState` _returnvalue_3
    (:`HoppingLedge`
      (set `self.SelectedMontage` "/Game/Assets/Character/AnimSequences/Ledge_Hopping.Ledge_Hopping")
      (set `self.TargetLocation` (`self.GetTargetLocation` "HoppingLedge"))
      (set `self.Duration` 0.333))
    (:`ClimbingRope`
      (set `self.SelectedMontage` "/Game/Assets/Character/AnimSequences/Rope_ClimbUp.Rope_ClimbUp")
      (set `self.TargetLocation` (`self.GetTargetLocation` "ClimbingRope"))
      (set `self.Duration` 0.35)))
  (`PaperZDPlaySlotOverrideAction.PlayAnimationOverrideWithCallbacks` _returnvalue_2 (`self.SelectedMontage`)
    (:`then`
      (`AbilityTask_ApplyRootMotionMoveToForce.ApplyRootMotionMoveToForce` "None" (`self.TargetLocation`) (`self.Duration`) false "MOVE_Walking" false null "ClampVelocity"
        (:`OnTimedOutAndDestinationReached`
          (`self.K2_EndAbility`)
          (`KismetSystemLibrary.PrintString` "Destination Reached"))))
    (:`OnCompleted`
      (`KismetSystemLibrary.PrintString` "Anim Complete"))
    (:`OnCancelled`
      (`self.K2_EndAbility`)
      (`KismetSystemLibrary.PrintString` "Anim Cancelled"))))

(fn `GetTargetLocation`
  (params (CombatState :type "ECombatState Enum" :default "Unoccupied"))
  (returns (ReturnValue :type "Vector Structure"))
  (bind _returnvalue (`self.GetAvatarActorFromActorInfo`))
  (bind _returnvalue_2 (`self.GetAvatarActorFromActorInfo`))
  (switch `ECombatState` CombatState
    (:`HoppingLedge`
      (return (+ (`Actor.K2_GetActorLocation` _returnvalue_2) (`KismetMathLibrary.MakeVector` (* (.x (`Actor.GetActorForwardVector` _returnvalue_2)) 50.0) 0.0 (+ (`CapsuleComponent.GetScaledCapsuleHalfHeight` (`Character.CapsuleComponent` (cast `Character` _returnvalue_2 :!pure true))) 15.0)))))
    (:`ClimbingRope`
      (return (+ (`Actor.K2_GetActorLocation` _returnvalue) (`KismetMathLibrary.MakeVector` 0.0 0.0 (+ (* (`CapsuleComponent.GetScaledCapsuleHalfHeight` (`Character.CapsuleComponent` (cast `Character` _returnvalue :!pure true))) 2.0) 10.0)))))))