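; Gameplay ability that gives the avatar a short forward swim impulse.
; On activation it checks and commits the cooldown, initializes, then plays the Swimming override animation on the avatar's Paper anim instance.
; A brief additive constant root motion force pushes along the actor's forward vector and clamps velocity when finished.
; The ability ends when the force finishes or the animation is cancelled.
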(event `self.K2_OnEndAbility`
  (params (bWasCancelled :type Boolean)))

(event `self.K2_ActivateAbility`
  (bind _returnvalue (`self.K2_CheckAbilityCooldown`))
  (if _returnvalue
    (`self.K2_CommitAbilityCooldown` false)
    (`self.InitAbility`)
    (bind _returnvalue_2 (message `CombatInterface.GetPaperAnimInstance` (`self.GetAvatarActorFromActorInfo`)))
    (`PaperZDPlaySlotOverrideAction.PlayAnimationOverrideWithCallbacks` _returnvalue_2 "/Game/Assets/Character/AnimSequences/Swimming.Swimming"
      (:`then`
        (`AbilityTask_ApplyRootMotionConstantForce.ApplyRootMotionConstantForce` "None" (`Actor.GetActorForwardVector` (`self.GetAvatarActorFromActorInfo`)) 750.0 0.05 true null "ClampVelocity" (0.0 0.0 0.0) 200.0
          (:`OnFinish`
            (`self.K2_EndAbility`))))
      (:`OnCancelled`
        (`self.K2_EndAbility`)))))