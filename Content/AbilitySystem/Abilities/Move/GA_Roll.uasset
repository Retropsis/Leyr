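; Gameplay ability for a dodge-style roll on a Paper 2D character, playing the Roll animation override.
; On activation it applies a forward root-motion force, timed to match the flipbook for smooth exit movement, and spawns direction-flipped sliding dust.
; A combo-window event adds the Execute tag, which is removed when the animation completes or cancels and the ability ends.
; OnEndAbility sends the RollingEnd combat state to the avatar.
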(event `self.K2_OnEndAbility`
  (params (bWasCancelled :type Boolean))
  (`self.PrepareToEndAbility`)
  (message `CombatInterface.SetCombatStateToHandle` (`self.GetAvatarActorFromActorInfo`) "RollingEnd" (make `CombatStateParams`)))

(event `self.K2_ActivateAbility`
  (bind _returnvalue (`self.GetAvatarActorFromActorInfo`))
  (`self.InitAbility`)
  (bind _returnvalue_2 (message `CombatInterface.GetPaperAnimInstance` (`self.GetAvatarActorFromActorInfo`)))
  (`PaperZDPlaySlotOverrideAction.PlayAnimationOverrideWithCallbacks` _returnvalue_2 "/Game/Assets/Character/AnimSequences/Roll.Roll"
    (:`then`
      (`AbilityTask_WaitGameplayEvent.WaitGameplayEvent` (struct :`TagName` "Montage.Roll.End") null true
        (:`then`
          (`AbilityTask_WaitGameplayEvent.WaitGameplayEvent` (struct :`TagName` "Montage.EndAbility") null true
            (:`then`
              (`AbilityTask_WaitGameplayEvent.WaitGameplayEvent` (struct :`TagName` "Abilities.Combo.Window.Begin") null true
                (:`then`
                  (`AbilityTask_ApplyRootMotionConstantForce.ApplyRootMotionConstantForce` "None" (`Actor.GetActorForwardVector` (`self.GetAvatarActorFromActorInfo`)) 700.0 (`self.RollDuration`) true null "ClampVelocity" (0.0 0.0 0.0) 500.0
                    (:`then`
                      _)
                    (:`OnFinish`
                      _))
                  (bind _returnvalue_3 (`NiagaraFunctionLibrary.SpawnSystemAtLocation` "/Game/Effects/Dust/Sliding/NS_Sliding_Dust.NS_Sliding_Dust" (- (`Actor.K2_GetActorLocation` _returnvalue) (`KismetMathLibrary.MakeVector` 0.0 5.0 (`CapsuleComponent.GetScaledCapsuleHalfHeight` (`Character.CapsuleComponent` (cast `Character` _returnvalue :!pure true)))))))
                  (`NiagaraComponent.SetVariableVec2` _returnvalue_3 "SpriteUVScale" (`KismetMathLibrary.MakeVector2D` (.x (`Actor.GetActorForwardVector` _returnvalue)) 1.0)))
                (:`EventReceived`
                  (`AbilitySystemBlueprintLibrary.AddLooseGameplayTags` (`self.GetAvatarActorFromActorInfo`) (`BlueprintGameplayTagLibrary.MakeGameplayTagContainerFromTag` (struct :`TagName` "Abilities.Combo.Window.Execute"))))))))))
    (:`OnCompleted`
      (`AbilitySystemBlueprintLibrary.RemoveLooseGameplayTags` (`self.GetAvatarActorFromActorInfo`) (`BlueprintGameplayTagLibrary.MakeGameplayTagContainerFromTag` (struct :`TagName` "Abilities.Combo.Window.Execute")) :!label _label)
      (`self.K2_EndAbility`))
    (:`OnCancelled`
      (goto _label))))