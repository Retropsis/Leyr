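; Gameplay ability for shielding that holds a shield stance until the input is released.
; Activation plays start animations on the Paper2D character, upper body and weapon anim instances.
; The Montage.Shielding.Begin event adds the shielding tag and sets the Shielding combat state.
; Release restores the Unoccupied state, plays end animations and removes the tag, with the ability ending when the character's end animation completes or is cancelled.
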(event `self.K2_OnEndAbility`
  (params (bWasCancelled :type Boolean))
  (`self.PrepareToEndAbility`))

(event `self.K2_ActivateAbility`
  (`self.InitAbility`)
  (`PaperZDPlaySlotOverrideAction.PlayAnimationOverrideWithCallbacks` (`self.PaperAnimInstance`) "/Game/Assets/Character/AnimSequences/Character_Shielding_Start.Character_Shielding_Start"
    (:`then`
      (`PaperZDPlaySlotOverrideAction.PlayAnimationOverrideWithCallbacks` (`self.UpperBodyAnimInstance`) "/Game/Assets/Character/AnimSequences/Character_Shielding_Start_Upper.Character_Shielding_Start_Upper"
        (:`then`
          (`PaperZDPlaySlotOverrideAction.PlayAnimationOverrideWithCallbacks` (`self.WeaponAnimInstance`) "/Game/Assets/Equipment/Shield/AnimSequences/Shield_Start.Shield_Start"
            (:`then`
              (`AbilityTask_WaitGameplayEvent.WaitGameplayEvent` (struct :`TagName` "Montage.Shielding.Begin") null true
                (:`then`
                  (`AbilityTask_WaitInputRelease.WaitInputRelease` true
                    (:`OnRelease`
                      (message `CombatInterface.SetCombatStateToHandle` (`self.GetAvatarActorFromActorInfo`) "Unoccupied" (make `CombatStateParams`))
                      (`PaperZDPlaySlotOverrideAction.PlayAnimationOverrideWithCallbacks` (`self.PaperAnimInstance`) "/Game/Assets/Character/AnimSequences/Character_Shielding_End.Character_Shielding_End"
                        (:`then`
                          (`PaperZDPlaySlotOverrideAction.PlayAnimationOverrideWithCallbacks` (`self.UpperBodyAnimInstance`) "/Game/Assets/Character/AnimSequences/Character_Shielding_End_Upper.Character_Shielding_End_Upper"
                            (:`then`
                              (`PaperZDPlaySlotOverrideAction.PlayAnimationOverrideWithCallbacks` (`self.WeaponAnimInstance`) "/Game/Assets/Equipment/Shield/AnimSequences/Shield_End.Shield_End"
                                (:`then`
                                  (`AbilitySystemBlueprintLibrary.RemoveLooseGameplayTags` (`self.GetAvatarActorFromActorInfo`) (`BlueprintGameplayTagLibrary.MakeGameplayTagContainerFromTag` (struct :`TagName` "Montage.Shielding"))))))))
                        (:`OnCompleted`
                          (`self.K2_EndAbility` :!label _label))
                        (:`OnCancelled`
                          (goto _label))))))
                (:`EventReceived`
                  (`AbilitySystemBlueprintLibrary.AddLooseGameplayTags` (`self.GetAvatarActorFromActorInfo`) (`BlueprintGameplayTagLibrary.MakeGameplayTagContainerFromTag` (struct :`TagName` "Montage.Shielding")))
                  (message `CombatInterface.SetCombatStateToHandle` (`self.GetAvatarActorFromActorInfo`) "Shielding" (make `CombatStateParams`)))))))))
    (:`OnCancelled`
      (`self.K2_EndAbility`))))