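; Gameplay ability for the AI Thrower's flamethrower attack, which deals repeated damage in front of the avatar.
; Plays a random attack montage as a Paper animation override, then waits for its tagged gameplay event to spawn a yaw-aligned Niagara flame.
; After a short delay, a looping timer box-traces for a set number of ticks, applying damage and firing a weapon GameplayCue on hits, then ends the ability.
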(event `self.K2_ActivateAbility`
  (bind _returnvalue (`self.GetAvatarActorFromActorInfo`))
  (bind _returnvalue_2 (`self.GetAvatarActorFromActorInfo`))
  (bind _yaw (.yaw (`Actor.K2_GetActorRotation` _returnvalue)))
  (bind _returnvalue_3 (message `CombatInterface.GetPaperAnimInstance` _returnvalue_2))
  (bind _returnvalue_4 (message `CombatInterface.GetAttackMontages` _returnvalue_2 (`self.SequenceType`)))
  (bind _output_get (set `self.TaggedMontage` (`KismetArrayLibrary.Array_Random` _returnvalue_4)))
  (bind (_abilitypower _damagetype _montagetag _sockettag _montage) (break `TaggedMontage` _output_get))
  (`PaperZDPlaySlotOverrideAction.PlayAnimationOverrideWithCallbacks` _returnvalue_3 _montage
    (:`then`
      (`AbilityTask_WaitGameplayEvent.WaitGameplayEvent` _montagetag null true
        (:`EventReceived`
          (bind _returnvalue_5 (`NiagaraFunctionLibrary.SpawnSystemAtLocation` "/Game/Effects/FlameThrower/NS_FlameThrower.NS_FlameThrower" (+ (`Actor.K2_GetActorLocation` _returnvalue) (* (`Actor.GetActorForwardVector` _returnvalue) 25.0)) (`KismetMathLibrary.MakeRotator` 0.0 0.0 _yaw)))
          (`NiagaraComponent.SetVariableFloat` _returnvalue_5 "SpriteRotationAngle" _yaw)
          (`KismetSystemLibrary.Delay` 0.1)
          (bind _returnvalue_6 (`KismetSystemLibrary.K2_SetTimerDelegate` (delegate `BoxTraceTick`) 0.6 true))
          (set `self.BoxTraceTickTimer` _returnvalue_6)
          (set `self.CurrentTick` 0))))
    (:`OnCancelled`
      (`self.K2_EndAbility`))))

(event `BoxTraceTick`
  (if (< (`self.CurrentTick`) (`self.NumTicks`))
    (`/Engine/EditorBlueprintResources/StandardMacros.IncrementInt` (`self.CurrentTick`)
      (:`  `
        (bind _returnvalue (`MeleeGameplayAbility.BoxTrace` true))
        (`self.ForEachHitTryCausingDamage` _returnvalue)
        (if (`self.bHasHitTarget`)
          (`self.K2_ExecuteGameplayCueWithParams` (struct :`TagName` "GameplayCue.Weapon") (`AbilitySystemBlueprintLibrary.MakeGameplayCueParameters` 0.0 0.0 (struct) (struct) (struct) (`BlueprintGameplayTagLibrary.MakeGameplayTagContainerFromTag` (`self.MontageTag`)) (struct) (`self.HitLocation`) (0.0 0.0 0.0) null (`self.GetAvatarActorFromActorInfo`) (`self.HitActor`))))))
    (else
      (`KismetSystemLibrary.K2_ClearAndInvalidateTimerHandle` (`self.BoxTraceTickTimer`))
      (`self.K2_EndAbility`))))