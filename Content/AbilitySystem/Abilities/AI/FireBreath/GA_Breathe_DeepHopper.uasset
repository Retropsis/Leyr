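; Gameplay ability for the Deep Hopper AI's fire breath attack.
; Sets the multi-part character to its attack state, playing Paper animation overrides alongside a sped-up breathe montage.
; A gameplay event from the attack animation spawns the Niagara breath at the combat socket, aligned to actor yaw.
; A looping timer then repeats box-trace damage and weapon cues until the tick count ends the ability, returning parts to idle.
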(event `self.K2_OnEndAbility`
  (params (bWasCancelled :type Boolean))
  (message `MultiPartAIInterface.UpdateMultiPartAnimInstances` (`self.MultiPartAICharacter`) "Idle"))

(event `self.K2_ActivateAbility`
  (bind _returnvalue (`self.GetAvatarActorFromActorInfo`))
  (bind _returnvalue_2 (`self.GetAvatarActorFromActorInfo`))
  (bind _yaw (.yaw (`Actor.K2_GetActorRotation` _returnvalue_2)))
  (bind _asmulti_part_aicharacter (cast `MultiPartAICharacter` (`self.GetAvatarActorFromActorInfo`)))
  (set `self.MultiPartAICharacter` _asmulti_part_aicharacter)
  (`self.InitAbility`)
  (bind _returnvalue_3 (message `CombatInterface.GetPaperAnimInstance` _returnvalue))
  (bind _returnvalue_4 (message `CombatInterface.GetTaggedMontageByTag` _returnvalue (`BlueprintGameplayTagLibrary.MakeLiteralGameplayTag` (struct :`TagName` "Montage.Attack.1")) "Default"))
  (bind _output_get (set `self.TaggedMontage` _returnvalue_4))
  (bind (_montagetag _sockettag _montage) (break `TaggedMontage` _output_get))
  (`PaperZDPlaySlotOverrideAction.PlayAnimationOverrideWithCallbacks` _returnvalue_3 _montage
    (:`then`
      (`AbilityTask_WaitGameplayEvent.WaitGameplayEvent` _montagetag null true
        (:`then`
          (message `MultiPartAIInterface.UpdateMultiPartAnimInstances` (`self.MultiPartAICharacter`) "Attack")
          (bind _returnvalue_5 (message `MultiPartAIInterface.GetMultiPartAnimInstance` (`self.MultiPartAICharacter`)))
          (`AnimInstance.Montage_Play` _returnvalue_5 "/Game/Assets/3D/Hopper/AM_DeepHopper_Breathe.AM_DeepHopper_Breathe" 2.5 "MontageLength" 0.0 true))
        (:`EventReceived`
          (`PaperZDPlaySlotOverrideAction.PlayAnimationOverrideWithCallbacks` (`self.PaperAnimInstance`) "/Game/AI/DeepHopper/AnimSequences/Hopper_Body_Breathe.Hopper_Body_Breathe"
            (:`then`
              (bind _returnvalue_6 (message `CombatInterface.GetCombatSocketLocation` _returnvalue_2 (`BlueprintGameplayTagLibrary.MakeLiteralGameplayTag` (struct :`TagName` "Montage.Attack.1"))))
              (bind _returnvalue_7 (`NiagaraFunctionLibrary.SpawnSystemAtLocation` "/Game/Effects/FireBreath/NS_FireBreath.NS_FireBreath" _returnvalue_6 (`KismetMathLibrary.MakeRotator` 0.0 0.0 _yaw)))
              (`NiagaraComponent.SetVariableFloat` _returnvalue_7 "SpriteRotationAngle" _yaw)
              (`KismetSystemLibrary.Delay` 0.1)
              (bind _returnvalue_8 (`KismetSystemLibrary.K2_SetTimerDelegate` (delegate `BoxTraceTick`) 0.6 true))
              (set `self.BoxTraceTickTimer` _returnvalue_8)
              (set `self.CurrentTick` 0)
              (`self.BoxTraceTick`))
            (:`OnCompleted`
              (`PaperZDPlaySlotOverrideAction.PlayAnimationOverrideWithCallbacks` (`self.PaperAnimInstance`) "/Game/AI/DeepHopper/AnimSequences/Hopper_Body_Breathe.Hopper_Body_Breathe"))))))))

(event `BoxTraceTick`
  (if (< (`self.CurrentTick`) (`self.NumTicks`))
    (`/Engine/EditorBlueprintResources/StandardMacros.IncrementInt` (`self.CurrentTick`)
      (:`  `
        (bind _returnvalue (`MeleeGameplayAbility.BoxTrace` false))
        (`self.ForEachHitTryCausingDamage` _returnvalue)
        (if (`self.bHasHitTarget`)
          (`self.ExecuteDamageGameplayCue` (struct :`TagName` "GameplayCue.Weapon")))))
    (else
      (`KismetSystemLibrary.K2_ClearAndInvalidateTimerHandle` (`self.BoxTraceTickTimer`))
      (`self.K2_EndAbility`))))