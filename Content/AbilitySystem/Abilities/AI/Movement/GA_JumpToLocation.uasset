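; AI gameplay ability that launches the avatar Character in a jump relative to its combat target, moving along X only.
; The landing point sits a short offset from the target on the character's side; when close and that point is out of bounds, it becomes a long forward leap.
; Suggested projectile velocity drives LaunchCharacter, using a faster high arc for the fallback.
; A Paper2D jump animation override ends the ability on completion or cancellation.
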(event `self.K2_ActivateAbility`
  (bind (_endlocation _iswithinbounds) (`self.CalcultaeEndLocation`))
  (bind _returnvalue (`Actor.K2_GetActorLocation` (`self.Character`)))
  (`self.InitAbility`)
  (set `self.Character` (cast `Character` (`self.GetAvatarActorFromActorInfo`) :!pure true))
  (bind _returnvalue_2 (message `EnemyInterface.GetCombatTarget` (`self.GetAvatarActorFromActorInfo`)))
  (set `self.CombatTarget` _returnvalue_2)
  (`self.CombatTarget`
    (:`then`
      (if _iswithinbounds
        (bind _tossvelocity (`GameplayStatics.BlueprintSuggestProjectileVelocity` _returnvalue _endlocation 1000.0 0.0 "DoNotTrace"))
        (`Character.LaunchCharacter` (`self.Character`) _tossvelocity true true)
        (else
          (bind _tossvelocity_2 (`GameplayStatics.BlueprintSuggestProjectileVelocity` _returnvalue _endlocation 1600.0 -1960.0 "DoNotTrace" 0.0 true true))
          (`Character.LaunchCharacter` (`self.Character`) _tossvelocity_2 true true)))
      (`PaperZDPlaySlotOverrideAction.PlayAnimationOverrideWithCallbacks` (`self.PaperAnimInstance`) "/Game/AI/TheScourge/AnimSequences/Jump.Jump"
        (:`OnCompleted`
          _)
        (:`OnCancelled`
          _))
      (`self.K2_EndAbility`))
    (:`else`
      (`self.K2_EndAbility`))))

(fn `CalcultaeEndLocation`
  (returns (EndLocation :type "Vector Structure") (IsWithinBounds :type Boolean))
  (locals (JumpLocation :type "Vector Structure" :default (0.0 0.0 0.0)))
  (bind _returnvalue (`KismetMathLibrary.MakeVector` (+ (.x (`Actor.K2_GetActorLocation` (`self.Character`))) (.x (* (`Actor.GetActorForwardVector` (`self.Character`)) 1200.0))) (.y (`Actor.K2_GetActorLocation` (`self.Character`))) (.z (`Actor.K2_GetActorLocation` (`self.Character`)))))
  (set `local.JumpLocation` (`self.GetJumpLocation`))
  (if (> (`Actor.GetDistanceTo` (`self.Character`) (`self.CombatTarget`)) 325.0)
    (return (`local.JumpLocation`) true)
    (else
      (bind _returnvalue_2 (message `AIInterface.IsWithinBounds` (`self.Character`) (`local.JumpLocation`)))
      (if _returnvalue_2
        (`KismetSystemLibrary.DrawDebugSphere` (`local.JumpLocation`) 25.0 12 (struct :`R` 1.0 :`G` 0.0685 :`A` 1.0) 1.0)
        (return (`local.JumpLocation`) true)
        (else
          (`KismetSystemLibrary.DrawDebugSphere` _returnvalue 25.0 12 (struct :`G` 0.188994 :`B` 1.0 :`A` 1.0) 1.0)
          (return _returnvalue false))))))

(fn `GetJumpLocation`
  (returns (ReturnValue :type "Vector Structure"))
  (return (`KismetMathLibrary.MakeVector` (+ (.x (`Actor.K2_GetActorLocation` (`self.CombatTarget`))) (* (.x (`KismetMathLibrary.Normal` (- (`Actor.K2_GetActorLocation` (`self.Character`)) (`Actor.K2_GetActorLocation` (`self.CombatTarget`))))) 225.0)) (.y (`Actor.K2_GetActorLocation` (`self.Character`))) (.z (`Actor.K2_GetActorLocation` (`self.Character`))))))