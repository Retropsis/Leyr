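; GA_Leap is an AI movement gameplay ability that makes a toad-animated character leap forward by a random short, average or long strength.
; That strength scales the Toad_Leap Paper animation's play rate and the force and duration of an additive root motion constant force, applied after a Jump.
; The ability ends when the force finishes or the animation completes or is cancelled.
; It also stores actor and leap locations, unused in this graph.
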(event `self.K2_OnEndAbility`
  (params (bWasCancelled :type Boolean))
  (`self.PrepareToEndAbility`))

(event `self.K2_ActivateAbility`
  (bind _returnvalue (`self.GetAvatarActorFromActorInfo`))
  (bind _strength (`self.Strength`))
  (`self.InitAbility`)
  (bind _output_get (set `self.StrengthSelection` (`KismetMathLibrary.RandomIntegerInRange` 0 2)))
  (bind _output_get_2 (set `self.Strength` (select `int` _output_get :`0` (`self.ShortStrength`) :`1` (`self.AverageStrength`) :`2` (`self.LongStrength`))))
  (`PaperZDPlaySlotOverrideAction.PlayAnimationOverrideWithCallbacks` (`self.PaperAnimInstance`) "/Game/AI/Toad/AnimSequences/Toad_Leap.Toad_Leap" "DefaultSlot" (* _output_get_2 0.58)
    (:`then`
      (set `self.ActorLocation` (`Actor.K2_GetActorLocation` (`self.GetAvatarActorFromActorInfo`)))
      (set `self.LeapLocation` (- (`Actor.K2_GetActorLocation` _returnvalue) (* (`Actor.GetActorForwardVector` _returnvalue) (select `int` (`KismetMathLibrary.RandomIntegerInRange` 0 2) :`0` (`self.ShortStrength`) :`1` (`self.AverageStrength`) :`2` (`self.LongStrength`)))))
      (`Character.Jump` (cast `Character` (`self.GetAvatarActorFromActorInfo`) :!pure true))
      (`AbilityTask_ApplyRootMotionConstantForce.ApplyRootMotionConstantForce` "None" (`Actor.GetActorForwardVector` (`self.GetAvatarActorFromActorInfo`)) (* _strength 125.0) (* _strength 0.58) true null "MaintainLastRootMotionVelocity"
        (:`OnFinish`
          (`self.K2_EndAbility`))))
    (:`OnCompleted`
      (`self.K2_EndAbility` :!label _label))
    (:`OnCancelled`
      (goto _label))))