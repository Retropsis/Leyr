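; GA_Leap_DeepHopper is an AI movement ability that makes the Deep Hopper jump forward with a random short, average or long strength.
; It plays the leap montage on the multi-part flipbook mesh and messages the character's anim instances to switch to Leap, then back to Idle on end.
; A jump plus additive root-motion force drives the hop, with strength scaling montage rate, force and duration.
; Either montage or force finishing ends the ability.
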(event `self.K2_OnEndAbility`
  (params (bWasCancelled :type Boolean))
  (`self.PrepareToEndAbility`)
  (message `MultiPartAIInterface.UpdateMultiPartAnimInstances` (`self.MultiPartAICharacter`) "Idle"))

(event `self.K2_ActivateAbility`
  (bind _returnvalue (`self.GetAvatarActorFromActorInfo`))
  (bind _strength (`self.Strength`))
  (`self.InitAbility`)
  (bind _asmulti_part_aicharacter (cast `MultiPartAICharacter` (`self.GetAvatarActorFromActorInfo`)))
  (set `self.MultiPartAICharacter` _asmulti_part_aicharacter)
  (bind _output_get (set `self.StrengthSelection` (`KismetMathLibrary.RandomIntegerInRange` 0 2)))
  (bind _output_get_2 (set `self.Strength` (select `int` _output_get :`0` (`self.ShortStrength`) :`1` (`self.AverageStrength`) :`2` (`self.LongStrength`))))
  (`|PlayMontage` (`MultiPartAICharacter.MultiPartFlipbook` (`self.MultiPartAICharacter`)) "/Game/Assets/3D/Hopper/AM_DeepHopper_Leap.AM_DeepHopper_Leap" (* _output_get_2 2.0)
    (:`then`
      (message `MultiPartAIInterface.UpdateMultiPartAnimInstances` (`self.MultiPartAICharacter`) "Leap")
      (set `self.ActorLocation` (`Actor.K2_GetActorLocation` (`self.GetAvatarActorFromActorInfo`)))
      (set `self.LeapLocation` (- (`Actor.K2_GetActorLocation` _returnvalue) (* (`Actor.GetActorForwardVector` _returnvalue) (select `int` (`KismetMathLibrary.RandomIntegerInRange` 0 2) :`0` (`self.ShortStrength`) :`1` (`self.AverageStrength`) :`2` (`self.LongStrength`)))))
      (`Character.Jump` (cast `Character` (`self.GetAvatarActorFromActorInfo`) :!pure true))
      (`AbilityTask_ApplyRootMotionConstantForce.ApplyRootMotionConstantForce` "None" (`Actor.GetActorForwardVector` (`self.GetAvatarActorFromActorInfo`)) (* _strength 125.0) (* _strength 0.58) true null "MaintainLastRootMotionVelocity"
        (:`OnFinish`
          (`self.K2_EndAbility`))))
    (:`OnCompleted`
      (`self.K2_EndAbility` :!label _label))
    (:`OnInterrupted`
      (goto _label))))