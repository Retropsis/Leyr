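; Giant crocodile AI ability for a jump bite attack, triggered during the creature's ascent.
; An ascent attack gameplay event plays the bite montage on the multi-part flipbook mesh.
; Montage events drive a box trace that deals damage with a weapon cue on hit, plus a hit stop on the character.
; Montage blend-out flags the anim instance to end surfacing, and ending the ability sends an end-ability event to the avatar.
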(event `self.K2_OnEndAbility`
  (params (bWasCancelled :type Boolean))
  (`self.PrepareToEndAbility`)
  (`AbilitySystemBlueprintLibrary.SendGameplayEventToActor` (`self.GetAvatarActorFromActorInfo`) (struct :`TagName` "Montage.EndAbility")))

(event `self.K2_ActivateAbility`
  (`self.InitAbility`)
  (`AbilityTask_WaitGameplayEvent.WaitGameplayEvent` (struct :`TagName` "Montage.Ascent.Attack") null true
    (:`then`
      (bind _asmulti_part_aicharacter (cast `MultiPartAICharacter` (`self.GetAvatarActorFromActorInfo`)))
      (set `self.MultiPartAICharacter` _asmulti_part_aicharacter))
    (:`EventReceived`
      (`|PlayMontage` (`MultiPartAICharacter.MultiPartFlipbook` (`self.MultiPartAICharacter`)) "/Game/Assets/3D/Crocodile/AM_BiteAttck.AM_BiteAttck"
        (:`then`
          (`AbilityTask_WaitGameplayEvent.WaitGameplayEvent` (struct :`TagName` "Montage.Attack.1") null true
            (:`then`
              (`AbilityTask_WaitGameplayEvent.WaitGameplayEvent` (struct :`TagName` "Montage.HitStop") null true
                (:`EventReceived`
                  (bind _asbase_character (cast `BaseCharacter` (`self.GetAvatarActorFromActorInfo`)))
                  (`BaseCharacter.HitStop` _asbase_character 0.3 0.2))))
            (:`EventReceived`
              (bind _returnvalue (`self.BoxTrace` true))
              (`self.ForEachHitTryCausingDamage` _returnvalue)
              (if (`self.bHasHitTarget`)
                (`self.ExecuteDamageGameplayCue` (struct :`TagName` "GameplayCue.Weapon"))))))
        (:`OnCompleted`
          (`self.K2_EndAbility` :!label _label))
        (:`OnBlendOut`
          (bind _asabp_giant_crocodile (cast `/Game/AI/GiantCrocodile/ABP_GiantCrocodile` (`SkeletalMeshComponent.GetAnimInstance` (`MultiPartAICharacter.MultiPartFlipbook` (`self.MultiPartAICharacter`)))))
          (set `/Game/AI/GiantCrocodile/ABP_GiantCrocodile.bEndSurfacing` true _asabp_giant_crocodile)
          (goto _label))
        (:`OnInterrupted`
          (goto _label))))))