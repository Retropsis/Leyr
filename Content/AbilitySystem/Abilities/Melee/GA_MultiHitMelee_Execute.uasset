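; Gameplay ability for an execute melee attack that locks avatar movement while a tagged Paper animation override plays.
; A one-time gameplay event matching the montage tag removes the execute window tag, box-traces, and damages hostile blocking hits.
; A successful hit fires a single weapon gameplay cue above the loop's HitActor.
; Animation completion or cancellation restores movement, clears the player's attacking flag and ends the ability.
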(event `self.K2_OnEndAbility`
  (params (bWasCancelled :type Boolean)))

(event `self.K2_ActivateAbility`
  (`KismetSystemLibrary.PrintString` "Execute" true true (struct :`R` 0.7075 :`G` 1.0 :`A` 1.0))
  (set `self.HasHitTarget` false)
  (bind _returnvalue (message `CombatInterface.GetTaggedMontageByTag` (`self.GetAvatarActorFromActorInfo`) (`self.MontageTag`)))
  (bind ((`Montage` _montage) (`MontageTag` _montagetag)) (break `TaggedMontage` _returnvalue))
  (set `self.MontageTag` _montagetag)
  (set `self.Montage` _montage)
  (message `CombatInterface.SetMovementEnabled` (`self.GetAvatarActorFromActorInfo`) false)
  (bind _returnvalue_2 (message `CombatInterface.GetPaperAnimInstance` (`self.GetAvatarActorFromActorInfo`)))
  (`PaperZDPlaySlotOverrideAction.PlayAnimationOverrideWithCallbacks` _returnvalue_2 (`self.Montage`)
    (:`then`
      (`AbilityTask_WaitGameplayEvent.WaitGameplayEvent` (`self.MontageTag`) null true
        (:`EventReceived`
          (`AbilitySystemBlueprintLibrary.RemoveLooseGameplayTags` (`self.GetAvatarActorFromActorInfo`) (`BlueprintGameplayTagLibrary.MakeGameplayTagContainerFromTag` (struct :`TagName` "Abilities.Window.Execute")))
          (bind _returnvalue_3 (`self.BoxTrace` false))
          (for _array_element _returnvalue_3
            (bind (_bblockinghit _binitialoverlap _time _distance _location _impactpoint _normal _impactnormal _physmat _hitactor) (`GameplayStatics.BreakHitResult` _array_element))
            (set `self.HitActor` _hitactor)
            (if _bblockinghit
              (if (`LeyrAbilitySystemLibrary.IsHostile` (`self.HitActor`) (`self.GetAvatarActorFromActorInfo`))
                (`self.CauseDamage` (`self.HitActor`))
                (set `self.HasHitTarget` true))))
          (message `CombatInterface.GetImpactEffect` (`self.HitActor`))
          (if (`self.HasHitTarget`)
            (`self.K2_ExecuteGameplayCueWithParams` (struct :`TagName` "GameplayCue.Weapon") (`AbilitySystemBlueprintLibrary.MakeGameplayCueParameters` 0.0 0.0 (struct) (struct) (struct) (`BlueprintGameplayTagLibrary.MakeGameplayTagContainerFromTag` (`self.MontageTag`)) (struct) (+ (`Actor.K2_GetActorLocation` (`self.HitActor`)) (0.0 0.0 75.0)) (0.0 0.0 0.0) null (`self.GetAvatarActorFromActorInfo`) (`self.HitActor`)))))))
    (:`OnCompleted`
      (message `CombatInterface.SetMovementEnabled` (`self.GetAvatarActorFromActorInfo`) true :!label _label)
      (set `/Game/Player/BP_PlayerCharacter.IsAttacking` false (cast `/Game/Player/BP_PlayerCharacter` (`self.GetAvatarActorFromActorInfo`) :!pure true))
      (`self.K2_EndAbility`))
    (:`OnCancelled`
      (goto _label))))