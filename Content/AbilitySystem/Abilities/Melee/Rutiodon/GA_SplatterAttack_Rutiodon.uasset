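; Melee gameplay ability for the Rutiodon's splatter attack, which faces the combat target and strikes toward the ground beneath it.
; Plays a Paper2D animation override and the splatter montage, while the avatar runs a multi-part montage toward the computed destination.
; That destination comes from a downward trace under the target, falling back to a point ahead of the avatar.
; A montage-tag gameplay event triggers box-trace damage and, on hit, weapon/wound cues.
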(event `self.K2_OnEndAbility`
  (params (bWasCancelled :type Boolean))
  (`self.PrepareToEndAbility`))

(event `self.K2_ActivateAbility`
  (bind _returnvalue (`self.GetAvatarActorFromActorInfo`))
  (`self.InitAbility`)
  (bind _returnvalue_2 (message `EnemyInterface.GetCombatTarget` _returnvalue))
  (set `self.CombatTarget` _returnvalue_2)
  (message `CombatInterface.UpdateFacingTarget` _returnvalue (`Actor.K2_GetActorLocation` _returnvalue_2))
  (bind _returnvalue_3 (message `CombatInterface.GetTaggedMontageByTag` (`self.GetAvatarActorFromActorInfo`) (`BlueprintGameplayTagLibrary.MakeLiteralGameplayTag` (struct :`TagName` "Montage.Attack.2")) "Default"))
  (bind _output_get (set `self.TaggedMontage` _returnvalue_3))
  (bind ((`MontageTag` _montagetag) (`Montage` _montage)) (break `TaggedMontage` _output_get))
  (set `self.MontageTag` _montagetag)
  (`PaperZDPlaySlotOverrideAction.PlayAnimationOverrideWithCallbacks` (`self.PaperAnimInstance`) _montage
    (:`then`
      (`AbilityTask_PlayMontageAndWait.CreatePlayMontageAndWaitProxy` "None" "/Game/Assets/3D/Rutiodon/AM_Splatter.AM_Splatter"
        (:`then`
          (message `MultiPartAIInterface.PlayMultiPartMontages` (`self.GetAvatarActorFromActorInfo`) (`BlueprintGameplayTagLibrary.MakeLiteralGameplayTag` (struct :`TagName` "Montage.Attack.2")) (`self.CalculateTargetDestination`))
          (`AbilityTask_WaitGameplayEvent.WaitGameplayEvent` (`self.MontageTag`) null true
            (:`EventReceived`
              (bind _returnvalue_4 (`self.BoxTrace` true))
              (`self.ForEachHitTryCausingDamage` _returnvalue_4)
              (if (`self.bHasHitTarget`)
                (`self.ExecuteDamageGameplayCue` (struct :`TagName` "GameplayCue.Weapon") (struct :`TagName` "GameplayCue.Wound.Impact.Average.Random"))))))
        (:`OnCompleted`
          (`self.K2_EndAbility` :!label _label))
        (:`OnCancelled`
          (goto _label))))))

(fn `CalculateTargetDestination`
  (returns (TargetDestination :type "Vector Structure"))
  (bind _returnvalue (`self.GetAvatarActorFromActorInfo`))
  (bind _returnvalue_2 (`Actor.K2_GetActorLocation` (`self.CombatTarget`)))
  (`/Engine/EditorBlueprintResources/StandardMacros.IsValid` (`self.CombatTarget`)
    (:`Is Valid`
      (bind (_outhit _returnvalue_3) (`KismetSystemLibrary.LineTraceSingle` _returnvalue_2 (- _returnvalue_2 (0.0 0.0 200.0)) "TraceTypeQuery1" false (`|MakeArray` (`self.CombatTarget`) (`self.GetAvatarActorFromActorInfo`)) "ForDuration"))
      (if _returnvalue_3
        (return (`KismetMathLibrary.MakeVector` (.x (`.Location` (`GameplayStatics.BreakHitResult` _outhit))) 0.0 (+ (.z (`.Location` (`GameplayStatics.BreakHitResult` _outhit))) 33.0)))
        (else
          _)))
    (:`Is Not Valid`
      _))
  (return (+ (`Actor.K2_GetActorLocation` _returnvalue) (`KismetMathLibrary.MakeVector` (* (.x (`Actor.GetActorForwardVector` _returnvalue)) 125.0) 0.0 -25.0))))