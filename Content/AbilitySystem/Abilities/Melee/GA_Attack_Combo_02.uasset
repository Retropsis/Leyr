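; Gameplay Ability for the second melee combo attack, played as a PaperZD animation override.
; A montage-tag event triggers a box trace that attempts damage and fires a weapon GameplayCue on hit.
; Combo window events swap the first window's loose tag for this attack's, then remove it.
; Completion or cancellation clears IsAttacking and ends after a short delay; execute-window logic is present but disconnected.
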(event `self.K2_OnEndAbility`
  (params (bWasCancelled :type Boolean)))

(event `self.K2_ActivateAbility`
  (`self.InitAbility`)
  (`self.SetCurrentSequence`)
  (`PaperZDPlaySlotOverrideAction.PlayAnimationOverrideWithCallbacks` (`self.PaperAnimInstance`) (`self.SelectedMontage`)
    (:`then`
      (`AbilityTask_WaitGameplayEvent.WaitGameplayEvent` (`self.MontageTag`) null true
        (:`then`
          (`AbilityTask_WaitGameplayEvent.WaitGameplayEvent` (struct :`TagName` "Abilities.Combo.Window.Begin") null true
            (:`then`
              (`AbilityTask_WaitGameplayEvent.WaitGameplayEvent` (struct :`TagName` "Abilities.Combo.Window.End") null true
                (:`EventReceived`
                  (`AbilitySystemBlueprintLibrary.RemoveLooseGameplayTags` (`self.GetAvatarActorFromActorInfo`) (`self.ComboWindowTag`)))))
            (:`EventReceived`
              (`AbilitySystemBlueprintLibrary.RemoveLooseGameplayTags` (`self.GetAvatarActorFromActorInfo`) (`BlueprintGameplayTagLibrary.MakeGameplayTagContainerFromTag` (struct :`TagName` "Abilities.Combo.Window.1")))
              (`AbilitySystemBlueprintLibrary.AddLooseGameplayTags` (`self.GetAvatarActorFromActorInfo`) (`self.ComboWindowTag`)))))
        (:`EventReceived`
          ;[0 0 0] Box Trace Event
          (bind _returnvalue (`self.BoxTrace` false))
          (`self.ForEachHitTryCausingDamage` _returnvalue)
          (if (`self.bHasHitTarget`)
            (`self.K2_ExecuteGameplayCueWithParams` (struct :`TagName` "GameplayCue.Weapon") (`AbilitySystemBlueprintLibrary.MakeGameplayCueParameters` 0.0 0.0 (struct) (struct) (struct) (`BlueprintGameplayTagLibrary.MakeGameplayTagContainerFromTag` (`self.MontageTag`)) (struct) (+ (`Actor.K2_GetActorLocation` (`self.HitActor`)) (0.0 0.0 75.0)) (0.0 0.0 0.0) null (`self.GetAvatarActorFromActorInfo`) (`self.HitActor`)))))))
    (:`OnCompleted`
      (`self.PrepareToEndAbility` :!label _label)
      (set `PlayerCharacter.bIsAttacking` false (cast `PlayerCharacter` (`self.GetAvatarActorFromActorInfo`) :!pure true))
      (`KismetSystemLibrary.Delay` 0.2)
      (`self.K2_EndAbility`))
    (:`OnCancelled`
      (goto _label))))