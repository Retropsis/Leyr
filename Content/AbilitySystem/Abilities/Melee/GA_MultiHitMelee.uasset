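; Gameplay ability for combo-indexed melee attacks on Paper2D-animated characters, locking movement while each attack plays.
; On activation it queries the avatar through interface messages for the combo index, its tagged montage and the Paper anim instance, then plays that animation as an override.
; The montage's tag is awaited once as a gameplay event, triggering a box trace that damages a blocking hit.
; Completion or cancellation restores movement and ends the ability.
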(event `self.K2_OnEndAbility`
  (params (bWasCancelled :type Boolean)))

(event `self.K2_ActivateAbility`
  (bind _returnvalue (`self.GetAvatarActorFromActorInfo`))
  (message `CombatInterface.SetMovementEnabled` (`self.GetAvatarActorFromActorInfo`) false)
  (bind _returnvalue_2 (message `CombatInterface.GetAttackComboIndex` _returnvalue))
  (bind _returnvalue_3 (message `CombatInterface.GetTaggedMontageByIndex` _returnvalue _returnvalue_2))
  (bind _returnvalue_4 (message `CombatInterface.GetPaperAnimInstance` (`self.GetAvatarActorFromActorInfo`)))
  (bind ((`Montage` _montage) (`MontageTag` _montagetag)) (break `TaggedMontage` _returnvalue_3))
  (set `self.MontageTag` _montagetag)
  (`PaperZDPlaySlotOverrideAction.PlayAnimationOverrideWithCallbacks` _returnvalue_4 _montage
    (:`then`
      (`AbilityTask_WaitGameplayEvent.WaitGameplayEvent` _montagetag null true
        (:`EventReceived`
          (bind _returnvalue_5 (`self.BoxTrace`))
          (bind (_bblockinghit _binitialoverlap _time _distance _location _impactpoint _normal _impactnormal _physmat _hitactor) (`GameplayStatics.BreakHitResult` _returnvalue_5))
          (set `self.HitActor` _hitactor)
          (if _bblockinghit
            (`self.CauseDamage` (`self.HitActor`))))))
    (:`OnCompleted`
      (message `CombatInterface.SetMovementEnabled` (`self.GetAvatarActorFromActorInfo`) true :!label _label)
      (`self.K2_EndAbility`))
    (:`OnCancelled`
      (goto _label))))