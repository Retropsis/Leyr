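; Melee attack gameplay ability for the Loppestre, which turns toward its combat target and strikes with a pincer.
; It layers a tag-selected Paper animation override, matching multi-part montages and the right-pincer montage.
; A gameplay event matching the montage tag triggers one box trace that applies damage, with weapon and wound cues on a hit.
; Montage completion or cancellation ends the ability, which returns the multi-part animations to Idle.
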(event `self.K2_OnEndAbility`
  (params (bWasCancelled :type Boolean))
  (`self.PrepareToEndAbility`)
  (message `MultiPartAIInterface.UpdateMultiPartAnimInstances` (`self.GetAvatarActorFromActorInfo`) "Idle"))

(event `self.K2_ActivateAbility`
  (bind _returnvalue (`self.GetAvatarActorFromActorInfo`))
  (`self.InitAbility`)
  (bind _returnvalue_2 (message `EnemyInterface.GetCombatTarget` _returnvalue))
  (message `CombatInterface.UpdateFacingTarget` _returnvalue (`Actor.K2_GetActorLocation` _returnvalue_2))
  (bind _returnvalue_3 (message `CombatInterface.GetTaggedMontageByTag` (`self.GetAvatarActorFromActorInfo`) (`BlueprintGameplayTagLibrary.MakeLiteralGameplayTag` (struct :`TagName` "Montage.Attack.1")) "Default"))
  (bind _output_get (set `self.TaggedMontage` _returnvalue_3))
  (bind ((`MontageTag` _montagetag) (`Montage` _montage)) (break `TaggedMontage` _output_get))
  (set `self.MontageTag` _montagetag)
  (`PaperZDPlaySlotOverrideAction.PlayAnimationOverrideWithCallbacks` (`self.PaperAnimInstance`) _montage
    (:`then`
      (message `MultiPartAIInterface.PlayMultiPartMontages` (`self.GetAvatarActorFromActorInfo`) (`BlueprintGameplayTagLibrary.MakeLiteralGameplayTag` (struct :`TagName` "Montage.Attack.1")))
      (`AbilityTask_PlayMontageAndWait.CreatePlayMontageAndWaitProxy` "None" "/Game/Assets/3D/Loppestre/AM_Pincer_R_Attack.AM_Pincer_R_Attack"
        (:`then`
          (`AbilityTask_WaitGameplayEvent.WaitGameplayEvent` (`self.MontageTag`) null true
            (:`EventReceived`
              (bind _returnvalue_4 (`self.BoxTrace` false))
              (`self.ForEachHitTryCausingDamage` _returnvalue_4)
              (if (`self.bHasHitTarget`)
                (`self.ExecuteDamageGameplayCue` (struct :`TagName` "GameplayCue.Weapon") (struct :`TagName` "GameplayCue.Wound.Impact.Average.Random"))))))
        (:`OnCompleted`
          (`self.K2_EndAbility` :!label _label))
        (:`OnCancelled`
          (goto _label))))))