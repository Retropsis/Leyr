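; Gameplay ability for a melee attack that only runs while the avatar's combat state is Swimming, otherwise ending immediately.
; It picks a sequence and plays it as a Paper2D animation override, waiting once for the montage tag event to box trace and damage targets.
; A hit fires a weapon gameplay cue above the hit actor.
; Completion or cancellation prepares cleanup and ends after a brief delay.
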(event `self.K2_ActivateAbility`
  (bind _returnvalue (message `CombatInterface.GetCombatState` (`self.GetAvatarActorFromActorInfo`)))
  (if (`|EnumEquality` _returnvalue "Swimming")
    (`self.InitAbility`)
    (`self.SetCurrentSequence`)
    (`PaperZDPlaySlotOverrideAction.PlayAnimationOverrideWithCallbacks` (`self.PaperAnimInstance`) (`self.SelectedMontage`)
      (:`then`
        (`AbilityTask_WaitGameplayEvent.WaitGameplayEvent` (`self.MontageTag`) null true
          (:`EventReceived`
            (bind _returnvalue_2 (`self.BoxTrace` true))
            (`self.ForEachHitTryCausingDamage` _returnvalue_2)
            (if (`self.bHasHitTarget`)
              (`self.K2_ExecuteGameplayCueWithParams` (struct :`TagName` "GameplayCue.Weapon") (`AbilitySystemBlueprintLibrary.MakeGameplayCueParameters` 0.0 0.0 (struct) (struct) (struct) (`BlueprintGameplayTagLibrary.MakeGameplayTagContainerFromTag` (`self.MontageTag`)) (struct) (+ (`Actor.K2_GetActorLocation` (`self.HitActor`)) (0.0 0.0 75.0)) (0.0 0.0 0.0) null (`self.GetAvatarActorFromActorInfo`) (`self.HitActor`)))))))
      (:`OnCompleted`
        (`self.PrepareToEndAbility` :!label _label)
        (`KismetSystemLibrary.Delay` 0.2)
        (`self.K2_EndAbility`))
      (:`OnCancelled`
        (goto _label)))
    (else
      (`self.K2_EndAbility`))))