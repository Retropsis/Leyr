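; Gameplay ability for a Paper2D melee attack, named for use on ground slopes.
; On activation it selects a sequence and plays it as an animation override, waiting for one montage-tag gameplay event.
; That event runs a box trace, applies damage to hits and, on a hit, fires a weapon gameplay cue just above the target.
; When the animation completes or is cancelled, it prepares to end, then ends after a short delay.
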(event `self.K2_ActivateAbility`
  (`self.InitAbility`)
  (`self.SetCurrentSequence`)
  (`PaperZDPlaySlotOverrideAction.PlayAnimationOverrideWithCallbacks` (`self.PaperAnimInstance`) (`self.SelectedMontage`)
    (:`then`
      (`AbilityTask_WaitGameplayEvent.WaitGameplayEvent` (`self.MontageTag`) null true
        (:`EventReceived`
          (bind _returnvalue (`self.BoxTrace` false))
          (`self.ForEachHitTryCausingDamage` _returnvalue)
          (if (`self.bHasHitTarget`)
            (`self.K2_ExecuteGameplayCueWithParams` (struct :`TagName` "GameplayCue.Weapon") (`AbilitySystemBlueprintLibrary.MakeGameplayCueParameters` 0.0 0.0 (struct) (struct) (struct) (`BlueprintGameplayTagLibrary.MakeGameplayTagContainerFromTag` (`self.MontageTag`)) (struct) (+ (`Actor.K2_GetActorLocation` (`self.HitActor`)) (0.0 0.0 75.0)) (0.0 0.0 0.0) null (`self.GetAvatarActorFromActorInfo`) (`self.HitActor`)))))))
    (:`OnCompleted`
      (`self.PrepareToEndAbility` :!label _label)
      (`KismetSystemLibrary.Delay` 0.2)
      (`self.K2_EndAbility`))
    (:`OnCancelled`
      (goto _label))))