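; Melee whip gameplay ability that spawns a BP_Whip actor while the avatar plays its 2D use animation.
; On activation it starts the animation override, spawns the whip at the avatar's transform and attaches it to the weapon combat socket, keeping world transform.
; Animation completion or cancellation notifies the whip that the attack finished, then ends the ability after a short delay.
; Ending destroys the whip and runs end preparation, both only if the whip is valid.
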(event `self.K2_OnEndAbility`
  (params (bWasCancelled :type Boolean))
  (`KismetSystemLibrary.PrintString` "End Ability" true true (struct :`R` 1.0 :`G` 0.021536 :`A` 1.0) 4.0)
  (bind _bp_whip (`self.BP_Whip`)
    (:`then`
      (`Actor.K2_DestroyActor` _bp_whip)
      (`self.PrepareToEndAbility`))
    (:`else`)))

(event `self.K2_ActivateAbility`
  (`self.InitAbility`)
  (`PaperZDPlaySlotOverrideAction.PlayAnimationOverrideWithCallbacks` (`self.PaperAnimInstance`) "/Game/Assets/Character/AnimSequences/Character_Use.Character_Use"
    (:`then`
      (bind _returnvalue (`|SpawnActorFromClass` "/Game/AbilitySystem/Actor/Weapon/BP_Whip.BP_Whip_C" (`Actor.GetTransform` (`self.GetAvatarActorFromActorInfo`)) "AlwaysSpawn" "MultiplyWithRoot" null null))
      (bind _output_get (set `self.BP_Whip` _returnvalue))
      (`Actor.K2_AttachToComponent` _output_get (`Actor.RootComponent` (`self.GetAvatarActorFromActorInfo`)) "CombatSocket.Weapon" "KeepWorld" "KeepWorld" "KeepWorld" true))
    (:`OnCompleted`
      (`Whip.HandleAttackFinished` (`self.BP_Whip`) :!label _label)
      (`KismetSystemLibrary.Delay` 1.0)
      (`self.K2_EndAbility`))
    (:`OnCancelled`
      (goto _label))))