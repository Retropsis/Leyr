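; Monk martial arts melee ability that plays an attack animation chosen from the current combat state.
; It applies a block-direction rule tag while active, plays the sequence as a Paper animation override and ends when that completes or is cancelled.
; Animation-driven gameplay events trigger a box trace for damage with Monk weapon and wound cues, hit stop, and an impulse on the avatar.
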(event `self.K2_OnEndAbility`
  (params (bWasCancelled :type Boolean))
  (`self.PrepareToEndAbilityWithParams` (make `EndAbilityParams` true (struct :`GameplayTags` (struct :`(TagName` "CombatState.Rule.Block.Direction"))))))

(event `self.K2_ActivateAbility`
  (`self.K2_CommitAbility`)
  (`self.InitAbilityWithParams` (make `InitAbilityParams` true (struct :`GameplayTags` (struct :`(TagName` "CombatState.Rule.Block.Direction")))))
  (`self.SelectMontageTagFromCombatState`)
  (`self.SetCurrentSequence`)
  (bind _selectedmontage (`self.SelectedMontage`)
    (:`then`
      (`PaperZDPlaySlotOverrideAction.PlayAnimationOverrideWithCallbacks` (`self.PaperAnimInstance`) _selectedmontage
        (:`then`
          (`AbilityTask_WaitGameplayEvent.WaitGameplayEvent` (`self.MontageTag`) null true
            (:`then`
              (`AbilityTask_WaitGameplayEvent.WaitGameplayEvent` (struct :`TagName` "Montage.HitStop") null true
                (:`then`
                  (`AbilityTask_WaitGameplayEvent.WaitGameplayEvent` (struct :`TagName` "Montage.Impulse") null true
                    (:`EventReceived`
                      (message `CombatInterface.AddImpulse` (`self.GetAvatarActorFromActorInfo`) (`self.HitImpulse`)))))
                (:`EventReceived`
                  (`self.ApplyHitStop`))))
            (:`EventReceived`
              ;[0 0 0] Box Trace Event
              (bind _returnvalue (`self.BoxTrace` false))
              (`self.ForEachHitTryCausingDamage` _returnvalue)
              (if (`self.bHasHitTarget`)
                (`self.ExecuteDamageGameplayCue` (struct :`TagName` "GameplayCue.Weapon.Monk") (struct :`TagName` "GameplayCue.Wound.Impact.Average.Random"))))))
        (:`OnCompleted`
          (`self.K2_EndAbility` :!label _label))
        (:`OnCancelled`
          (goto _label))))
    (:`else`
      (goto _label))))