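; Melee attack gameplay ability that plays a random attack animation from the avatar and damages a hostile it hits.
; The animation plays as a Paper animation override, and the ability ends when it completes or is cancelled.
; A one-shot gameplay event matching the attack's tag triggers a box trace, applies damage and fires a weapon GameplayCue at the target.
; Target-facing and radius-based hit logic remain but are disconnected.
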(event `self.K2_ActivateAbility`
  (bind _returnvalue (`self.GetAvatarActorFromActorInfo`))
  (set `self.HasHitTarget` false)
  (bind _returnvalue_2 (message `CombatInterface.GetPaperAnimInstance` _returnvalue))
  (bind _returnvalue_3 (message `CombatInterface.GetAttackMontages` _returnvalue))
  (bind _output_get (set `self.TaggedMontage` (`KismetArrayLibrary.Array_Random` _returnvalue_3)))
  (bind (_montage _montagetag) (break `TaggedMontage` _output_get))
  (`PaperZDPlaySlotOverrideAction.PlayAnimationOverrideWithCallbacks` _returnvalue_2 _montage
    (:`then`
      (`AbilityTask_WaitGameplayEvent.WaitGameplayEvent` _montagetag null true
        (:`EventReceived`
          (bind _returnvalue_4 (`self.BoxTrace`))
          (bind (_bblockinghit _binitialoverlap _time _distance _location _impactpoint _normal _impactnormal _physmat _hitactor) (`GameplayStatics.BreakHitResult` _returnvalue_4))
          (set `self.HitActor` _hitactor)
          (if _bblockinghit
            (if (`LeyrAbilitySystemLibrary.IsHostile` (`self.HitActor`) (`self.GetAvatarActorFromActorInfo`))
              (`self.CauseDamage` (`self.HitActor`))
              (set `self.HasHitTarget` true)
              (message `CombatInterface.GetImpactEffect` (`self.HitActor`))
              (if (`self.HasHitTarget`)
                (`self.K2_ExecuteGameplayCueWithParams` (struct :`TagName` "GameplayCue.Weapon") (`AbilitySystemBlueprintLibrary.MakeGameplayCueParameters` 0.0 0.0 (struct) (struct) (struct) (`BlueprintGameplayTagLibrary.MakeGameplayTagContainerFromTag` (`.MontageTag` (break `TaggedMontage` (`self.TaggedMontage`)))) (struct) (+ (`Actor.K2_GetActorLocation` (`self.HitActor`)) (0.0 0.0 75.0)) (0.0 0.0 0.0) null (`self.GetAvatarActorFromActorInfo`) (`self.HitActor`)))))))))
    (:`OnCompleted`
      (`self.K2_EndAbility` :!label _label))
    (:`OnCancelled`
      (goto _label))))