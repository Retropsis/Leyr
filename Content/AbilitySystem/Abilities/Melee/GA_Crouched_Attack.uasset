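; Gameplay ability for a crouched melee attack, run only when the avatar's combat state is Unoccupied.
; It locks movement and plays a PaperZD animation override chosen by tag, switching montage and setting gravity scale if airborne.
; A gameplay event matching the montage tag triggers a box trace that damages hostile actors and fires a weapon GameplayCue on hit.
; Completion or cancellation restores movement and gravity, then ends the ability after a short delay.
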(event `self.K2_ActivateAbility`
  (bind _returnvalue (`self.GetAvatarActorFromActorInfo`))
  (bind _returnvalue_2 (`self.GetAvatarActorFromActorInfo`))
  (bind _returnvalue_3 (message `CombatInterface.GetCombatState` (`self.GetAvatarActorFromActorInfo`)))
  (if (`|EnumEquality` _returnvalue_3 "Unoccupied")
    (bind _returnvalue_4 (message `CombatInterface.IsCharacterAirborne` _returnvalue_2))
    (bind _returnvalue_5 (message `CombatInterface.GetGravityScale` _returnvalue_2))
    (message `CombatInterface.SetGravityScale` _returnvalue_2 (`KismetMathLibrary.SelectFloat` 1.0 _returnvalue_5 _returnvalue_4))
    (set `self.HasHitTarget` false)
    (set `self.MontageTag` (select `bool` _returnvalue_4 :`false` (`self.MainMontageTag`) :`true` (`self.AlternativeMontageTag`)))
    (message `CombatInterface.SetMovementEnabled` (`self.GetAvatarActorFromActorInfo`) false)
    (bind _returnvalue_6 (message `CombatInterface.GetPaperAnimInstance` _returnvalue))
    (bind _returnvalue_7 (message `CombatInterface.GetTaggedMontageByTag` _returnvalue (`self.MontageTag`)))
    (bind ((`Montage` _montage) (`MontageTag` _montagetag)) (break `TaggedMontage` _returnvalue_7))
    (`PaperZDPlaySlotOverrideAction.PlayAnimationOverrideWithCallbacks` _returnvalue_6 _montage
      (:`then`
        (`AbilityTask_WaitGameplayEvent.WaitGameplayEvent` _montagetag null true
          (:`EventReceived`
            (bind _returnvalue_8 (`self.BoxTrace`))
            (for _array_element _returnvalue_8
              (bind (_bblockinghit _binitialoverlap _time _distance _location _impactpoint _normal _impactnormal _physmat _hitactor) (`GameplayStatics.BreakHitResult` _array_element))
              (set `self.HitActor` _hitactor)
              (if _bblockinghit
                (if (`LeyrAbilitySystemLibrary.IsHostile` (`self.HitActor`) (`self.GetAvatarActorFromActorInfo`))
                  (`self.CauseDamage` (`self.HitActor`))
                  (set `self.HasHitTarget` true))))
            (message `CombatInterface.GetImpactEffect` (`self.HitActor`))
            (if (`self.HasHitTarget`)
              (`self.K2_ExecuteGameplayCueWithParams` (struct :`TagName` "GameplayCue.Weapon") (`AbilitySystemBlueprintLibrary.MakeGameplayCueParameters` 0.0 0.0 (struct) (struct) (struct) (`BlueprintGameplayTagLibrary.MakeGameplayTagContainerFromTag` (`.MontageTag` (break `TaggedMontage` (`self.TaggedMontage`)))) (struct) (+ (`Actor.K2_GetActorLocation` (`self.HitActor`)) (0.0 0.0 75.0)) (0.0 0.0 0.0) null (`self.GetAvatarActorFromActorInfo`) (`self.HitActor`)))))))
      (:`OnCompleted`
        (message `CombatInterface.SetMovementEnabled` (`self.GetAvatarActorFromActorInfo`) true :!label _label)
        (message `CombatInterface.ResetGravityScale` (`self.GetAvatarActorFromActorInfo`))
        (`KismetSystemLibrary.Delay` 0.66)
        (`self.K2_EndAbility`))
      (:`OnCancelled`
        (goto _label)))
    (else
      (`self.K2_EndAbility`))))