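; Melee gameplay ability for a jump bite attack that turns the avatar toward its combat target and plays a randomly picked PaperZD attack animation.
; A gameplay event matching the montage tag triggers one box trace that applies damage and, on a hit, fires a weapon gameplay cue.
; When the animation completes or is cancelled, the character falls under set gravity briefly, then a timer restores Flying movement and ends the ability.
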(event `self.K2_ActivateAbility`
  (bind _returnvalue (`self.GetAvatarActorFromActorInfo`))
  (bind _charactermovement (`Character.CharacterMovement` (cast `Character` (`self.GetAvatarActorFromActorInfo`) :!pure true)))
  (`self.InitAbility`)
  (bind _returnvalue_2 (message `EnemyInterface.GetCombatTarget` _returnvalue))
  (message `CombatInterface.UpdateFacingTarget` _returnvalue (`Actor.K2_GetActorLocation` _returnvalue_2))
  (bind _returnvalue_3 (message `CombatInterface.GetAttackMontages` (`self.GetAvatarActorFromActorInfo`)))
  (bind ((`DamageType` _damagetype) (`MontageTag` _montagetag) (`Montage` _montage)) (break `TaggedMontage` (`KismetArrayLibrary.Array_Random` _returnvalue_3)))
  (set `self.MontageTag` _montagetag)
  (`PaperZDPlaySlotOverrideAction.PlayAnimationOverrideWithCallbacks` (`self.PaperAnimInstance`) _montage
    (:`then`
      (`AbilityTask_WaitGameplayEvent.WaitGameplayEvent` (`self.MontageTag`) null true
        (:`EventReceived`
          (bind _returnvalue_4 (`self.BoxTrace` false))
          (`self.ForEachHitTryCausingDamage` _returnvalue_4)
          (if (`self.bHasHitTarget`)
            (`self.K2_ExecuteGameplayCueWithParams` (struct :`TagName` "GameplayCue.Weapon") (`AbilitySystemBlueprintLibrary.MakeGameplayCueParameters` 0.0 0.0 (struct) (struct) (struct) (`BlueprintGameplayTagLibrary.MakeGameplayTagContainerFromTag` (`self.MontageTag`)) (struct) (+ (`Actor.K2_GetActorLocation` (`self.HitActor`)) (0.0 0.0 75.0)) (0.0 0.0 0.0) null (`self.GetAvatarActorFromActorInfo`) (`self.HitActor`)))))))
    (:`OnCompleted`
      (`CharacterMovementComponent.SetMovementMode` _charactermovement "MOVE_Falling" 0 :!label _label)
      (`KismetSystemLibrary.K2_SetTimerDelegate` (delegate `ResetMovementMode`) 0.15)
      (set `CharacterMovementComponent.GravityScale` 3.5 _charactermovement))
    (:`OnCancelled`
      (goto _label))))

(event `ResetMovementMode`
  (`CharacterMovementComponent.SetMovementMode` (`Character.CharacterMovement` (cast `Character` (`self.GetAvatarActorFromActorInfo`) :!pure true)) "MOVE_Flying" 0)
  (`self.PrepareToEndAbility`)
  (`self.K2_EndAbility`))