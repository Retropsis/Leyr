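; Gameplay ability for a one-handed melee roll attack, using a Paper animation instance.
; On activation it sets the avatar's RollingEnd combat state, initializes, picks the sequence and plays it as an animation override.
; A gameplay event matching the montage tag triggers one box trace that attempts damage and fires a gameplay cue above the hit actor.
; Animation completion or cancellation clears the player's attacking flag and ends the ability.
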(event `self.K2_OnEndAbility`
  (params (bWasCancelled :type Boolean)))

(event `self.K2_ActivateAbility`
  (message `CombatInterface.SetCombatStateToHandle` (`self.GetAvatarActorFromActorInfo`) "RollingEnd")
  (`self.InitAbility`)
  (`self.SetCurrentSequence`)
  (`PaperZDPlaySlotOverrideAction.PlayAnimationOverrideWithCallbacks` (`self.PaperAnimInstance`) (`self.SelectedMontage`)
    (:`then`
      (`AbilityTask_WaitGameplayEvent.WaitGameplayEvent` (`self.MontageTag`) null true
        (:`EventReceived`
          (bind _returnvalue (`self.BoxTrace` true))
          (`self.ForEachHitTryCausingDamage` _returnvalue)
          (if (`self.bHasHitTarget`)
            (`self.K2_ExecuteGameplayCueWithParams` (struct :`TagName` "GameplayCue.Execute") (`AbilitySystemBlueprintLibrary.MakeGameplayCueParameters` 0.0 0.0 (struct) (struct) (struct) (`BlueprintGameplayTagLibrary.MakeGameplayTagContainerFromTag` (`self.MontageTag`)) (struct) (+ (`Actor.K2_GetActorLocation` (`self.HitActor`)) (0.0 0.0 75.0)) (0.0 0.0 0.0) null (`self.GetAvatarActorFromActorInfo`) (`self.HitActor`)))))))
    (:`OnCompleted`
      (`self.PrepareToEndAbility` :!label _label)
      (set `PlayerCharacter.bIsAttacking` false (cast `PlayerCharacter` (`self.GetAvatarActorFromActorInfo`) :!pure true))
      (`self.K2_EndAbility`))
    (:`OnCancelled`
      (goto _label))))