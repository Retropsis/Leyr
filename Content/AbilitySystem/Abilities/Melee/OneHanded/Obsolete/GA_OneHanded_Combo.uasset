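; Gameplay ability for a one-handed melee combo attack, playing override animations on a Paper animation instance.
; Each step selects a tagged montage and waits for its gameplay event to box trace, damage hits and fire a weapon damage cue.
; Combo window begin and end events bracket an input wait, and a press loops back into the next step.
; When playback completes or cancels without a continuation, it clears the player's attacking flag and ends after a short delay.
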(event `self.K2_OnEndAbility`
  (params (bWasCancelled :type Boolean)))

(event `self.K2_ActivateAbility`
  (`self.InitAbility`)
  (`self.SelectMontageTagCombo` :!label _label)
  (`self.SetCurrentSequence`)
  (`PaperZDPlaySlotOverrideAction.PlayAnimationOverrideWithCallbacks` (`self.PaperAnimInstance`) (`self.SelectedMontage`)
    (:`then`
      (`AbilityTask_WaitGameplayEvent.WaitGameplayEvent` (`self.MontageTag`) null true
        (:`then`
          (`AbilityTask_WaitGameplayEvent.WaitGameplayEvent` (struct :`TagName` "Abilities.Combo.Window.Begin") null true
            (:`then`
              (`AbilityTask_WaitGameplayEvent.WaitGameplayEvent` (struct :`TagName` "Abilities.Combo.Window.End") null true
                (:`EventReceived`
                  (`self.OnComboWindowEnd`)
                  (set `self.bShouldEndAbility` true))))
            (:`EventReceived`
              (`self.OnComboWindowBegin`)
              (bind _asynctaskproxy (`AbilityTask_WaitInputPress.WaitInputPress` false)
                (:`then`
                  (set `self.WaitInputPressTask` _asynctaskproxy))
                (:`OnPress`
                  (set `self.bShouldEndAbility` false)
                  (goto _label))))))
        (:`EventReceived`
          ;[0 0 0] Box Trace Event
          (bind _returnvalue (`self.BoxTrace` false))
          (`self.ForEachHitTryCausingDamage` _returnvalue)
          (if (`self.bHasHitTarget`)
            (`self.ExecuteDamageGameplayCue` (struct :`TagName` "GameplayCue.Weapon"))))))
    (:`OnCompleted`
      ;[0 0 0] End Ability
      (if (`self.bShouldEndAbility`) :!label _label_2
        (`self.PrepareToEndAbility`)
        (set `PlayerCharacter.bIsAttacking` false (cast `PlayerCharacter` (`self.GetAvatarActorFromActorInfo`) :!pure true))
        (`KismetSystemLibrary.Delay` 0.2)
        (`self.K2_EndAbility`)))
    (:`OnCancelled`
      (goto _label_2))))