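; Gameplay ability for a one-handed crouched melee attack on a Paper2D animated character, filed under Obsolete.
; On activation it sets gravity scale to 1 if airborne, then plays the selected animation sequence as an override.
; A montage-tag gameplay event triggers a one-time box trace that tries to damage each hit and fires a weapon GameplayCue on success.
; Completion or cancellation resets gravity and ends the ability.
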(event `self.K2_ActivateAbility`
  (bind _returnvalue (`self.GetAvatarActorFromActorInfo`))
  (bind _returnvalue_2 (message `CombatInterface.IsCharacterAirborne` _returnvalue))
  (bind _returnvalue_3 (message `CombatInterface.GetGravityScale` _returnvalue))
  (message `CombatInterface.SetGravityScale` _returnvalue (`KismetMathLibrary.SelectFloat` 1.0 _returnvalue_3 _returnvalue_2))
  (`self.InitAbility`)
  (`self.SetCurrentSequence`)
  (`PaperZDPlaySlotOverrideAction.PlayAnimationOverrideWithCallbacks` (`self.PaperAnimInstance`) (`self.SelectedMontage`)
    (:`then`
      (`AbilityTask_WaitGameplayEvent.WaitGameplayEvent` (`self.MontageTag`) null true
        (:`EventReceived`
          (bind _returnvalue_4 (`self.BoxTrace` false))
          (`self.ForEachHitTryCausingDamage` _returnvalue_4)
          (if (`self.bHasHitTarget`)
            (`self.K2_ExecuteGameplayCueWithParams` (struct :`TagName` "GameplayCue.Weapon") (`AbilitySystemBlueprintLibrary.MakeGameplayCueParameters` 0.0 0.0 (struct) (struct) (struct) (`BlueprintGameplayTagLibrary.MakeGameplayTagContainerFromTag` (`self.MontageTag`)) (struct) (+ (`Actor.K2_GetActorLocation` (`self.HitActor`)) (0.0 0.0 75.0)) (0.0 0.0 0.0) null (`self.GetAvatarActorFromActorInfo`) (`self.HitActor`)))))))
    (:`OnCompleted`
      (`self.PrepareToEndAbility` :!label _label)
      (message `CombatInterface.ResetGravityScale` (`self.GetAvatarActorFromActorInfo`))
      (`self.K2_EndAbility`))
    (:`OnCancelled`
      (goto _label))))