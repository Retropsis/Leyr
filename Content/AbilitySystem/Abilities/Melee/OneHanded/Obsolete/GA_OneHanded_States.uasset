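; Obsolete gameplay ability for a one-handed melee attack, choosing its animation from the combat state.
; It commits, plays the selected sequence as a Paper animation override, and ends when playback completes or is cancelled.
; A one-shot gameplay event matching the montage tag triggers a box trace that tries to damage each hit.
; Successful hits execute a weapon damage gameplay cue and send a hit impulse message to the avatar.
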(event `self.K2_OnEndAbility`
  (params (bWasCancelled :type Boolean))
  (`self.PrepareToEndAbility`))

(event `self.K2_ActivateAbility`
  (`self.K2_CommitAbility`)
  (`self.InitAbility`)
  (`self.SelectMontageTagFromCombatState`)
  (`self.SetCurrentSequence`)
  (`PaperZDPlaySlotOverrideAction.PlayAnimationOverrideWithCallbacks` (`self.PaperAnimInstance`) (`self.SelectedMontage`)
    (:`then`
      (`AbilityTask_WaitGameplayEvent.WaitGameplayEvent` (`self.MontageTag`) null true
        (:`EventReceived`
          ;[0 0 0] Box Trace Event
          (bind _returnvalue (`self.BoxTrace` false))
          (`self.ForEachHitTryCausingDamage` _returnvalue)
          (if (`self.bHasHitTarget`)
            (`self.ExecuteDamageGameplayCue` (struct :`TagName` "GameplayCue.Weapon"))
            (if (`self.bHasHitTarget`)
              (message `CombatInterface.AddImpulse` (`self.GetAvatarActorFromActorInfo`) (`self.HitImpulse`)))))))
    (:`OnCompleted`
      (`self.K2_EndAbility` :!label _label))
    (:`OnCancelled`
      (goto _label))))