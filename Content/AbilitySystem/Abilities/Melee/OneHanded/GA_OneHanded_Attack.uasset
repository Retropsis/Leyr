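; One-handed melee attack ability that runs an input-driven combo on PaperAnimInstance and WeaponAnimInstance, blocking ground movement while active.
; Each step selects a sequence, plays paired character and weapon override animations, and box-traces for damage and impact cues on the montage's gameplay event.
; Combo window events let a press queue a loop back to the next step; otherwise the ability ends, and a hit-react cancellation always ends it.
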(event `self.K2_OnEndAbility`
  (params (bWasCancelled :type Boolean))
  (`self.PrepareToEndAbilityWithParams` (make `EndAbilityParams` true (struct :`GameplayTags` (struct :`(TagName` "CombatState.Rule.Block.Movement.Ground"))))))

(event `self.K2_ActivateAbility`
  (`self.InitAbilityWithParams` (make `InitAbilityParams` true (struct :`GameplayTags` (struct :`(TagName` "CombatState.Rule.Block.Movement.Ground")))))
  (`self.RestartCombo` :!label _label)
  (`self.SelectMontageTagCombo`)
  (`self.SetCurrentSequence`)
  (`PaperZDPlaySlotOverrideAction.PlayAnimationOverrideWithCallbacks` (`self.PaperAnimInstance`) (`self.SelectedMontage`)
    (:`then`
      (`PaperZDPlaySlotOverrideAction.PlayAnimationOverrideWithCallbacks` (`self.WeaponAnimInstance`) (`self.SelectedWeaponMontage`)
        (:`then`
          (`AbilityTask_WaitGameplayEvent.WaitGameplayEvent` (`self.MontageTag`) null true
            (:`then`
              (`AbilityTask_WaitGameplayEvent.WaitGameplayEvent` (struct :`TagName` "Abilities.Combo.Window.Begin") null true
                (:`then`
                  (`AbilityTask_WaitGameplayEvent.WaitGameplayEvent` (struct :`TagName` "Montage.Window.Combo") null true
                    (:`then`
                      (`AbilityTask_WaitGameplayEvent.WaitGameplayEvent` (struct :`TagName` "Abilities.Combo.Window.End") null true
                        (:`EventReceived`
                          (`self.OnComboWindowEnd`)
                          (set `self.bShouldEndAbility` true)
                          ;[0 0 0] End Ability
                          (if (`self.bShouldEndAbility`) :!label _label_2
                            (`self.K2_EndAbility` :!label _label_3)))))
                    (:`EventReceived`
                      (if (`self.bCueCombo`)
                        (set `self.bCueCombo` false)
                        (goto _label)))))
                (:`EventReceived`
                  (`self.OnComboWindowBegin`)
                  (bind _asynctaskproxy (`AbilityTask_WaitInputPress.WaitInputPress` false)
                    (:`then`
                      (set `self.WaitInputPressTask` _asynctaskproxy))
                    (:`OnPress`
                      (set `self.bShouldEndAbility` false)
                      (set `self.bCueCombo` true))))))
            (:`EventReceived`
              ;[0 0 0] Box Trace Event
              (bind _returnvalue (`self.BoxTrace` false))
              (`self.ForEachHitTryCausingDamage` _returnvalue)
              (if (`self.bHasHitTarget`)
                (`self.ExecuteDamageGameplayCue` (struct :`TagName` "GameplayCue.Weapon") (struct :`TagName` "GameplayCue.Wound.Impact.Average.Random"))))))))
    (:`OnCompleted`
      (goto _label_2))
    (:`OnCancelled`
      (if (`GameplayTagAssetInterface.HasMatchingGameplayTag` (`self.GetAbilitySystemComponentFromActorInfo`) (struct :`TagName` "StatusEffect.HitReact"))
        (goto _label_3)
        (else
          (goto _label_2))))))