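; Gameplay ability for Loppestre's melee spin attack against its current combat target.
; On activation it faces the target, plays the tagged Paper animation override, then starts timeline movement and multi-part montages aimed at an X-offset from the target.
; Alongside, AM_Spin_Attack plays; a gameplay event matching the montage tag triggers a one-time box trace, damage and impact cue.
; Montage completion or cancellation ends the ability, returning the multi-part animations to Idle.
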(event `self.K2_OnEndAbility`
  (params (bWasCancelled :type Boolean))
  (`self.PrepareToEndAbility`)
  (message `MultiPartAIInterface.UpdateMultiPartAnimInstances` (`self.GetAvatarActorFromActorInfo`) "Idle"))

(event `self.K2_ActivateAbility`
  (`self.InitAbility`)
  (bind _returnvalue (message `EnemyInterface.GetCombatTarget` (`self.GetAvatarActorFromActorInfo`)))
  (bind _output_get (set `self.CombatTargetLocation` (`Actor.K2_GetActorLocation` _returnvalue)))
  (message `CombatInterface.UpdateFacingTarget` (`self.GetAvatarActorFromActorInfo`) _output_get)
  (bind _returnvalue_2 (message `CombatInterface.GetTaggedMontageByTag` (`self.GetAvatarActorFromActorInfo`) (`BlueprintGameplayTagLibrary.MakeLiteralGameplayTag` (struct :`TagName` "Montage.Attack.2")) "Default"))
  (bind _output_get_2 (set `self.TaggedMontage` _returnvalue_2))
  (bind ((`MontageTag` _montagetag) (`Montage` _montage)) (break `TaggedMontage` _output_get_2))
  (set `self.MontageTag` _montagetag)
  (`PaperZDPlaySlotOverrideAction.PlayAnimationOverrideWithCallbacks` (`self.PaperAnimInstance`) _montage
    (:`then`
      (message `AIInterface.StartTimelineMovement` (`self.GetAvatarActorFromActorInfo`))
      (message `MultiPartAIInterface.PlayMultiPartMontages` (`self.GetAvatarActorFromActorInfo`) (`BlueprintGameplayTagLibrary.MakeLiteralGameplayTag` (struct :`TagName` "Montage.Attack.2")) (- (`self.CombatTargetLocation`) (`KismetMathLibrary.MakeVector` (* (.x (`Actor.GetActorForwardVector` (`self.GetAvatarActorFromActorInfo`))) 75.0))))
      (`AbilityTask_PlayMontageAndWait.CreatePlayMontageAndWaitProxy` "None" "/Game/Assets/3D/Loppestre/AM_Spin_Attack.AM_Spin_Attack"
        (:`then`
          (`AbilityTask_WaitGameplayEvent.WaitGameplayEvent` (`self.MontageTag`) null true
            (:`EventReceived`
              (bind _returnvalue_3 (`self.BoxTrace` false))
              (`self.ForEachHitTryCausingDamage` _returnvalue_3)
              (if (`self.bHasHitTarget`)
                (`self.ExecuteDamageGameplayCue` (struct :`TagName` "GameplayCue.Weapon") (struct :`TagName` "GameplayCue.Wound.Impact.Average.Random"))))))
        (:`OnCompleted`
          (`self.K2_EndAbility` :!label _label))
        (:`OnCancelled`
          (goto _label))))))