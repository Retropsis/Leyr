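; Melee combo gameplay ability that plays the selected attack as a Paper animation override.
; A montage-tag gameplay event runs a box trace, damages targets and fires a weapon GameplayCue on a hit.
; An execute-window event applies GE_Execute_Window, after which an input press stops the animation and ends the ability early.
; Animation completion or cancellation runs end preparation, clears the player's IsAttacking flag and ends the ability.
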(event `self.K2_OnEndAbility`
  (params (bWasCancelled :type Boolean)))

(event `self.K2_ActivateAbility`
  (`self.InitAbility`)
  (`self.SetCurrentComboSequence`)
  (`PaperZDPlaySlotOverrideAction.PlayAnimationOverrideWithCallbacks` (`self.PaperAnimInstance`) (`self.SelectedMontage`)
    (:`then`
      (`AbilityTask_WaitGameplayEvent.WaitGameplayEvent` (`self.MontageTag`) null true
        (:`then`
          (`AbilityTask_WaitGameplayEvent.WaitGameplayEvent` (struct :`TagName` "Montage.Window.Execute") null true
            (:`EventReceived`
              (`AbilitySystemComponent.BP_ApplyGameplayEffectToSelf` :`self` (`self.GetAbilitySystemComponentFromActorInfo`) :`GameplayEffectClass` "/Game/AbilitySystem/Effects/States/GE_Execute_Window.GE_Execute_Window_C" :`Level` 1.0)
              (`AbilityTask_WaitInputPress.WaitInputPress` false
                (:`OnPress`
                  (`PaperZDAnimInstance.StopAllAnimationOverrides` (`self.PaperAnimInstance`))
                  (`self.K2_EndAbility`))))))
        (:`EventReceived`
          (bind _returnvalue (`self.BoxTrace` false))
          (`self.ForEachHitTryCausingDamage` _returnvalue)
          (if (`self.bHasHitTarget`)
            (`self.K2_ExecuteGameplayCueWithParams` (struct :`TagName` "GameplayCue.Weapon") (`AbilitySystemBlueprintLibrary.MakeGameplayCueParameters` 0.0 0.0 (struct) (struct) (struct) (`BlueprintGameplayTagLibrary.MakeGameplayTagContainerFromTag` (`self.MontageTag`)) (struct) (+ (`Actor.K2_GetActorLocation` (`self.HitActor`)) (0.0 0.0 75.0)) (0.0 0.0 0.0) null (`self.GetAvatarActorFromActorInfo`) (`self.HitActor`)))))))
    (:`OnCompleted`
      (`self.PrepareToEndAbility` :!label _label)
      (set `PlayerCharacter.bIsAttacking` false (cast `PlayerCharacter` (`self.GetAvatarActorFromActorInfo`) :!pure true))
      (`self.K2_EndAbility`))
    (:`OnCancelled`
      (goto _label))))