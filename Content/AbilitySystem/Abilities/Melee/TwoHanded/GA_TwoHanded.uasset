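; Gameplay ability for a two-handed melee attack, pairing the character's PaperZD attack animation with a greatsword animation on the weapon.
; A gameplay event on the montage tag triggers a one-shot box trace that tries to damage each hit and fires a weapon damage cue when a target is hit.
; An end-ability event, or the character animation completing or being cancelled, clears the player's attacking flag and ends the ability.
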(event `self.K2_OnEndAbility`
  (params (bWasCancelled :type Boolean)))

(event `self.K2_ActivateAbility`
  (`self.InitAbility`)
  (`PaperZDPlaySlotOverrideAction.PlayAnimationOverrideWithCallbacks` (`self.PaperAnimInstance`) "/Game/Assets/Character/AnimSequences/2H_Attack.2H_Attack"
    (:`then`
      (`PaperZDPlaySlotOverrideAction.PlayAnimationOverrideWithCallbacks` (`self.WeaponAnimInstance`) "/Game/Assets/Equipment/TwoHanded/AnimSequences/GreatSword_Attack.GreatSword_Attack"
        (:`then`
          (`AbilityTask_WaitGameplayEvent.WaitGameplayEvent` (`self.MontageTag`) null true
            (:`then`
              (`AbilityTask_WaitGameplayEvent.WaitGameplayEvent` (struct :`TagName` "Montage.EndAbility") null true
                (:`EventReceived`
                  (`self.PrepareToEndAbility`)
                  (set `PlayerCharacter.bIsAttacking` false (cast `PlayerCharacter` (`self.GetAvatarActorFromActorInfo`) :!pure true))
                  (`self.K2_EndAbility`))))
            (:`EventReceived`
              ;[0 0 0] Box Trace Event
              (bind _returnvalue (`self.BoxTrace` false))
              (`self.ForEachHitTryCausingDamage` _returnvalue)
              (if (`self.bHasHitTarget`)
                (`self.ExecuteDamageGameplayCue` (struct :`TagName` "GameplayCue.Weapon"))))))))
    (:`OnCompleted`
      ;[0 0 0] End Ability
      (`self.PrepareToEndAbility` :!label _label)
      (set `PlayerCharacter.bIsAttacking` false (cast `PlayerCharacter` (`self.GetAvatarActorFromActorInfo`) :!pure true))
      (`KismetSystemLibrary.Delay` 0.1)
      (`self.K2_EndAbility`))
    (:`OnCancelled`
      (goto _label))))