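; Two-handed greatsword Execute melee ability that plays paired character and weapon animation overrides.
; A gameplay event during the start animation triggers a box trace that applies damage, with an Execute cue on hit.
; A successful execute launches a forward impulse dash that ignores a capsule collision channel until the ability ends; otherwise the end animation plays.
; Animation completion, cancellation or an end-ability event clears the attacking state and ends the ability.
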(event `self.K2_OnEndAbility`
  (params (bWasCancelled :type Boolean)))

(event `self.K2_ActivateAbility`
  (`self.InitAbility`)
  (`self.SetCurrentSequence`)
  (`PaperZDPlaySlotOverrideAction.PlayAnimationOverrideWithCallbacks` (`self.PaperAnimInstance`) "/Game/Assets/Character/AnimSequences/2H_Execute_Start.2H_Execute_Start"
    (:`then`
      (`PaperZDPlaySlotOverrideAction.PlayAnimationOverrideWithCallbacks` (`self.WeaponAnimInstance`) "/Game/Assets/Equipment/TwoHanded/AnimSequences/GreatSword_Execute_Start.GreatSword_Execute_Start"
        (:`then`
          (`AbilityTask_WaitGameplayEvent.WaitGameplayEvent` (`self.MontageTag`) null true
            (:`then`
              (`AbilityTask_WaitGameplayEvent.WaitGameplayEvent` (struct :`TagName` "Montage.EndAbility") null true
                (:`EventReceived`
                  (`self.PrepareToEndAbility`)
                  (set `PlayerCharacter.bIsAttacking` false (cast `PlayerCharacter` (`self.GetAvatarActorFromActorInfo`) :!pure true))
                  (`self.K2_EndAbility`))))
            (:`EventReceived`
              ;[0 0 0] Box Trace Event
              (bind _returnvalue (`self.BoxTrace` false))
              (`self.ForEachHitTryCausingDamage` _returnvalue)
              (if (`self.bExecuteSuccessful`)
                (`self.Dash`)
                (`PaperZDPlaySlotOverrideAction.PlayAnimationOverrideWithCallbacks` (`self.PaperAnimInstance`) "/Game/Assets/Character/AnimSequences/2H_Execute_Dash.2H_Execute_Dash"
                  (:`then`
                    (`PaperZDPlaySlotOverrideAction.PlayAnimationOverrideWithCallbacks` (`self.WeaponAnimInstance`) "/Game/Assets/Equipment/TwoHanded/AnimSequences/GreatSword_Execute_Dash.GreatSword_Execute_Dash"
                      (:`then`
                        (if (`self.bHasHitTarget`) :!label _label
                          (`self.ExecuteDamageGameplayCue` (struct :`TagName` "GameplayCue.Execute"))))))
                  (:`OnCompleted`
                    ;[0 0 0] End Ability
                    (`self.PrepareToEndAbility` :!label _label_2)
                    (`PrimitiveComponent.SetCollisionResponseToChannel` (`Character.CapsuleComponent` (cast `BaseCharacter` (`self.GetAvatarActorFromActorInfo`) :!pure true)) "ECC_GameTraceChannel2" "ECR_Block")
                    (set `PlayerCharacter.bIsAttacking` false (cast `PlayerCharacter` (`self.GetAvatarActorFromActorInfo`) :!pure true))
                    (`KismetSystemLibrary.Delay` 0.1)
                    (`self.K2_EndAbility`))
                  (:`OnCancelled`
                    (goto _label_2)))
                (else
                  (`PaperZDPlaySlotOverrideAction.PlayAnimationOverrideWithCallbacks` (`self.PaperAnimInstance`) "/Game/Assets/Character/AnimSequences/2H_Execute_End.2H_Execute_End"
                    (:`then`
                      (`PaperZDPlaySlotOverrideAction.PlayAnimationOverrideWithCallbacks` (`self.WeaponAnimInstance`) "/Game/Assets/Equipment/TwoHanded/AnimSequences/GreatSword_Execute_End.GreatSword_Execute_End"
                        (:`then`
                          (goto _label))))
                    (:`OnCompleted`
                      (goto _label_2))
                    (:`OnCancelled`
                      (goto _label_2))))))))))
    (:`OnCancelled`
      (goto _label_2))))

(fn `Dash`
  (bind _returnvalue (`self.GetAvatarActorFromActorInfo`))
  (`PrimitiveComponent.SetCollisionResponseToChannel` (`Character.CapsuleComponent` (cast `BaseCharacter` (`self.GetAvatarActorFromActorInfo`) :!pure true)) "ECC_GameTraceChannel2" "ECR_Ignore")
  (`CharacterMovementComponent.AddImpulse` (`Character.CharacterMovement` (cast `Character` _returnvalue :!pure true)) (* (`Actor.GetActorForwardVector` _returnvalue) 7500.0) true))