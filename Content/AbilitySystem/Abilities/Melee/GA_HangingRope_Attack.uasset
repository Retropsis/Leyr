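; Gameplay ability for a melee attack made while hanging on a rope.
; It disables movement and plays the avatar's tag-selected Paper 2D animation override, restoring movement and ending after a short delay on completion or cancel.
; A one-shot gameplay event triggers a box trace that damages hostile hits, then fires one weapon gameplay cue above the last traced actor if anything was damaged.
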(event `self.K2_OnEndAbility`
  (params (bWasCancelled :type Boolean)))

(event `self.K2_ActivateAbility`
  (set `self.HasHitTarget` false)
  (bind _output_get (set `self.MontageTag` (struct :`TagName` "Montage.Rope.Attack")))
  (bind _returnvalue (message `CombatInterface.GetTaggedMontageByTag` (`self.GetAvatarActorFromActorInfo`) _output_get))
  (set `self.Montage` (`.Montage` (break `TaggedMontage` _returnvalue)))
  (message `CombatInterface.SetMovementEnabled` (`self.GetAvatarActorFromActorInfo`) false)
  (bind _returnvalue_2 (message `CombatInterface.GetPaperAnimInstance` (`self.GetAvatarActorFromActorInfo`)))
  (`PaperZDPlaySlotOverrideAction.PlayAnimationOverrideWithCallbacks` _returnvalue_2 (`self.Montage`)
    (:`then`
      (`AbilityTask_WaitGameplayEvent.WaitGameplayEvent` (`self.MontageTag`) null true
        (:`EventReceived`
          (bind _returnvalue_3 (`self.BoxTrace`))
          (for _array_element _returnvalue_3
            (bind (_bblockinghit _binitialoverlap _time _distance _location _impactpoint _normal _impactnormal _physmat _hitactor) (`GameplayStatics.BreakHitResult` _array_element))
            (set `self.HitActor` _hitactor)
            (if _bblockinghit
              (if (`LeyrAbilitySystemLibrary.IsHostile` (`self.HitActor`) (`self.GetAvatarActorFromActorInfo`))
                (`self.CauseDamage` (`self.HitActor`))
                (set `self.HasHitTarget` true))))
          (message `CombatInterface.GetImpactEffect` (`self.HitActor`))
          (if (`self.HasHitTarget`)
            (`self.K2_ExecuteGameplayCueWithParams` (struct :`TagName` "GameplayCue.Weapon") (`AbilitySystemBlueprintLibrary.MakeGameplayCueParameters` 0.0 0.0 (struct) (struct) (struct) (`BlueprintGameplayTagLibrary.MakeGameplayTagContainerFromTag` (`self.MontageTag`)) (struct) (+ (`Actor.K2_GetActorLocation` (`self.HitActor`)) (0.0 0.0 75.0)) (0.0 0.0 0.0) null (`self.GetAvatarActorFromActorInfo`) (`self.HitActor`)))))))
    (:`OnCompleted`
      (message `CombatInterface.SetMovementEnabled` (`self.GetAvatarActorFromActorInfo`) true :!label _label)
      (`KismetSystemLibrary.Delay` 0.2)
      (`self.K2_EndAbility`))
    (:`OnCancelled`
      (goto _label))))