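; Gameplay ability that uses a health potion to heal its owner, apparently the menu-triggered variant.
; On activation it commits an inventory cost, then applies healing to its own ability system component, fires a cure gameplay cue attached to the owner's root and commits the cooldown.
; A failed cost only prints a not-enough-item message; both paths end the ability immediately.
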(event `self.K2_OnEndAbility`
  (params (bWasCancelled :type Boolean))
  (`self.PrepareToEndAbility`))

(event `self.K2_ActivateAbility`
  (`self.InitAbility`)
  (bind _returnvalue (`self.CommitInventoryCost` true))
  (if _returnvalue
    (`self.CauseHealing` (`self.GetAbilitySystemComponentFromActorInfo`))
    (`self.K2_ExecuteGameplayCueWithParams` (struct :`TagName` "GameplayCue.Healing.Cure.1") (`AbilitySystemBlueprintLibrary.MakeGameplayCueParameters` 0.0 0.0 (struct) (struct) (struct) (struct) (struct) (0.0 0.0 25.0) (0.0 0.0 0.0) null null null null 1 1 (`Actor.RootComponent` (`self.GetOwningActorFromActorInfo`))))
    (`self.K2_CommitAbilityCooldown` false)
    (`self.K2_EndAbility`)
    (else
      (`KismetSystemLibrary.PrintString` "NOT ENOUGH ITEM")
      (`self.K2_EndAbility`))))