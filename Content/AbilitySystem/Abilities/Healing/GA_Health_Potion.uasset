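; GA_Health_Potion is a Gameplay Ability that heals the user by consuming a health potion from inventory.
; On activation it initializes, then commits the inventory cost.
; On success it applies healing to the owner's ability system, spawns an attached leaves Niagara effect, plays a confirm sound, commits the cooldown and ends.
; If the cost fails, it prints a not-enough-item message and ends.
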(event `self.K2_ActivateAbility`
  (bind _returnvalue (`self.GetOwningActorFromActorInfo`))
  (bind _returnvalue_2 (`Actor.K2_GetActorLocation` _returnvalue))
  (`self.InitAbility`)
  (bind _returnvalue_3 (`self.CommitInventoryCost` true))
  (if _returnvalue_3
    (`self.CauseHealing` (`self.GetAbilitySystemComponentFromActorInfo`))
    (`NiagaraFunctionLibrary.SpawnSystemAttached` "/Game/Effects/Leaves/NS_Leaves.NS_Leaves" (`Actor.RootComponent` _returnvalue) "None" _returnvalue_2 (struct) "SnapToTarget" true)
    (`GameplayStatics.PlaySoundAtLocation` "/Engine/VREditor/Sounds/VR_confirm_Cue.VR_confirm_Cue" _returnvalue_2 (struct) 1.0 1.0 0.0 null null null null)
    (`self.K2_CommitAbilityCooldown` false)
    (`self.K2_EndAbility`)
    (else
      (`KismetSystemLibrary.PrintString` "NOT ENOUGH ITEM")
      (`self.K2_EndAbility`))))