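; Bow gameplay ability that spends inventory ammo, holds an aiming state, and fires a projectile when input is released.
; On release it commits, turns the avatar toward the cursor hit, and plays the lower shoot animation on its Paper anim instance.
; The shot gameplay event applies the avatar's pitch override, spawns the projectile and Niagara effect ahead of the actor, and exits aiming.
; Animation completion, cancellation or lack of ammo ends the ability.
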(event `self.K2_OnEndAbility`
  (params (bWasCancelled :type Boolean))
  (`self.PrepareToEndAbility`))

(event `self.K2_ActivateAbility`
  (bind _returnvalue (`self.GetAvatarActorFromActorInfo`))
  (bind _returnvalue_2 (`self.GetAvatarActorFromActorInfo`))
  (`self.InitAbility`)
  (bind _returnvalue_3 (`self.CommitInventoryCost` false))
  (if _returnvalue_3
    (`|ExecutionSequence`
      (:`then_0`
        ;[1 1 1] Make Aiming State
        (message `PlayerInterface.ToggleAiming` (`self.GetAvatarActorFromActorInfo`) true))
      (:`then_1`
        (`AbilityTask_WaitInputRelease.WaitInputRelease` false
          (:`OnRelease`
            (`self.K2_CommitAbility`)
            (bind (_asynctaskproxy _datahandle) (`TargetDataUnderCursor.CreateTargetDataUnderCursor`)
              (:`ValidData`
                (set `self.CursorHitLocation` (`.Location` (`GameplayStatics.BreakHitResult` (`AbilitySystemBlueprintLibrary.GetHitResultFromTargetData` _datahandle))))
                (message `CombatInterface.UpdateFacingTarget` (`self.GetAvatarActorFromActorInfo`) (`self.CursorHitLocation`))
                (bind _returnvalue_4 (message `CombatInterface.GetPaperAnimInstance` (`self.GetAvatarActorFromActorInfo`)))
                (`PaperZDPlaySlotOverrideAction.PlayAnimationOverrideWithCallbacks` _returnvalue_4 "/Game/Assets/Character/AnimSequences/Shoot_Lower.Shoot_Lower"
                  (:`then`
                    (`AbilityTask_WaitGameplayEvent.WaitGameplayEvent` (struct :`TagName` "Event.Montage.Bow.Shot") null true
                      (:`then`
                        (set `self.bHasTarget` true))
                      (:`EventReceived`
                        (bind _returnvalue_5 (message `CombatInterface.GetOverridePitch` (`self.GetAvatarActorFromActorInfo`)))
                        (`self.SetPitchOverride` true _returnvalue_5)
                        (`self.SpawnProjectile` (`BlueprintGameplayTagLibrary.MakeLiteralGameplayTag` (struct :`TagName` "CombatSocket.Weapon.UpperBody")) (+ (`Actor.K2_GetActorLocation` _returnvalue_2) (* (`Actor.GetActorForwardVector` _returnvalue_2) 125.0) (* (`Actor.GetActorUpVector` _returnvalue_2) 25.0)))
                        (message `PlayerInterface.ToggleAiming` (`self.GetAvatarActorFromActorInfo`) false)
                        (`NiagaraFunctionLibrary.SpawnSystemAtLocation` "/Game/Effects/BowShot/NS_BowShot.NS_BowShot" (+ (`Actor.K2_GetActorLocation` _returnvalue) (* (`Actor.GetActorForwardVector` _returnvalue) 55.0) (* (`Actor.GetActorUpVector` _returnvalue) 25.0))))))
                  (:`OnCompleted`
                    (`self.K2_EndAbility` :!label _label))
                  (:`OnCancelled`
                    (goto _label)))))))))
    (else
      (`KismetSystemLibrary.PrintString` "NOT ENOUGH AMMO")
      (`self.K2_EndAbility`))))