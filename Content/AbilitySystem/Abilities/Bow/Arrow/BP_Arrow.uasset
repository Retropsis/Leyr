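; Bow ability arrow projectile that plays a scripted tumble-and-move animation when its on-hit event fires.
; One timeline spins it on pitch by a randomly scaled curve (the track is named Yaw), zeroing roll and yaw.
; A parallel timeline lerps it without sweep from its initial hit position to a target location, then calls PrepareToDestroyProjectile.
; Both positions are only read here, not set.
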(event `self.OnHitTimeline`
  (set `self.RandomRotationAmount` (`KismetMathLibrary.RandomFloatInRange` 45.0 225.0))
  (`|ExecutionSequence`
    (:`then_0`
      (bind (_direction _yaw) (`Timeline|Timeline` :!via `PlayFromStart`)
        (:`Update`
          (`self.K2_SetActorRotation` (`KismetMathLibrary.MakeRotator` 0.0 (* _yaw (`self.RandomRotationAmount`)))))))
    (:`then_1`
      (bind (_direction_2 _alpha) (`Timeline|Timeline_0` :!via `PlayFromStart`)
        (:`Update`
          (`self.K2_SetActorLocation` (`KismetMathLibrary.VLerp` (`self.InitialOnHitTimeline`) (`self.TargetLocation`) _alpha)))
        (:`Finished`
          (`self.PrepareToDestroyProjectile`))))))

(fn `UserConstructionScript`)