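; GA_Weakened is a gameplay ability for the Weakened status state, pairing a gameplay effect with a hit-react animation.
; On activation it applies GE_Weakened to the owner and plays the avatar's tag-selected hit-react sequence as a PaperZD animation override, stopping weapon animation overrides.
; The ability ends when the animation completes or is cancelled, removing the effect through its stored handle, so the effect lasts only as long as the ability.
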(event `self.K2_OnEndAbility`
  (params (bWasCancelled :type Boolean))
  (`self.BP_RemoveGameplayEffectFromOwnerWithHandle` (`self.ActiveEffectHitReact`)))

(event `self.K2_ActivateAbility`
  (`KismetSystemLibrary.PrintString` "Weakened Activated" true true (struct :`R` 1.0 :`G` 0.143753 :`A` 1.0) 4.0)
  (bind _returnvalue (`self.BP_ApplyGameplayEffectToOwner` "/Game/AbilitySystem/Effects/States/GE_Weakened.GE_Weakened_C"))
  (set `self.ActiveEffectHitReact` _returnvalue)
  (bind _returnvalue_2 (message `CombatInterface.GetHitReactSequence` (`self.GetAvatarActorFromActorInfo`) (`BlueprintGameplayTagLibrary.MakeLiteralGameplayTag` (struct :`TagName` "StatusEffect.Weakened"))))
  (bind _returnvalue_3 (message `CombatInterface.GetPaperAnimInstance` (`self.GetAvatarActorFromActorInfo`)))
  (`PaperZDPlaySlotOverrideAction.PlayAnimationOverrideWithCallbacks` _returnvalue_3 _returnvalue_2
    (:`then`
      (bind _returnvalue_4 (message `CombatInterface.GetWeaponAnimInstance` (`self.GetAvatarActorFromActorInfo`)))
      (`PaperZDAnimInstance.StopAllAnimationOverrides` _returnvalue_4))
    (:`OnCompleted`
      (`self.K2_EndAbility` :!label _label))
    (:`OnCancelled`
      (goto _label))))