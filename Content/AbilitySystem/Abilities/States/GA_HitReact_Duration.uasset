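; Gameplay ability that escalates hit reactions by GE_HitReact_Duration stack count, skipping if the owner is Weakened.
; The first hit adds a stack, the second also plays a hit-react animation, and further hits apply Weakened with animation, afterimage and cooldown, or another stack while cooling down.
; On end, the last applied effect handle is fully removed at two-plus stacks, otherwise one stack is removed by an attribute-based random roll.
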(event `self.K2_OnEndAbility`
  (params (bWasCancelled :type Boolean))
  (if (>= (`self.Count`) 2)
    (`self.BP_RemoveGameplayEffectFromOwnerWithHandle` (`self.ActiveEffectHitReact`))
    (elif (< (`KismetMathLibrary.RandomIntegerInRange` 1 100) (`.ReturnValue` (`AbilitySystemBlueprintLibrary.GetFloatAttributeBaseFromAbilitySystemComponent` (`self.GetAbilitySystemComponentFromActorInfo`) (struct :`AttributeName` "Vitality" :`Attribute` "/Script/Leyr.BaseAttributeSet:Vitality" :`AttributeOwner` "/Script/CoreUObject.Class'/Script/Leyr.BaseAttributeSet'"))))
      (`self.BP_RemoveGameplayEffectFromOwnerWithHandle` (`self.ActiveEffectHitReact`) 1))))

(event `self.K2_ActivateAbility`
  (if (> (`AbilitySystemComponent.GetGameplayEffectCount` (`self.GetAbilitySystemComponentFromActorInfo`) "/Game/AbilitySystem/Effects/States/GE_Weakened.GE_Weakened_C" null true) 0)
    (`self.K2_EndAbility`)
    (else
      (bind _output_get (set `self.Count` (`AbilitySystemComponent.GetGameplayEffectCount` (`self.GetAbilitySystemComponentFromActorInfo`) "/Game/AbilitySystem/Effects/States/GE_HitReact_Duration.GE_HitReact_Duration_C" null true)))
      (switch `int` _output_get
        (:`Default`
          (if (>= (`self.Count`) 2)
            (bind _returnvalue (`self.K2_CheckAbilityCooldown`))
            (if _returnvalue
              (bind _returnvalue_2 (`self.BP_ApplyGameplayEffectToOwner` "/Game/AbilitySystem/Effects/States/GE_Weakened.GE_Weakened_C"))
              (set `self.ActiveEffectHitReact` _returnvalue_2)
              (bind _returnvalue_3 (message `CombatInterface.GetHitReactSequence` (`self.GetAvatarActorFromActorInfo`) (`BlueprintGameplayTagLibrary.MakeLiteralGameplayTag` (struct :`TagName` "StatusEffect.Weakened"))))
              (bind _returnvalue_4 (message `CombatInterface.GetPaperAnimInstance` (`self.GetAvatarActorFromActorInfo`)))
              (`PaperZDPlaySlotOverrideAction.PlayAnimationOverrideWithCallbacks` _returnvalue_4 _returnvalue_3
                (:`then`
                  (bind _returnvalue_5 (message `CombatInterface.GetWeaponAnimInstance` (`self.GetAvatarActorFromActorInfo`)))
                  (`PaperZDAnimInstance.StopAllAnimationOverrides` _returnvalue_5)
                  (`self.K2_CommitAbilityCooldown` false)
                  (`NiagaraFunctionLibrary.SpawnSystemAttached` "/Game/Effects/AfterImage/HitReact/NS_HitReact_AfterImage.NS_HitReact_AfterImage" (`Actor.RootComponent` (`self.GetAvatarActorFromActorInfo`)) "None" (0.0 0.0 0.0) (struct) "KeepRelativeOffset" true))
                (:`OnCompleted`
                  (`self.K2_EndAbility` :!label _label))
                (:`OnCancelled`
                  (goto _label)))
              (else
                (bind _returnvalue_6 (`self.BP_ApplyGameplayEffectToOwner` "/Game/AbilitySystem/Effects/States/GE_HitReact_Duration.GE_HitReact_Duration_C" :!label _label_2))
                (set `self.ActiveEffectHitReact` _returnvalue_6)
                (`KismetSystemLibrary.Delay` 0.2)
                (`self.K2_EndAbility`)))))
        (:`0`
          (goto _label_2))
        (:`1`
          (bind _returnvalue_7 (`self.BP_ApplyGameplayEffectToOwner` "/Game/AbilitySystem/Effects/States/GE_HitReact_Duration.GE_HitReact_Duration_C"))
          (set `self.ActiveEffectHitReact` _returnvalue_7)
          (bind _returnvalue_8 (message `CombatInterface.GetHitReactSequence` (`self.GetAvatarActorFromActorInfo`) (`BlueprintGameplayTagLibrary.MakeLiteralGameplayTag` (struct :`TagName` "StatusEffect.HitReact"))))
          (bind _returnvalue_9 (message `CombatInterface.GetPaperAnimInstance` (`self.GetAvatarActorFromActorInfo`)))
          (`PaperZDPlaySlotOverrideAction.PlayAnimationOverrideWithCallbacks` _returnvalue_9 _returnvalue_8
            (:`then`
              (bind _returnvalue_10 (message `CombatInterface.GetWeaponAnimInstance` (`self.GetAvatarActorFromActorInfo`)))
              (`PaperZDAnimInstance.StopAllAnimationOverrides` _returnvalue_10))
            (:`OnCompleted`
              (`self.K2_EndAbility` :!label _label_3))
            (:`OnCancelled`
              (goto _label_3))))))))