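; Gameplay ability that puts the avatar into a hit react state for the length of its hit react animation.
; On activation it applies the infinite hit react effect to the owner and plays the avatar's tagged sequence as a Paper animation override, stopping weapon animation overrides.
; Completion or cancellation of the animation ends the ability, which removes the effect through its stored handle.
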(event `self.K2_OnEndAbility`
  (params (bWasCancelled :type Boolean))
  (`self.BP_RemoveGameplayEffectFromOwnerWithHandle` (`self.ActiveEffectHitReact`)))

(event `self.K2_ActivateAbility`
  (bind _returnvalue (`self.BP_ApplyGameplayEffectToOwner` "/Game/AbilitySystem/Effects/States/GE_HitReact_Infinite.GE_HitReact_Infinite_C"))
  (set `self.ActiveEffectHitReact` _returnvalue)
  (bind _returnvalue_2 (message `CombatInterface.GetHitReactSequence` (`self.GetAvatarActorFromActorInfo`) (`BlueprintGameplayTagLibrary.MakeLiteralGameplayTag` (struct :`TagName` "StatusEffect.HitReact"))))
  (bind _returnvalue_3 (message `CombatInterface.GetPaperAnimInstance` (`self.GetAvatarActorFromActorInfo`)))
  (`PaperZDPlaySlotOverrideAction.PlayAnimationOverrideWithCallbacks` _returnvalue_3 _returnvalue_2
    (:`then`
      (bind _returnvalue_4 (message `CombatInterface.GetWeaponAnimInstance` (`self.GetAvatarActorFromActorInfo`)))
      (`PaperZDAnimInstance.StopAllAnimationOverrides` _returnvalue_4))
    (:`OnCompleted`
      (`self.K2_EndAbility` :!label _label))
    (:`OnCancelled`
      (goto _label))))