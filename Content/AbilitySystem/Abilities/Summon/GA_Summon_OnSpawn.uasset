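; Gameplay ability that summons random minions at shuffled spawn locations while blocking the caster's movement.
; On activation it spawns a particle effect per location and plays a Paper animation override, ending when that completes or is cancelled.
; The Montage.Casting event starts a delay-driven loop that spawns minions one at a time, facing away from the caster.
; Each gets an owner and controller, and updates the caster's minion count on spawn and destruction.
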(event `self.K2_OnEndAbility`
  (params (bWasCancelled :type Boolean))
  (`self.PrepareToEndAbilityWithParams` (make `EndAbilityParams` true (struct :`GameplayTags` (struct :`(TagName` "CombatState.Rule.Block.Movement"))))))

(event `self.K2_ActivateAbility`
  (bind _returnvalue (+ (`|GetArrayItem` (`self.SpawnLocations`) (`self.SpawnLocationIndex`)) (0.0 0.0 75.0)))
  (`self.InitAbilityWithParams` (make `InitAbilityParams` true (struct :`GameplayTags` (struct :`(TagName` "CombatState.Rule.Block.Movement")))))
  (`self.SetCurrentSequence`)
  (bind _returnvalue_2 (`self.GetSpawnLocations`))
  (bind _output_get (set `self.SpawnLocations` _returnvalue_2))
  (`KismetArrayLibrary.Array_Shuffle` _output_get)
  (for _ (`self.SpawnLocations`)
    ;[1 1 1] Make Summon Particle
    (`NiagaraFunctionLibrary.SpawnSystemAtLocation` null))
  (`PaperZDPlaySlotOverrideAction.PlayAnimationOverrideWithCallbacks` (`self.PaperAnimInstance`) (`self.SelectedMontage`)
    (:`then`
      (`AbilityTask_WaitGameplayEvent.WaitGameplayEvent` (struct :`TagName` "Montage.Casting") null true
        (:`EventReceived`
          (if (< (`self.SpawnLocationIndex`) (`KismetArrayLibrary.Array_Length` (`self.SpawnLocations`))) :!label _label
            (bind _returnvalue_3 (`|SpawnActorFromClass` (`self.GetRandomMinionClass`) (`KismetMathLibrary.MakeTransform` _returnvalue (`KismetMathLibrary.MakeRotator` 0.0 0.0 (.yaw (`KismetMathLibrary.FindLookAtRotation` (`Actor.K2_GetActorLocation` (`self.GetAvatarActorFromActorInfo`)) _returnvalue)))) "AdjustIfPossibleButAlwaysSpawn" "MultiplyWithRoot" null null))
            (message `AIInterface.SetOwningSummoner` _returnvalue_3 (`self.GetAvatarActorFromActorInfo`))
            (add `Actor.OnDestroyed` _returnvalue_3 (delegate `OnDestroyed_Event`))
            (`Pawn.SpawnDefaultController` _returnvalue_3)
            (message `CombatInterface.IncrementMinionCount` (`self.GetAvatarActorFromActorInfo`) 1)
            (`/Engine/EditorBlueprintResources/StandardMacros.IncrementInt` (`self.SpawnLocationIndex`)
              (:`  `
                (`KismetSystemLibrary.Delay` 0.2)
                (goto _label)))))))
    (:`OnCompleted`
      (`self.K2_EndAbility` :!label _label_2))
    (:`OnCancelled`
      (goto _label_2))))

(event `OnDestroyed_Event`
  (params (DestroyedActor :type "Actor Object Reference"))
  (message `CombatInterface.IncrementMinionCount` (`self.GetAvatarActorFromActorInfo`) -1))