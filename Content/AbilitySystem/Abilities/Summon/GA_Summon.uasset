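; Gameplay ability that summons random minions around its avatar, using a Paper2D-style animation override for the attack.
; On activation it shuffles the spawn locations, plays a particle at each and starts the animation.
; The Montage.Attack.1 gameplay event starts a delayed loop spawning AI-controlled minions one by one, facing away from the avatar.
; Spawns and destructions update the avatar's minion count; only animation cancellation ends the ability.
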(event `self.K2_ActivateAbility`
  (bind _returnvalue (+ (`|GetArrayItem` (`self.SpawnLocations`) (`self.SpawnLocationIndex`)) (0.0 0.0 75.0)))
  (bind _returnvalue_2 (`self.GetSpawnLocations`))
  (bind _output_get (set `self.SpawnLocations` _returnvalue_2))
  (`KismetArrayLibrary.Array_Shuffle` _output_get)
  (for _ (`self.SpawnLocations`)
    ;[1 1 1] Make Summon Particle
    (`NiagaraFunctionLibrary.SpawnSystemAtLocation` null))
  (bind _returnvalue_3 (message `CombatInterface.GetPaperAnimInstance` (`self.GetAvatarActorFromActorInfo`)))
  (`PaperZDPlaySlotOverrideAction.PlayAnimationOverrideWithCallbacks` _returnvalue_3 "/Game/AI/Necromancer/Animation/AnimSequences/Attack_3.Attack_3"
    (:`then`
      (`AbilityTask_WaitGameplayEvent.WaitGameplayEvent` (struct :`TagName` "Montage.Attack.1") null true
        (:`EventReceived`
          (if (< (`self.SpawnLocationIndex`) (`KismetArrayLibrary.Array_Length` (`self.SpawnLocations`))) :!label _label
            (bind _returnvalue_4 (`|SpawnActorFromClass` (`self.GetRandomMinionClass`) (`KismetMathLibrary.MakeTransform` _returnvalue (`KismetMathLibrary.MakeRotator` 0.0 0.0 (.yaw (`KismetMathLibrary.FindLookAtRotation` (`Actor.K2_GetActorLocation` (`self.GetAvatarActorFromActorInfo`)) _returnvalue)))) "AdjustIfPossibleButAlwaysSpawn" "MultiplyWithRoot" null null))
            (add `Actor.OnDestroyed` _returnvalue_4 (delegate `OnDestroyed_Event`))
            (`Pawn.SpawnDefaultController` _returnvalue_4)
            (message `CombatInterface.IncrementMinionCount` (`self.GetAvatarActorFromActorInfo`) 1)
            (`/Engine/EditorBlueprintResources/StandardMacros.IncrementInt` (`self.SpawnLocationIndex`)
              (:`  `
                (`KismetSystemLibrary.Delay` 0.2)
                (goto _label)))))))
    (:`OnCancelled`
      (`self.K2_EndAbility`))))

(event `OnDestroyed_Event`
  (params (DestroyedActor :type "Actor Object Reference"))
  (message `CombatInterface.IncrementMinionCount` (`self.GetAvatarActorFromActorInfo`) -1))