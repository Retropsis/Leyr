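; Gameplay ability that summons one random minion at the avatar's weapon socket, blocking movement via a tag until the ability ends.
; It spawns an effect system at the avatar and plays a PaperZD animation override, waiting for the Montage.Casting event to spawn the minion.
; The minion faces away from the avatar with a default controller, and its spawn and destruction adjust the avatar's minion count.
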(event `self.K2_OnEndAbility`
  (params (bWasCancelled :type Boolean))
  (`self.PrepareToEndAbilityWithParams` (make `EndAbilityParams` true (struct :`GameplayTags` (struct :`(TagName` "CombatState.Rule.Block.Movement"))))))

(event `self.K2_ActivateAbility`
  (`self.InitAbilityWithParams` (make `InitAbilityParams` true (struct :`GameplayTags` (struct :`(TagName` "CombatState.Rule.Block.Movement")))))
  (`self.SetCurrentSequence`)
  (`NiagaraFunctionLibrary.SpawnSystemAtLocation` null (`Actor.K2_GetActorLocation` (`self.GetAvatarActorFromActorInfo`)))
  (`PaperZDPlaySlotOverrideAction.PlayAnimationOverrideWithCallbacks` (`self.PaperAnimInstance`) (`self.SelectedMontage`)
    (:`then`
      (`AbilityTask_WaitGameplayEvent.WaitGameplayEvent` (struct :`TagName` "Montage.Casting") null true
        (:`EventReceived`
          (bind _returnvalue (`self.GetSingleSpawnLocationAtSocket` (`BlueprintGameplayTagLibrary.MakeLiteralGameplayTag` (struct :`TagName` "CombatSocket.Weapon"))))
          (set `self.SpawnLocation` _returnvalue)
          (bind _returnvalue_2 (`|SpawnActorFromClass` (`self.GetRandomMinionClass`) (`KismetMathLibrary.MakeTransform` (`self.SpawnLocation`) (`KismetMathLibrary.MakeRotator` 0.0 0.0 (.yaw (`KismetMathLibrary.FindLookAtRotation` (`Actor.K2_GetActorLocation` (`self.GetAvatarActorFromActorInfo`)) (`self.SpawnLocation`))))) "AdjustIfPossibleButAlwaysSpawn" "MultiplyWithRoot" null null))
          (add `Actor.OnDestroyed` _returnvalue_2 (delegate `OnDestroyed_Event`))
          (`Pawn.SpawnDefaultController` _returnvalue_2)
          (message `CombatInterface.IncrementMinionCount` (`self.GetAvatarActorFromActorInfo`) 1))))
    (:`OnCancelled`
      (`self.K2_EndAbility`))))

(event `OnDestroyed_Event`
  (params (DestroyedActor :type "Actor Object Reference"))
  (message `CombatInterface.IncrementMinionCount` (`self.GetAvatarActorFromActorInfo`) -1))