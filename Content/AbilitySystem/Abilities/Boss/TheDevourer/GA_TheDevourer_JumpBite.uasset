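; Gameplay ability for The Devourer boss's jump bite, triggered once a Montage.Ascent.Attack event arrives.
; Plays the bite montage on the multi-part flipbook alongside a Paper crocodile animation override, with large water splash cues.
; Montage events drive hit stop and the strike, which turns the boss downward and box-traces for damage.
; Montage completion or interruption ends the ability, which sends Montage.EndAbility to the avatar.
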(event `self.K2_OnEndAbility`
  (params (bWasCancelled :type Boolean))
  (`self.PrepareToEndAbility`)
  (`AbilitySystemBlueprintLibrary.SendGameplayEventToActor` (`self.GetAvatarActorFromActorInfo`) (struct :`TagName` "Montage.EndAbility")))

(event `self.K2_ActivateAbility`
  (`self.InitAbility`)
  (`AbilityTask_WaitGameplayEvent.WaitGameplayEvent` (struct :`TagName` "Montage.Ascent.Attack") null true
    (:`then`
      (bind _asmulti_part_aicharacter (cast `MultiPartAICharacter` (`self.GetAvatarActorFromActorInfo`)))
      (set `self.MultiPartAICharacter` _asmulti_part_aicharacter))
    (:`EventReceived`
      (`|PlayMontage` (`MultiPartAICharacter.MultiPartFlipbook` (`self.MultiPartAICharacter`)) "/Game/Assets/3D/Crocodile/AM_BiteAttck.AM_BiteAttck"
        (:`then`
          (`PaperZDPlaySlotOverrideAction.PlayAnimationOverrideWithCallbacks` (`self.PaperAnimInstance`) "/Game/AI/GiantCrocodile/AnimSequences/GiantCrocodile_Bite.GiantCrocodile_Bite"
            (:`then`
              (`AbilityTask_WaitGameplayEvent.WaitGameplayEvent` (struct :`TagName` "Montage.Attack.1") null true
                (:`then`
                  (`AbilityTask_WaitGameplayEvent.WaitGameplayEvent` (struct :`TagName` "Montage.HitStop") null true
                    (:`then`
                      (`self.CueWaterSplashes` (0.0 0.0 330.0))
                      (`AbilityTask_WaitGameplayEvent.WaitGameplayEvent` (struct :`TagName` "Montage.Cue.1") null true
                        (:`EventReceived`
                          (`self.CueWaterSplashes` (75.0 0.0 330.0)))))
                    (:`EventReceived`
                      (bind _asbase_character (cast `BaseCharacter` (`self.GetAvatarActorFromActorInfo`)))
                      (`BaseCharacter.HitStop` _asbase_character 0.3 0.2))))
                (:`EventReceived`
                  (message `MultiPartAIInterface.ChangeDirection` (`self.MultiPartAICharacter`) "Downward")
                  (bind _returnvalue (`self.BoxTrace` true))
                  (`self.ForEachHitTryCausingDamage` _returnvalue)
                  (if (`self.bHasHitTarget`)
                    (`self.ExecuteDamageGameplayCue` (struct :`TagName` "GameplayCue.Weapon"))))))))
        (:`OnCompleted`
          (`self.K2_EndAbility` :!label _label))
        (:`OnInterrupted`
          (goto _label))))))

(fn `CueWaterSplashes`
  (params (Offset :type "Vector Structure"))
  (bind _returnvalue (`self.GetAvatarActorFromActorInfo`))
  (`GameplayCueFunctionLibrary.ExecuteGameplayCueOnActor` (`self.GetAvatarActorFromActorInfo`) (struct :`TagName` "GameplayCue.WaterSplash.Large") (`AbilitySystemBlueprintLibrary.MakeGameplayCueParameters` 0.0 0.0 (struct) (struct) (struct) (struct) (struct) (+ (`Actor.K2_GetActorLocation` _returnvalue) Offset) (0.0 0.0 0.0) _returnvalue)))