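; Gameplay Ability that plays the avatar's hit reaction while a GE_HitReact effect is active on it.
; On activation it applies the effect, gets the hit-react sequence from the avatar and plays it as an animation override on BaseCharacter's AnimationComponent instance.
; Completion or cancellation of the animation removes the effect by its stored handle and ends the ability.
; An unconnected montage-based version of the same flow remains in the graph but never runs.
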(event `self.K2_ActivateAbility`
  (bind _returnvalue (`self.BP_ApplyGameplayEffectToOwner` "/Game/AbilitySystem/Effects/GE_HitReact.GE_HitReact_C"))
  (set `self.ActiveEffectHitReact` _returnvalue)
  (bind _returnvalue_2 (message `CombatInterface.GetHitReactSequence` (`self.GetAvatarActorFromActorInfo`)))
  (`PaperZDPlaySlotOverrideAction.PlayAnimationOverrideWithCallbacks` (`PaperZDAnimationComponent.AnimInstance` (`BaseCharacter.AnimationComponent` (cast `BaseCharacter` (`self.GetAvatarActorFromActorInfo`) :!pure true))) _returnvalue_2
    (:`OnCompleted`
      _)
    (:`OnCancelled`
      _))
  (`self.BP_RemoveGameplayEffectFromOwnerWithHandle` (`self.ActiveEffectHitReact`))
  (`self.K2_EndAbility`))