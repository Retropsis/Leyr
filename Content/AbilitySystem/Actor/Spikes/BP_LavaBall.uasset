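; BP_LavaBall is a lava ball actor that launches from its initial location up to an apex and drops back down.
; LaunchTimeline sets the state to MovingUp, waits briefly, then a rise timeline lerps the actor's location toward the apex.
; When that finishes, the state becomes MovingDown and a separate falling timeline lerps it back without sweep, ending in Idle.
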(event `self.LaunchTimeline`
  (set `self.LavaBallState` "MovingUp")
  (`KismetSystemLibrary.Delay` 0.2)
  (bind (_direction _z) (`Timeline|LavaBallTimeline` :!via `PlayFromStart`)
    (:`Update`
      (`self.K2_SetActorLocation` (`KismetMathLibrary.VLerp` (`self.InitialLocation`) (`self.ApexLocation`) _z)))
    (:`Finished`
      (set `self.LavaBallState` "MovingDown")
      (bind (_direction_2 _z_2) (`Timeline|FallingTimeline` :!via `PlayFromStart`)
        (:`Update`
          (`self.K2_SetActorLocation` (`KismetMathLibrary.VLerp` (`self.ApexLocation`) (`self.InitialLocation`) _z_2)))
        (:`Finished`
          (set `self.LavaBallState` "Idle"))))))

(fn `UserConstructionScript`)