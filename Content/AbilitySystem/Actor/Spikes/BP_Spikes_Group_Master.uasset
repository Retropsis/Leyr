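; BP_Spikes_Group_Master is a base spike-strip actor that builds itself from sprite tiles in the Construction Script.
; BuildTileMap refills a PaperGroupedSprite along BuildDirection at 64-unit spacing, using optional first/last caps and random picks from Tiles otherwise.
; It sizes BoxCollision to Length and offsets the sprites to center them along that axis.
; Only horizontal and vertical layouts are implemented; diagonal options yield zero vectors.
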(fn `BuildTileMap`
  (locals (TileIndex :type Integer))
  (bind _outitem (`KismetArrayLibrary.Array_Random` (`self.Tiles`)))
  (`PaperGroupedSpriteComponent.ClearInstances` (`self.PaperGroupedSprite`))
  (for _index (range (`self.Length`))
    (set `local.TileIndex` _index)
    (`PaperGroupedSpriteComponent.AddInstance` (`self.PaperGroupedSprite`) (`KismetMathLibrary.MakeTransform` (select `EBuildDirection` (`self.BuildDirection`) :`Horizontal` (`KismetMathLibrary.MakeVector` (`KismetMathLibrary.Conv_IntToDouble` (* (`local.TileIndex`) 64)) 0.0 (`self.SpriteGroupZ`)) :`Vertical` (`KismetMathLibrary.MakeVector` (`self.SpriteGroupZ`) 0.0 (`KismetMathLibrary.Conv_IntToDouble` (* (`local.TileIndex`) 64))))) (select `bool` (and (== (`local.TileIndex`) 0) (`KismetSystemLibrary.IsValid` (`self.FirstTile`))) :`false` (select `bool` (and (== (`local.TileIndex`) (- (`self.Length`) 1)) (`KismetSystemLibrary.IsValid` (`self.LastTile`))) :`false` (select `bool` (`KismetSystemLibrary.IsValid` _outitem) :`false` (`|GetArrayItem` (`self.Tiles`)) :`true` _outitem) :`true` (`self.LastTile`)) :`true` (`self.FirstTile`)) false (struct :`R` 1.0 :`G` 1.0 :`B` 1.0 :`A` 1.0)))
  (`BoxComponent.SetBoxExtent` (`self.BoxCollision`) (select `EBuildDirection` (`self.BuildDirection`) :`Horizontal` (`KismetMathLibrary.MakeVector` (`KismetMathLibrary.Conv_IntToDouble` (* (`self.Length`) 32)) 100.0 (`self.BoxExtentHeight`)) :`Vertical` (`KismetMathLibrary.MakeVector` (`self.BoxExtentHeight`) 100.0 (`KismetMathLibrary.Conv_IntToDouble` (* (`self.Length`) 32)))) true)
  (`SceneComponent.K2_SetRelativeLocation` (`self.PaperGroupedSprite`) (select `EBuildDirection` (`self.BuildDirection`) :`Horizontal` (`KismetMathLibrary.MakeVector` (`KismetMathLibrary.Conv_IntToDouble` (* (* (- (`self.Length`) 1) 32) -1)) 0.0 -16.0) :`Vertical` (`KismetMathLibrary.MakeVector` 0.0 0.0 (`KismetMathLibrary.Conv_IntToDouble` (* (* (- (`self.Length`) 1) 32) -1)))) false false))

(fn `UserConstructionScript`
  (`self.BuildTileMap`))