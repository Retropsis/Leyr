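; Falling spikes actor that hangs from a chain of sprites, with chain links hidden above a set height.
; The construction script stacks the first chain sprite vertically as grouped sprite instances, one per unit of Length; the top-cap sprite code never runs.
; Tick makes instances above the VisibilityPoint height captured at BeginPlay transparent and the rest opaque white, recolouring every instance each frame.
; BeginPlay also draws a debug line at that height.
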(event `self.ReceiveBeginPlay`
  (bind _output_get (set `self.VisibilityPosition` (`SceneComponent.K2_GetComponentLocation` (`self.VisibilityPoint`))))
  (`KismetSystemLibrary.DrawDebugLine` (+ _output_get (-50.0 0.0 0.0)) (+ _output_get (50.0 0.0 0.0)) (struct :`G` 1.0 :`B` 0.702494 :`A` 1.0) 180.0))

(event `self.ReceiveTick`
  (params (DeltaSeconds :type "Float (single-precision)"))
  (for _index (range (`PaperGroupedSpriteComponent.GetInstanceCount` (`self.PaperGroupedSprite`)))
    (if (> (.z (.location (`PaperGroupedSpriteComponent.GetInstanceTransform` (`self.PaperGroupedSprite`) _index true))) (.z (`self.VisibilityPosition`)))
      (`PaperGroupedSpriteComponent.UpdateInstanceColor` :`self` (`self.PaperGroupedSprite`) :`InstanceIndex` _index)
      (else
        (`PaperGroupedSpriteComponent.UpdateInstanceColor` (`self.PaperGroupedSprite`) _index (struct :`R` 1.0 :`G` 1.0 :`B` 1.0 :`A` 1.0) true)))))

(fn `BuildChains`
  (`PaperGroupedSpriteComponent.ClearInstances` (`self.PaperGroupedSprite`))
  (for _index (range 1 (+ (`self.Length`) 1))
    (`/Engine/EditorBlueprintResources/StandardMacros.IsValid` (`|GetArrayItem` (`self.Chains`))
      (:`Is Valid`
        (`PaperGroupedSpriteComponent.AddInstance` (`self.PaperGroupedSprite`) (`KismetMathLibrary.MakeTransform` (+ (`KismetMathLibrary.MakeVector` 0.0 0.0 (`KismetMathLibrary.Conv_IntToDouble` (* _index 96))) (0.0 0.0 45.0))) (`|GetArrayItem` (`self.Chains`)) false (struct :`R` 1.0 :`G` 1.0 :`B` 1.0 :`A` 1.0))))))

(fn `UserConstructionScript`
  (`self.BuildChains`))