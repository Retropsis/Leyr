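; Moving spike trap actor that damages actors touching its hit collision as the Paper2D flipbook animates.
; A looping timer started on BeginPlay sweeps HitCollision to the flipbook's "HitCollision" socket, so the hitbox follows the animation in steps without using Tick.
; Begin overlap calls CauseDamage on any valid actor, while end overlap only prints the actor's name for debugging.
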(event `self.ReceiveBeginPlay`
  (`KismetSystemLibrary.K2_SetTimerDelegate` (delegate `CustomEvent`) 0.15 true))

(event `CustomEvent`
  (if (`SceneComponent.DoesSocketExist` (`self.PaperFlipbook`) "HitCollision")
    (`SceneComponent.K2_SetWorldLocation` (`self.HitCollision`) (`SceneComponent.GetSocketLocation` (`self.PaperFlipbook`) "HitCollision") true false)))

(event `self.HitCollision.OnComponentBeginOverlap`
  (params (OverlappedComponent :type "PrimitiveComponent Object Reference") (OtherActor :type "Actor Object Reference") (OtherComp :type "PrimitiveComponent Object Reference") (OtherBodyIndex :type Integer) (bFromSweep :type Boolean) (SweepResult :type "HitResult Structure (by ref)"))
  (`/Engine/EditorBlueprintResources/StandardMacros.IsValid` OtherActor
    (:`Is Valid`
      (`self.CauseDamage` OtherActor))))

(event `self.HitCollision.OnComponentEndOverlap`
  (params (OverlappedComponent :type "PrimitiveComponent Object Reference") (OtherActor :type "Actor Object Reference") (OtherComp :type "PrimitiveComponent Object Reference") (OtherBodyIndex :type Integer))
  (`KismetSystemLibrary.PrintString` (`KismetSystemLibrary.GetDisplayName` OtherActor) true true (struct :`G` 0.66 :`B` 1.0 :`A` 1.0) 2.0 "fffffffff"))

(fn `UserConstructionScript`)