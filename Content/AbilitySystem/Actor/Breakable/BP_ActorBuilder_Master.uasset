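; BP_ActorBuilder_Master is a builder actor under Breakable that assembles a grid of child actors from a configurable class.
; The construction script calls BuildChildActors in Horizontal mode, the only direction implemented.
; Nested width and height loops add child actor components, spaced by tile size along the forward and up vectors.
; Each spawned child receives a ShowTopSpriteMessage carrying the TopVisibility setting.
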(event `self.BuildChildActors`
  (params (Direction :type "EBuildDirection Enum" :default "None"))
  (switch `EBuildDirection` Direction
    (:`Horizontal`
      (for _index (range (`self.WidthCount`))
        (for _index_2 (range (`self.HeightCount`))
          (bind _returnvalue (`AddComponent|NODE_AddChildActorComponent-0` :`RelativeTransform` (`KismetMathLibrary.MakeTransform` (+ (* (`self.GetActorForwardVector`) (* _index (`self.TileWidth`))) (* (`self.GetActorUpVector`) (* _index_2 (`self.TileHeight`)))))))
          (`ChildActorComponent.SetChildActorClass` _returnvalue (`self.ChildActorClass`))
          (message `ConstructionInterface.ShowTopSprite` (`ChildActorComponent.ChildActor` _returnvalue) (`self.TopVisibility`)))))))

(fn `UserConstructionScript`
  (`self.BuildChildActors` "Horizontal"))