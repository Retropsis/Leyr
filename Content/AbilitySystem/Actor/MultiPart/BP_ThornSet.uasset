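; BP_ThornSet is a multi-part thorn actor with an ability system, built on a multi-part flipbook with physics constraints.
; BeginPlay binds overlap events on five capsules along the body and prints every gameplay attribute on screen as debug output.
; HandleDetachment finds the first flipbook constraint whose parent body matches the given bone and makes it linearly breakable at a low threshold, so the part can break off.
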(event `self.ReceiveBeginPlay`
  (bind _returnvalue (`AbilitySystemBlueprintLibrary.GetAbilitySystemComponent` null))
  (`parent.ReceiveBeginPlay`)
  (add `PrimitiveComponent.OnComponentBeginOverlap` (`self.Capsule_1`) (`|CreateDelegate` :!event `OnBeginOverlap`))
  (add `PrimitiveComponent.OnComponentBeginOverlap` (`self.Capsule_2`) (`|CreateDelegate` :!event `OnBeginOverlap`))
  (add `PrimitiveComponent.OnComponentBeginOverlap` (`self.Capsule_Tail`) (`|CreateDelegate` :!event `OnBeginOverlap`))
  (add `PrimitiveComponent.OnComponentBeginOverlap` (`self.Capsule_3`) (`|CreateDelegate` :!event `OnBeginOverlap`))
  (add `PrimitiveComponent.OnComponentBeginOverlap` (`self.Capsule_Root`) (`|CreateDelegate` :!event `OnBeginOverlap`))
  (bind _returnvalue_2 (`AbilitySystemComponent.GetAttributeSet` _returnvalue "/Script/Leyr.BaseAttributeSet"))
  (for _array_element (`AbilitySystemComponent.GetAllAttributes` _returnvalue)
    (`KismetSystemLibrary.PrintString` (`AbilitySystemBlueprintLibrary.GetDebugStringFromGameplayAttribute` _array_element) true true (struct :`R` 1.0 :`G` 0.039766 :`A` 1.0) 8.0)))

(event `self.HandleDetachment`
  (params (BoneName :type Name))
  (bind _outconstraints (`SkeletalMeshComponent.GetConstraints` (`self.MultiPartFlipbook`) false))
  (for _array_element _outconstraints
    (bind _parentbody (`ConstraintInstanceBlueprintLibrary.GetAttachedBodyNames` _array_element))
    (if (== _parentbody BoneName)
      (`ConstraintInstanceBlueprintLibrary.SetLinearBreakable` _array_element true 10.0)
      (break))))

(fn `UserConstructionScript`)