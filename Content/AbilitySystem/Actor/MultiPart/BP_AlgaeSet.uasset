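; BP_AlgaeSet is a multi-part flipbook algae actor that reacts physically to overlaps and can detach parts.
; An ImpulseBox overlap enables physics blending and sets a three-second timer.
; The timer plays a timeline that drives the physics blend weight, then disables simulation and collision.
; Detachment makes the first constraint whose parent body matches the given bone linearly breakable at a low threshold.
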(event `self.ReceiveBeginPlay`
  (add `PrimitiveComponent.OnComponentBeginOverlap` (`self.ImpulseBox`) (`|CreateDelegate` :!event `OnBeginOverlap`)))

(event `self.HandleBeginOverlap`
  (`KismetSystemLibrary.K2_SetTimerDelegate` (delegate `ResetPhysics`) 3.0)
  (`SkeletalMeshComponent.SetEnablePhysicsBlending` (`self.MultiPartFlipbook`) true))

(event `ResetPhysics`
  (bind (_direction _blend) (`Timeline|Timeline` :!via `PlayFromStart`)
    (:`Update`
      (`SkeletalMeshComponent.SetAllBodiesPhysicsBlendWeight` (`self.MultiPartFlipbook`) _blend false))
    (:`Finished`
      (`PrimitiveComponent.SetSimulatePhysics` (`self.MultiPartFlipbook`) false)
      (`PrimitiveComponent.SetCollisionEnabled` (`self.MultiPartFlipbook`) "NoCollision"))))

(event `self.HandleDetachment`
  (params (BoneName :type Name))
  (bind _outconstraints (`SkeletalMeshComponent.GetConstraints` (`self.MultiPartFlipbook`) false))
  (for _array_element _outconstraints
    (bind _parentbody (`ConstraintInstanceBlueprintLibrary.GetAttachedBodyNames` _array_element))
    (if (== _parentbody BoneName)
      (`ConstraintInstanceBlueprintLibrary.SetLinearBreakable` _array_element true 10.0)
      (break))))

(fn `UserConstructionScript`)