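; Vine set actor built on a multi-part flipbook with physics constraints, whose segments can detach by bone name.
; On begin play it binds the impulse box overlap and gathers five capsules.
; Detachment turns off flipbook collision responses, makes constraints parented to that bone breakable at a low linear threshold, and spawns an attached effect for each.
; Capsules socketed to that bone then lose collision.
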(event `self.ReceiveBeginPlay`
  (add `PrimitiveComponent.OnComponentBeginOverlap` (`self.ImpulseBox`) (`|CreateDelegate` :!event `OnBeginOverlap`))
  (`KismetArrayLibrary.Array_Add` (`self.Capsules`) (`self.Capsule_1`))
  (`KismetArrayLibrary.Array_Add` (`self.Capsules`) (`self.Capsule_2`))
  (`KismetArrayLibrary.Array_Add` (`self.Capsules`) (`self.Capsule_3`))
  (`KismetArrayLibrary.Array_Add` (`self.Capsules`) (`self.Capsule_4`))
  (`KismetArrayLibrary.Array_Add` (`self.Capsules`) (`self.Capsule_5`)))

(event `self.HandleDetachment`
  (params (BoneName :type Name))
  (set `self.Bone` BoneName)
  (`PrimitiveComponent.SetCollisionResponseToAllChannels` (`self.MultiPartFlipbook`) "ECR_Ignore")
  (bind _outconstraints (`SkeletalMeshComponent.GetConstraints` (`self.MultiPartFlipbook`) false))
  (for _array_element _outconstraints
    (bind _parentbody (`ConstraintInstanceBlueprintLibrary.GetAttachedBodyNames` _array_element))
    (if (== _parentbody (`self.Bone`))
      (`ConstraintInstanceBlueprintLibrary.SetLinearBreakable` _array_element true 10.0)
      (`NiagaraFunctionLibrary.SpawnSystemAttached` (`self.InteractEffect`) (`self.MultiPartFlipbook`) (`self.Bone`) (0.0 0.0 0.0) (struct) "KeepRelativeOffset" true)))
  (for _array_element_2 (`self.Capsules`)
    (if (== (`SceneComponent.GetAttachSocketName` _array_element_2) (`self.Bone`))
      (`PrimitiveComponent.SetCollisionEnabled` _array_element_2 "NoCollision"))))

(fn `UserConstructionScript`)