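; BP_PendulunScythe is a pendulum scythe actor that rotates its box collision according to an Angle value.
; Each tick it sets the BoxCollision relative pitch to Angle plus a 90-degree offset; the graph only reads Angle and does not compute it.
; The construction script adds a child actor of a configurable class and attaches it to BoxCollision, so it follows the rotation.
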(event `self.ReceiveTick`
  (params (DeltaSeconds :type "Float (single-precision)"))
  (`SceneComponent.K2_SetRelativeRotation` (`self.BoxCollision`) (`KismetMathLibrary.MakeRotator` 0.0 (+ (`self.Angle`) 90.0)) false false))

(fn `UserConstructionScript`
  (bind _returnvalue (`AddComponent|NODE_AddChildActorComponent-0` :`RelativeTransform` (`KismetMathLibrary.MakeTransform` (`SceneComponent.RelativeLocation` (`self.BoxCollision`)))))
  (`ChildActorComponent.SetChildActorClass` _returnvalue (`self.ChildActorClass`))
  (`SceneComponent.K2_AttachToComponent` _returnvalue (`self.BoxCollision`) "None" "KeepRelative" "KeepRelative" "KeepRelative" true))